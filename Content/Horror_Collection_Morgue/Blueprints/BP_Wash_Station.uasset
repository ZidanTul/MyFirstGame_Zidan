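; BP_Wash_Station is a morgue wash station prop with a posable faucet and two taps.
; The construction script passes a separate yaw variable for each of the three meshes to a RotateZ helper, which sets that mesh's relative rotation.
; RotateZ can negate the yaw, though no call here uses that option, and the event graph holds only disabled placeholder events.
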(event EventBeginPlay)

(event Collision|EventActorBeginOverlap
  (params (OtherActor :type Actor%20Object%20Reference)))

(event EventTick
  (params (DeltaSeconds :type Float%20%28single-precision%29)))

(fn ConstructionScript
  (CallFunction|RotateZ (Variables|Default|GetFaucet_tap) false (Variables|Default|GetFaucet))
  (CallFunction|RotateZ (Variables|Default|GetTap1) false (Variables|Default|GetTap_1))
  (CallFunction|RotateZ (Variables|Default|GetTap2) false (Variables|Default|GetTap_2)))

(fn RotateZ
  (params (Z%20%28Yaw%29 :type Float%20%28double-precision%29) (Invert%20Z :type Boolean) (TargetMesh :type Scene%20Component%20Object%20Reference))
  (if Invert%20Z
    (Transformation|SetRelativeRotation TargetMesh (Math|Rotator|MakeRotator 0.0 0.0 (* Z%20%28Yaw%29 -1.0)) false false)
    (else
      (Transformation|SetRelativeRotation TargetMesh (Math|Rotator|MakeRotator 0.0 0.0 Z%20%28Yaw%29) false false)))
  (return))