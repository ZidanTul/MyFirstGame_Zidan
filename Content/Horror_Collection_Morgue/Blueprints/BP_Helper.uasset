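; BP_Helper is a helper actor that places many copies of one mesh through an InstancedStaticMesh component.
; Its construction script assigns the Mesh variable, then adds an instance for each entry in the Locations array.
; Rotations and Scales act as parallel arrays, applied only when both hold that index; otherwise the instance gets location alone.
; The event graph contains only disabled placeholder events, so the actor has no gameplay logic.
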(event EventBeginPlay)

(event Collision|EventActorBeginOverlap
  (params (OtherActor :type Actor%20Object%20Reference)))

(event EventTick
  (params (DeltaSeconds :type Float%20%28single-precision%29)))

(fn ConstructionScript
  (bind _instancedstaticmesh (Variables|Default|GetInstancedStaticMesh))
  (bind _locations (Variables|Default|GetLocations))
  (bind _rotations (Variables|Default|GetRotations))
  (bind _scales (Variables|Default|GetScales))
  (Components|StaticMesh|SetStaticMesh _instancedstaticmesh (Variables|Default|GetMesh))
  (if (Utilities|Array|IsValidIndex _locations)
    (for (_array_element _array_index) _locations
      (if (and (Utilities|Array|IsValidIndex _rotations _array_index) (Utilities|Array|IsValidIndex _scales _array_index))
        (Components|InstancedStaticMesh|AddInstance _instancedstaticmesh (Math|Transform|MakeTransform _array_element (Utilities|Array|Get(acopy) _rotations _array_index) (Utilities|Array|Get(acopy) _scales _array_index)) false)
        (else
          (Components|InstancedStaticMesh|AddInstance _instancedstaticmesh (Math|Transform|MakeTransform _array_element "0, 0, 0" "1.000000,1.000000,1.000000") false))))))