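; Configurable four-door morgue freezer prop, posed entirely in the Construction Script with no runtime logic.
; Per-door rotation values swing the doors, mirrored on 1 and 3, and show each chamber and door back only once slightly open.
; Trays apply their slide only behind wide-open doors, with body trays moving three times as far as rails.
; The top fridge unit can be toggled and slid; the extra mesh assignments are unconnected.
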(event EventBeginPlay)

(event Collision|EventActorBeginOverlap
  (params (OtherActor :type Actor%20Object%20Reference)))

(event EventTick
  (params (DeltaSeconds :type Float%20%28single-precision%29)))

(fn ConstructionScript
  (bind _tray1 (Variables|SlideTray|GetTray1))
  (bind _tray2 (Variables|SlideTray|GetTray2))
  (bind _tray3 (Variables|SlideTray|GetTray3))
  (bind _tray4 (Variables|SlideTray|GetTray4))
  (Transformation|AddLocalRotation (Variables|Default|GetMorgue_Fridge_SM_Fridge_Door1) (Math|Rotator|MakeRotator 0.0 0.0 (* (Variables|DoorParameter|GetDoor1Rotate) -1.0)) false false)
  (Transformation|AddLocalRotation (Variables|Default|GetMorgue_Fridge_SM_Fridge_Door2) (Math|Rotator|MakeRotator 0.0 0.0 (Variables|DoorParameter|GetDoor2Rotate)) false false)
  (Transformation|AddLocalRotation (Variables|Default|GetMorgue_Fridge_SM_Fridge_Door3) (Math|Rotator|MakeRotator 0.0 0.0 (* (Variables|DoorParameter|GetDoor3Rotate) -1.0)) false false)
  (Transformation|AddLocalRotation (Variables|Default|GetMorgue_Fridge_SM_Fridge_Door4) (Math|Rotator|MakeRotator 0.0 0.0 (Variables|DoorParameter|GetDoor4Rotate)) false false)
  (if (> (Variables|DoorParameter|GetDoor1Rotate) 2.0)
    (Rendering|SetVisibility (Variables|Default|GetMorgue_Fridge_SM_Chamber1) true true)
    (else
      (Rendering|SetVisibility (Variables|Default|GetMorgue_Fridge_SM_Chamber1) false true)))
  (if (> (Variables|DoorParameter|GetDoor2Rotate) 2.0)
    (Rendering|SetVisibility (Variables|Default|GetMorgue_Fridge_SM_Fridge_DoorBack2) true true)
    (else
      (Rendering|SetVisibility (Variables|Default|GetMorgue_Fridge_SM_Fridge_DoorBack2) false true)))
  (if (> (Variables|DoorParameter|GetDoor3Rotate) 2.0)
    (Rendering|SetVisibility (Variables|Default|GetMorgue_Fridge_SM_Fridge_DoorBack3) true true)
    (else
      (Rendering|SetVisibility (Variables|Default|GetMorgue_Fridge_SM_Chamber3) false true)))
  (if (> (Variables|DoorParameter|GetDoor4Rotate) 2.0)
    (Rendering|SetVisibility (Variables|Default|GetMorgue_Fridge_SM_Chamber4) true true)
    (else
      (Rendering|SetVisibility (Variables|Default|GetMorgue_Fridge_SM_Chamber4) false true)))
  (Rendering|SetVisibility (Variables|Default|GetMorgue_Fridge_SM_Refr) (Variables|FridgeOnTop|Get?FridgeOnTop) false)
  (Transformation|SetRelativeLocation (Variables|Default|GetMorgue_Fridge_SM_Refr) (Math|Vector|MakeVector (Variables|FridgeOnTop|GetFridgeSlide) 0.0 0.0) false false)
  (if (> (Variables|DoorParameter|GetDoor1Rotate) 123.0)
    (Transformation|SetRelativeLocation (Variables|Default|GetMorgue_Fridge_SM_Rails1) (Math|Vector|MakeVector 0.0 _tray1 0.0) false false)
    (Transformation|SetRelativeLocation (Variables|Default|GetMorgue_Fridge_SM_BodyTray1) (Math|Vector|MakeVector 0.0 (* _tray1 3.0) 0.0) false false))
  (if (> (Variables|DoorParameter|GetDoor2Rotate) 123.0)
    (Transformation|SetRelativeLocation (Variables|Default|GetMorgue_Fridge_SM_Rails2) (Math|Vector|MakeVector 0.0 _tray2 0.0) false false)
    (Transformation|SetRelativeLocation (Variables|Default|GetMorgue_Fridge_SM_BodyTray2) (Math|Vector|MakeVector 0.0 (* _tray2 3.0) 0.0) false false))
  (if (> (Variables|DoorParameter|GetDoor3Rotate) 123.0)
    (Transformation|SetRelativeLocation (Variables|Default|GetMorgue_Fridge_SM_Rails3) (Math|Vector|MakeVector 0.0 _tray3 0.0) false false)
    (Transformation|SetRelativeLocation (Variables|Default|GetMorgue_Fridge_SM_BodyTray3) (Math|Vector|MakeVector 0.0 (* _tray3 3.0) 0.0) false false))
  (if (> (Variables|DoorParameter|GetDoor4Rotate) 123.0)
    (Transformation|SetRelativeLocation (Variables|Default|GetMorgue_Fridge_SM_Rails4) (Math|Vector|MakeVector 0.0 _tray4 0.0) false false)
    (Transformation|SetRelativeLocation (Variables|Default|GetMorgue_Fridge_SM_BodyTray4) (Math|Vector|MakeVector 0.0 (* _tray4 3.0) 0.0) false false)))