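; Configurable floor lamp prop for the morgue environment, built entirely in the construction script with no active event logic.
; Height, Pitch and Roll parameters move, stretch and rotate the lamp's mesh parts.
; On switches the spot and point lights, while LightColor and LightIntensity drive the spotlight.
; When on, intensity also rotates one mesh part and, with color, feeds emissive materials and an optional, visibility-toggled light-shaft mesh.
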(event EventBeginPlay)

(event Collision|EventActorBeginOverlap
  (params (OtherActor :type Actor%20Object%20Reference)))

(event EventTick
  (params (DeltaSeconds :type Float%20%28single-precision%29)))

(fn ConstructionScript
  (bind _lightintensity (Variables|Base|GetLightIntensity))
  (bind _height (Variables|Base|GetHeight))
  (Transformation|SetRelativeLocation (Variables|Default|GetSM_LampFloor_01b) (Math|Vector|MakeVector 0.0 0.0 _height) false false)
  (Transformation|SetWorldScale3D (Variables|Default|GetSM_LampFloor_01f) (+ (Math|Vector|MakeVector 0.0 0.0 (* _height -0.06)) (Transformation|GetWorldScale (Variables|Default|GetSM_LampFloor_01f))))
  (Transformation|SetRelativeRotation (Variables|Default|GetSM_LampFloor_01d) (Math|Rotator|MakeRotator -14.091 (Variables|Base|GetPitch) 0.0) false false)
  (Transformation|SetRelativeRotation (Variables|Default|GetSM_LampFloor_01e) (Math|Rotator|MakeRotator (Variables|Base|GetRoll) 0.0 0.0) false false)
  (Rendering|SetVisibility (Variables|Default|GetSpotLight) (Variables|Base|Get?On) false)
  (Rendering|Components|Light|SetLightColor (Variables|Default|GetSpotLight) (Variables|Base|GetLightColor) true)
  (Rendering|Components|Light|SetIntensity (Variables|Default|GetSpotLight) (Variables|Base|GetLightIntensity))
  (Rendering|SetVisibility (Variables|Default|GetPointLight) (Variables|Base|Get?On) false)
  (if (Variables|Base|Get?On)
    (Transformation|SetRelativeRotation (Variables|Default|GetSM_LampFloor_01c) (Math|Rotator|MakeRotator 0.0 0.0 (* _lightintensity 0.052)) false false)
    (Rendering|Material|SetScalarParameterValueonMaterials (Variables|Default|GetSM_LampFloor_01g) "EmissiveInt" (* _lightintensity 0.005))
    (Rendering|Material|SetVectorParameterValueonMaterials (Variables|Default|GetSM_LampFloor_01g) "EmissiveColor" (Math|Conversions|ToVector(LinearColor) (Variables|Base|GetLightColor)))
    (if (Variables|Base|Get?LightShaftOn)
      (Rendering|ToggleVisibility (Variables|Default|GetSM_Lightshaft) false)
      (Rendering|Material|SetScalarParameterValueonMaterials (Variables|Default|GetSM_Lightshaft) "Emissive" (/ (Variables|Base|GetLightIntensity) 3e+02))
      (Rendering|Material|SetScalarParameterValueonMaterials (Variables|Default|GetSM_Lightshaft) "Foggy" (Variables|LightShaft|GetFoggy))
      (Rendering|Material|SetScalarParameterValueonMaterials (Variables|Default|GetSM_Lightshaft) "ShaftLenght" (Variables|LightShaft|GetShaftLenght))
      (Rendering|Material|SetVectorParameterValueonMaterials (Variables|Default|GetSM_Lightshaft) "ShaftColor" (Math|Conversions|ToVector(LinearColor) (Variables|Base|GetLightColor))))
    (else
      (Transformation|SetRelativeRotation (Variables|Default|GetSM_LampFloor_01c) "0, 0, 0" false false))))