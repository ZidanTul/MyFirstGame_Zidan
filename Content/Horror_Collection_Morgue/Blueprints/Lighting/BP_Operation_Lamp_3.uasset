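; Configurable two-headed operating lamp prop for the morgue environment, set up entirely in the Construction Script with no runtime logic.
; Exposed rotation and length variables pose the jointed bases, arms and heads.
; On1 and On2 toggle the five-bulb and twelve-bulb heads through emissive mesh visibility, propagated to children.
; Shared color and intensity drive spotlights and materials, while LightShaftOn shows fake shaft meshes on lit heads, tuned by fog and length parameters.
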(event EventBeginPlay)

(event Collision|EventActorBeginOverlap
  (params (OtherActor :type Actor%20Object%20Reference)))

(event EventTick
  (params (DeltaSeconds :type Float%20%28single-precision%29)))

(fn ConstructionScript
  (bind _staticmesh (Variables|Default|GetStaticMesh))
  (bind _lightcolor (Variables|LightCustomize|GetLightColor))
  (bind _spotlight (Variables|Default|GetSpotLight))
  (bind _staticmesh12 (Variables|Default|GetStaticMesh12))
  (bind _lightintensity (Variables|LightCustomize|GetLightIntensity))
  (bind _lightcolor_2 (Variables|LightCustomize|GetLightColor))
  (bind _spotlight15 (Variables|Default|GetSpotLight15))
  (bind _lightintensity_2 (Variables|LightCustomize|GetLightIntensity))
  (bind _lightcolor_3 (Variables|LightCustomize|GetLightColor))
  (bind _staticmesh4 (Variables|Default|GetStaticMesh4))
  (bind _lightcolor_4 (Variables|LightCustomize|GetLightColor))
  (bind _emissive4 (Variables|Default|GetEmissive4))
  (bind _returnvalue (Math|Conversions|ToVector(LinearColor) _lightcolor_2))
  (bind _returnvalue_2 (Math|Conversions|ToVector(LinearColor) _lightcolor_3))
  (Transformation|SetRelativeRotation (Variables|Default|GetSM_Operation_Lamp_3_Element_2) (Math|Rotator|MakeRotator 0.0 0.0 (Variables|Base_1st|GetYaw_1st_Lamp)) false false)
  (Transformation|SetRelativeRotation (Variables|Default|GetSM_Operation_Lamp_3_Element_3) (Math|Rotator|MakeRotator 0.0 0.0 (Variables|Base_2nd|GetYaw_2nd_Lamp)) false false)
  (Transformation|SetRelativeRotation (Variables|Default|GetSM_Operation_Lamp_3_Element_4) (Math|Rotator|MakeRotator (Variables|Base_1st|GetRoll_1st_Base) 0.0 0.0) false false)
  (Transformation|SetRelativeRotation (Variables|Default|GetSM_Operation_Lamp_3_Element_4_1) (Math|Rotator|MakeRotator (Variables|Base_2nd|GetRoll_2nd_Base) 0.0 0.0) false false)
  (Transformation|AddLocalOffset (Variables|Default|GetSM_Operation_Lamp_3_Element_5) (Math|Vector|MakeVector 0.0 (Variables|Base_1st|GetLenght_1st_Lamp) 0.0) false false)
  (Transformation|SetRelativeRotation (Variables|Default|GetSM_Operation_Lamp_3_Element_5) (Math|Rotator|MakeRotator 0.0 (Variables|Base_1st|GetPitch_1st_Lamp) 0.0) false false)
  (Transformation|SetRelativeRotation (Variables|Default|GetSM_Operation_Lamp_3_Element_8) (Math|Rotator|MakeRotator 0.0 (Variables|Base_2nd|GetPitch_2nd_Lamp) 0.0) false false)
  (Transformation|SetRelativeRotation (Variables|Default|GetSM_Operation_Lamp_3_Element_6) (Math|Rotator|MakeRotator (Variables|Base_1st|GetRoll_1st_Lamp) 0.0 0.0) false false)
  (Transformation|SetRelativeRotation (Variables|Default|GetSM_Operation_Lamp_3_Element_9) (Math|Rotator|MakeRotator (Variables|Base_2nd|GetRoll_2nd_Lamp) 0.0 0.0) false false)
  (if (Variables|Base_1st|Get?On1)
    (Rendering|SetVisibility _emissive4 true true)
    (if (Variables|LightCustomize|Get?Light_Shaft_On)
      (Rendering|SetVisibility _staticmesh true false)
      (Rendering|Components|Light|SetIntensity _spotlight _lightintensity_2)
      (Rendering|Components|Light|SetLightColor _spotlight _lightcolor_2 true)
      (Rendering|Material|SetVectorParameterValueonMaterials (Variables|Default|GetEmissive5) "EmissiveColor" _returnvalue)
      (Rendering|Material|SetVectorParameterValueonMaterials (Variables|Default|GetStaticMesh2) "ShaftColor" _returnvalue)
      (Rendering|Material|SetScalarParameterValueonMaterials _staticmesh4 "Emissive" (/ _lightintensity_2 3e+02))
      (Rendering|Material|SetScalarParameterValueonMaterials _staticmesh4 "Foggy" (Variables|LightCustomize|GetFoggy))
      (Rendering|Material|SetScalarParameterValueonMaterials (Variables|Default|GetStaticMesh3) "ShaftLenght" (Variables|LightCustomize|GetShaftLenght))
      (else
        (Rendering|SetVisibility _staticmesh false false :!label _label)
        (Rendering|Components|Light|SetIntensity (Variables|Default|GetSpotLight3) (Variables|LightCustomize|GetLightIntensity))
        (Rendering|Material|SetVectorParameterValueonMaterials (Variables|Default|GetEmissive5) "EmissiveColor" (Math|Conversions|ToVector(LinearColor) _lightcolor_4))
        (Rendering|Components|Light|SetLightColor (Variables|Default|GetSpotLight4) _lightcolor_4 true)))
    (else
      (Rendering|SetVisibility _emissive4 false true)
      (goto _label)))
  (if (Variables|Base_2nd|Get?On2)
    (Rendering|SetVisibility (Variables|Default|GetEmissive12) true true)
    (if (Variables|LightCustomize|Get?Light_Shaft_On)
      (Rendering|SetVisibility _staticmesh12 true false)
      (Rendering|Components|Light|SetIntensity _spotlight15 _lightintensity)
      (Rendering|Components|Light|SetLightColor _spotlight15 _lightcolor_3 true)
      (Rendering|Material|SetVectorParameterValueonMaterials (Variables|Default|GetEmissive9) "EmissiveColor" _returnvalue_2)
      (Rendering|Material|SetVectorParameterValueonMaterials _staticmesh12 "ShaftColor" _returnvalue_2)
      (Rendering|Material|SetScalarParameterValueonMaterials (Variables|Default|GetStaticMesh11) "Emissive" (/ _lightintensity 3e+02))
      (Rendering|Material|SetScalarParameterValueonMaterials (Variables|Default|GetStaticMesh11) "Foggy" (Variables|LightCustomize|GetFoggy))
      (Rendering|Material|SetScalarParameterValueonMaterials (Variables|Default|GetStaticMesh11) "ShaftLenght" (Variables|LightCustomize|GetShaftLenght))
      (else
        (Rendering|SetVisibility (Variables|Default|GetStaticMesh11) false false :!label _label_2)
        (Rendering|Components|Light|SetIntensity (Variables|Default|GetSpotLight15) (Variables|LightCustomize|GetLightIntensity))
        (Rendering|Material|SetVectorParameterValueonMaterials (Variables|Default|GetEmissive9) "EmissiveColor" (Math|Conversions|ToVector(LinearColor) _lightcolor))
        (Rendering|Components|Light|SetLightColor (Variables|Default|GetSpotLight5) _lightcolor true)))
    (else
      (Rendering|SetVisibility (Variables|Default|GetEmissive17) false true)
      (goto _label_2))))