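; Modular morgue ceiling section that configures itself in the Construction Script as solid, with lamp, damaged, or frame only.
; GeneralType toggles visibility of panels, frame, lamp, glass and point light.
; Damaged variants use a random stream to set root rotations through Random90Degrees and randomly tilt panels through AngleX/AngleY helpers.
; AngleX also stores a separately drawn Angle1, which decides whether the cables show.
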(event EventBeginPlay)

(event Collision|EventActorBeginOverlap
  (params (OtherActor :type Actor%20Object%20Reference)))

(event EventTick
  (params (DeltaSeconds :type Float%20%28single-precision%29)))

(fn ConstructionScript
  (bind _stream (Variables|Default|GetStream))
  (bind _stream_2 (Variables|Default|GetStream))
  (bind _stream_3 (Variables|Default|GetStream))
  (bind _stream_4 (Variables|Default|GetStream))
  (bind _angle1 (Variables|Default|GetAngle1))
  (bind _angle1_2 (Variables|Default|GetAngle1))
  (switch Utilities|FlowControl|Switch|SwitchonBP_Ceiling_System_Enum (Variables|Default|GetGeneral%20Type)
    (:NewEnumerator0
      (Rendering|SetVisibility (Variables|Default|GetSM_Lamp_Section_base_low) false true)
      (Rendering|SetVisibility (Variables|Default|GetPanel5) true false))
    (:NewEnumerator1
      (Rendering|SetVisibility (Variables|Default|GetPanel5) false true)
      (Rendering|SetVisibility (Variables|Default|GetPanel9) true false))
    (:NewEnumerator2
      (Rendering|SetVisibility (Variables|Default|GetSM_Lamp_Section_base_low) false true)
      (Rendering|SetVisibility (Variables|Default|GetPanel5) true false)
      (Transformation|SetWorldRotation (Variables|Default|GetRoot5) (Utilities|Random90Degrees _stream_2) false false)
      (Transformation|SetWorldRotation (Variables|Default|GetRoot2) (Utilities|Random90Degrees _stream_2) false false)
      (Transformation|SetWorldRotation (Variables|Default|GetRoot3) (Utilities|Random90Degrees _stream_2) false false)
      (Transformation|SetWorldRotation (Variables|Default|GetRoot4) (Utilities|Random90Degrees _stream_2) false false)
      (Transformation|SetWorldRotation (Variables|Default|GetRoot1) (Utilities|Random90Degrees _stream_2) false false)
      (Transformation|SetWorldRotation (Variables|Default|GetRoot7) (Utilities|Random90Degrees _stream_2) false false)
      (Transformation|SetWorldRotation (Variables|Default|GetRoot6) (Utilities|Random90Degrees _stream_2) false false)
      (Transformation|SetWorldRotation (Variables|Default|GetRoot9) (Utilities|Random90Degrees _stream_2) false false)
      (Transformation|SetWorldRotation (Variables|Default|GetRoot8) (Utilities|Random90Degrees _stream_2) false false)
      (CallFunction|AngleX _stream_3 (Variables|Default|GetPanel3))
      (CallFunction|Angle-X _stream_3 (Variables|Default|GetPanel7))
      (CallFunction|AngleX _stream_3 (Variables|Default|GetPanel1))
      (CallFunction|AngleY _stream_3 (Variables|Default|GetPanel4))
      (CallFunction|AngleY _stream_3 (Variables|Default|GetPanel5))
      (CallFunction|AngleY _stream_3 (Variables|Default|GetPanel6))
      (CallFunction|AngleY _stream_3 (Variables|Default|GetPanel2))
      (CallFunction|Angle-Y _stream_3 (Variables|Default|GetPanel8))
      (CallFunction|Angle-X _stream_3 (Variables|Default|GetPanel9))
      (if (and (>= _angle1 0.0) (< _angle1 4e+01))
        (Rendering|SetVisibility (Variables|Default|GetCable2) false false)
        (else
          (Rendering|SetVisibility (Variables|Default|GetCable) true false))))
    (:NewEnumerator3
      (Rendering|SetVisibility (Variables|Default|GetPanel5) false true)
      (Rendering|SetVisibility (Variables|Default|GetPanel9) true false)
      (Transformation|SetWorldRotation (Variables|Default|GetRoot5) (Utilities|Random90Degrees _stream) false false)
      (Transformation|SetWorldRotation (Variables|Default|GetRoot2) (Utilities|Random90Degrees _stream) false false)
      (Transformation|SetWorldRotation (Variables|Default|GetRoot3) (Utilities|Random90Degrees _stream) false false)
      (Transformation|SetWorldRotation (Variables|Default|GetRoot4) (Utilities|Random90Degrees _stream) false false)
      (Transformation|SetWorldRotation (Variables|Default|GetRoot1) (Utilities|Random90Degrees _stream) false false)
      (Transformation|SetWorldRotation (Variables|Default|GetRoot7) (Utilities|Random90Degrees _stream) false false)
      (Transformation|SetWorldRotation (Variables|Default|GetRoot6) (Utilities|Random90Degrees _stream) false false)
      (Transformation|SetWorldRotation (Variables|Default|GetRoot9) (Utilities|Random90Degrees _stream) false false)
      (Transformation|SetWorldRotation (Variables|Default|GetRoot8) (Utilities|Random90Degrees _stream) false false)
      (CallFunction|AngleX _stream_4 (Variables|Default|GetPanel3))
      (CallFunction|Angle-X _stream_4 (Variables|Default|GetPanel7))
      (CallFunction|AngleX _stream_4 (Variables|Default|GetPanel1))
      (CallFunction|AngleY _stream_4 (Variables|Default|GetPanel4))
      (CallFunction|AngleY _stream_4 (Variables|Default|GetPanel5))
      (CallFunction|AngleY _stream_4 (Variables|Default|GetPanel6))
      (CallFunction|AngleY _stream_4 (Variables|Default|GetPanel2))
      (CallFunction|Angle-Y _stream_4 (Variables|Default|GetPanel8))
      (CallFunction|Angle-X _stream_4 (Variables|Default|GetPanel9))
      (if (and (>= _angle1_2 0.0) (< _angle1_2 4e+01))
        (Rendering|SetVisibility (Variables|Default|GetCable2) false false)
        (else
          (Rendering|SetVisibility (Variables|Default|GetCable) true false))))
    (:NewEnumerator6
      (Rendering|SetVisibility (Variables|Default|GetSM_Lamp_Section_base_low) false true)
      (Rendering|SetVisibility (Variables|Default|GetRoot9) false true))))

(fn AngleY
  (params (Stream :type Random%20Stream%20Structure%20%28by%20ref%29) (Target :type Scene%20Component%20Object%20Reference))
  (bind _returnvalue (Math|Random|RandomIntegerinRangefromStream Stream 0 90))
  (if (< _returnvalue 10)
    _
    (else
      (Transformation|AddLocalRotation Target (Math|Rotator|MakeRotator 0.0 (Math|Conversions|ToFloat(Integer) _returnvalue) 0.0) false false)))
  (return))

(fn AngleX
  (params (Stream :type Random%20Stream%20Structure%20%28by%20ref%29) (Target :type Scene%20Component%20Object%20Reference))
  (bind _returnvalue (Math|Random|RandomIntegerinRangefromStream Stream 0 90))
  (bind _returnvalue_2 (Math|Conversions|ToFloat(Integer) _returnvalue))
  (if (<= _returnvalue 10)
    _
    (else
      (Transformation|AddLocalRotation Target (Math|Rotator|MakeRotator _returnvalue_2 0.0 0.0) false false)
      (Variables|Default|SetAngle1 _returnvalue_2)))
  (return))

(fn Angle-X
  (params (Stream :type Random%20Stream%20Structure%20%28by%20ref%29) (Target :type Scene%20Component%20Object%20Reference))
  (bind _returnvalue (Math|Random|RandomIntegerinRangefromStream Stream 0 90))
  (if (< _returnvalue 10)
    (Transformation|AddLocalRotation Target (Math|Rotator|MakeRotator (* (Math|Conversions|ToFloat(Integer) _returnvalue) -1.0) 0.0 0.0) false false)
    (return)))

(fn Angle-Y
  (params (Stream :type Random%20Stream%20Structure%20%28by%20ref%29) (Target :type Scene%20Component%20Object%20Reference))
  (bind _returnvalue (Math|Random|RandomIntegerinRangefromStream Stream 0 90))
  (if (< _returnvalue 10)
    _
    (else
      (Transformation|AddLocalRotation Target (Math|Rotator|MakeRotator 0.0 (* (Math|Conversions|ToFloat(Integer) _returnvalue) -1.0) 0.0) false false)))
  (return))