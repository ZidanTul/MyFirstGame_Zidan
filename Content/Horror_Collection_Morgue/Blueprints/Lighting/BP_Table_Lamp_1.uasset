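; Configurable table lamp prop with a spotlight and an optional fake light-shaft mesh, set up entirely in the Construction Script.
; MainPitch tilts the lamp top and counter-rotates a second element at four times the angle.
; On and LightShaftOn control visibility, while color and intensity drive the spotlight and shaft material, alongside fog and length parameters.
; Switching off hides light and shaft but still applies LightColor to the lamp's emissive material.
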(event EventBeginPlay)

(event Collision|EventActorBeginOverlap
  (params (OtherActor :type Actor%20Object%20Reference)))

(event EventTick
  (params (DeltaSeconds :type Float%20%28single-precision%29)))

(fn ConstructionScript
  (bind _main_pitch (Variables|Default|GetMain%20Pitch))
  (bind _staticmesh (Variables|Default|GetStaticMesh))
  (bind _staticmesh_2 (Variables|Default|GetStaticMesh))
  (bind _lightcolor (Variables|Default|GetLightColor))
  (bind _lightcolor_2 (Variables|Default|GetLightColor))
  (bind _light_intensity (Variables|Default|GetLight%20Intensity))
  (bind _spotlight (Variables|Default|GetSpotLight))
  (bind _spotlight_2 (Variables|Default|GetSpotLight))
  (bind _returnvalue (Math|Conversions|ToVector(LinearColor) _lightcolor))
  (Transformation|SetRelativeRotation (Variables|Default|GetSM_Table_Lamp_top) (Math|Rotator|MakeRotator 0.0 _main_pitch 0.0) false false)
  (Transformation|SetRelativeRotation (Variables|Default|GetSM_Table_Lamp_1_element_1) (Math|Rotator|MakeRotator 0.0 (* _main_pitch -4.0) 0.0) false false)
  (if (Variables|Default|Get?On)
    (Rendering|SetVisibility _staticmesh_2 true false)
    (if (Variables|Default|Get?LightShaftOn)
      (Rendering|SetVisibility (Variables|Default|GetStaticMesh) true false)
      (Rendering|Components|Light|SetIntensity _spotlight_2 _light_intensity)
      (Rendering|Material|SetVectorParameterValueonMaterials (Variables|Default|GetSM_Lamp_Floor_1_element_6) "EmissiveColor" _returnvalue)
      (Rendering|Material|SetVectorParameterValueonMaterials (Variables|Default|GetStaticMesh) "ShaftColor" _returnvalue)
      (Rendering|Components|Light|SetLightColor _spotlight_2 _lightcolor true)
      (Rendering|Material|SetScalarParameterValueonMaterials (Variables|Default|GetStaticMesh) "Emissive" (/ _light_intensity 3e+02))
      (Rendering|Material|SetScalarParameterValueonMaterials _staticmesh "Foggy" (Variables|Default|GetFoggy))
      (Rendering|Material|SetScalarParameterValueonMaterials _staticmesh "ShaftLenght" (Variables|Default|GetShaftLenght))
      (else
        (Rendering|SetVisibility (Variables|Default|GetStaticMesh) false false :!label _label)
        (Rendering|Components|Light|SetIntensity _spotlight (Variables|Default|GetLight%20Intensity))
        (Rendering|Material|SetVectorParameterValueonMaterials (Variables|Default|GetSM_Lamp_Floor_1_element_6) "EmissiveColor" (Math|Conversions|ToVector(LinearColor) _lightcolor_2))
        (Rendering|Components|Light|SetLightColor _spotlight _lightcolor_2 true)))
    (else
      (Rendering|SetVisibility _staticmesh_2 false false)
      (goto _label))))