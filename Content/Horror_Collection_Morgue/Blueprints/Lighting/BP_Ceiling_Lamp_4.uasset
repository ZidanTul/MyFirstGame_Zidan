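; Configurable ceiling lamp prop for the morgue environment, set up entirely in the Construction Script with no runtime logic.
; AddWiresLength stretches the wire by adding to the Z scale of SMWireSpline and StaticMesh.
; The Light toggle sets SpotLight visibility, propagated to its children.
; When on, LightColor tints both SpotLight and PointLight, and LightIntensity drives the spot, with the point light at one third strength.
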(event EventBeginPlay)

(event Collision|EventActorBeginOverlap
  (params (OtherActor :type Actor%20Object%20Reference)))

(event EventTick
  (params (DeltaSeconds :type Float%20%28single-precision%29)))

(fn ConstructionScript
  (bind _spotlight (Variables|Default|GetSpotLight))
  (bind _sm_wire_spline (Variables|Default|GetSM_wire_spline))
  (bind _light_intensity (Variables|Default|GetLight_Intensity))
  (bind _relativescale3d (Variables|/Script/Engine.SceneComponent|GetRelativeScale3D _sm_wire_spline))
  (bind (_x _y _z) (Math|Vector|BreakVector _relativescale3d))
  (Transformation|SetRelativeScale3D (Variables|Default|GetStaticMesh) (Math|Vector|MakeVector _x _y (+ _z (Variables|Default|GetAdd_Wires_Length))))
  (if (Variables|Default|Get?Light)
    (Rendering|SetVisibility _spotlight true true)
    (Rendering|Components|Light|SetIntensity (Variables|Default|GetSpotLight) _light_intensity)
    (Rendering|Components|Light|SetIntensity (Variables|Default|GetPointLight) (/ _light_intensity 3.0))
    (Rendering|Components|Light|SetLightColor (Variables|Default|GetSpotLight) (Variables|Default|GetLight_Color) true)
    (else
      (Rendering|SetVisibility _spotlight false true))))