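; Configurable four-light operating lamp prop for a morgue scene, with adjustable arm rotations, optional light shafts and flicker.
; The construction script poses the lamp, toggles each emissive component with its children, and applies intensity, color and shaft settings to spotlights and materials.
; When Flicker is enabled, Tick plays a timeline that varies spotlight intensity around the base value, scaling shaft and bulb emissive material parameters to match.
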(event EventTick
  (params (DeltaSeconds :type Float%20%28single-precision%29))
  (bind _lightintensity (Variables|Base|GetLightIntensity))
  (if (Variables|LightCustomize|Get?Flicker)
    (bind _flick (Timeline|Timeline_0 Play)
      (:Update
        (bind _output_get (Variables|Default|SetMinInt (- _lightintensity 5e+02)))
        (bind _output_get_2 (Variables|Default|SetMaxInt (+ _lightintensity 5e+02)))
        (Rendering|Components|Light|SetIntensity (Variables|Default|GetSpotLight) (Math|Float|Lerp _output_get _output_get_2 _flick))
        (Rendering|Material|SetScalarParameterValueonMaterials (Variables|Default|GetStaticMesh1) "Emissive" (/ (Math|Float|Lerp _output_get _output_get_2 _flick) 3.6e+02))
        (Rendering|Material|SetScalarParameterValueonMaterials (Variables|Default|GetEmissive1) "EmissiveIntensity" (/ (Math|Float|Lerp _output_get _output_get_2 _flick) 1.93e+03))))))

(fn ConstructionScript
  (bind _lightcolor (Variables|Base|GetLightColor))
  (bind _staticmesh1 (Variables|Default|GetStaticMesh1))
  (bind _emissive1 (Variables|Default|GetEmissive1))
  (bind _returnvalue (Math|Conversions|ToVector(LinearColor) _lightcolor))
  (Transformation|SetRelativeRotation (Variables|Default|GetSM_Operation_Lamp_2_element_2) (Math|Rotator|MakeRotator (Variables|Base|GetMainRoll) 0.0 0.0) false false)
  (Transformation|SetRelativeRotation (Variables|Default|GetOperation_Lamp_Element_3) (Math|Rotator|MakeRotator 0.0 (Variables|Base|GetLampRoll) 0.0) false false)
  (Transformation|SetRelativeRotation (Variables|Default|GetSM_Operation_Lamp_2_element_4) (Math|Rotator|MakeRotator (Variables|Base|GetMainPitch) 0.0 0.0) false false)
  (if (Variables|Base|Get?On)
    (Rendering|SetVisibility _emissive1 true true)
    (Rendering|SetVisibility (Variables|Default|GetEmissive1) (Variables|LightCustomize|Get?On1) true)
    (Rendering|SetVisibility (Variables|Default|GetEmissive2) (Variables|LightCustomize|Get?On2) true)
    (Rendering|SetVisibility (Variables|Default|GetEmissive3) (Variables|LightCustomize|Get?On3) true)
    (Rendering|SetVisibility (Variables|Default|GetEmissive4) (Variables|LightCustomize|Get?On4) true)
    (if (Variables|Base|Get?LighShaftOn)
      (Rendering|Components|Light|SetIntensity (Variables|Default|GetSpotLight) (Variables|Base|GetLightIntensity))
      (Rendering|Components|Light|SetLightColor (Variables|Default|GetSpotLight) _lightcolor true)
      (Rendering|Material|SetVectorParameterValueonMaterials (Variables|Default|GetEmissive3) "EmissiveColor" _returnvalue)
      (Rendering|Material|SetVectorParameterValueonMaterials (Variables|Default|GetStaticMesh1) "ShaftColor" _returnvalue)
      (Rendering|Material|SetScalarParameterValueonMaterials _staticmesh1 "Emissive" (/ (Variables|Base|GetLightIntensity) 3e+02))
      (Rendering|Material|SetScalarParameterValueonMaterials _staticmesh1 "Foggy" (Variables|LightShaft|GetFoggy))
      (Rendering|Material|SetScalarParameterValueonMaterials _staticmesh1 "ShaftLenght" (Variables|LightShaft|GetShaftLenght))
      (else
        (Rendering|SetVisibility (Variables|Default|GetStaticMesh2) false false)
        (Rendering|Components|Light|SetIntensity (Variables|Default|GetSpotLight) (Variables|Base|GetLightIntensity))
        (Rendering|Material|SetVectorParameterValueonMaterials (Variables|Default|GetEmissive3) "EmissiveColor" (Math|Conversions|ToVector(LinearColor) (Variables|Base|GetLightColor)))))
    (else
      (Rendering|SetVisibility _emissive1 false true))))