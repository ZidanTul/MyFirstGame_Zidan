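; Configurable surgical operation lamp prop for the morgue environment, built entirely in the Construction Script with no runtime logic.
; Exposed yaw, pitch, roll, height and length variables pose the articulated arm by rotating and offsetting its mesh elements.
; A master switch and three per-bulb toggles control emissive visibility, propagated to children.
; Shared color and intensity drive three spotlights, emissive materials and optional fake light-shaft meshes, whose materials also take fog and length parameters.
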(event EventBeginPlay)

(event Collision|EventActorBeginOverlap
  (params (OtherActor :type Actor%20Object%20Reference)))

(event EventTick
  (params (DeltaSeconds :type Float%20%28single-precision%29)))

(fn ConstructionScript
  (bind _lightcolor (Variables|Base|GetLightColor))
  (bind _staticmesh2 (Variables|Default|GetStaticMesh2))
  (bind _lightcolor_2 (Variables|Base|GetLightColor))
  (bind _emissive2 (Variables|Default|GetEmissive2))
  (bind _returnvalue (Math|Conversions|ToVector(LinearColor) _lightcolor_2))
  (Transformation|SetRelativeRotation (Variables|Default|GetSM_Operation_Lamp_1_element_2) (Math|Rotator|MakeRotator 0.0 0.0 (Variables|Base|GetMainYaw)) false false)
  (Transformation|AddLocalOffset (Variables|Default|GetSM_Operation_Lamp_1_element_4) (Math|Vector|MakeVector 0.0 0.0 (Variables|Base|GetHeight)) false false)
  (Transformation|SetRelativeRotation (Variables|Default|GetSM_Operation_Lamp_1_element_5) (Math|Rotator|MakeRotator (Variables|Base|GetMainPitch) 0.0 0.0) false false)
  (Transformation|AddLocalOffset (Variables|Default|GetSM_Operation_Lamp_1_element_6) (Math|Vector|MakeVector 0.0 (Variables|Base|GetLampLenght) 0.0) false false)
  (Transformation|SetRelativeRotation (Variables|Default|GetSM_Operation_Lamp_1_element_6) (Math|Rotator|MakeRotator 0.0 (Variables|Base|GetLampRoll) 0.0) false false)
  (Transformation|SetRelativeRotation (Variables|Default|GetSM_Operation_Lamp_1_element_7) (Math|Rotator|MakeRotator (Variables|Base|GetLampPitch) 0.0 0.0) false false)
  (if (Variables|Base|Get?On)
    (Rendering|SetVisibility _emissive2 true true)
    (Rendering|SetVisibility (Variables|Default|GetEmissive1) (Variables|LightCustomize|Get?On1) true)
    (Rendering|SetVisibility (Variables|Default|GetEmissive2) (Variables|LightCustomize|Get?On2) true)
    (Rendering|SetVisibility (Variables|Default|GetEmissive3) (Variables|LightCustomize|Get?On3) true)
    (if (Variables|Base|Get?LightShaftOn)
      (Rendering|Components|Light|SetIntensity (Variables|Default|GetSpotLight2) (Variables|Base|GetLightIntensity))
      (Rendering|Components|Light|SetLightColor (Variables|Default|GetSpotLight1) _lightcolor_2 true)
      (Rendering|Material|SetVectorParameterValueonMaterials (Variables|Default|GetEmissive2) "EmissiveColor" _returnvalue)
      (Rendering|Material|SetVectorParameterValueonMaterials (Variables|Default|GetStaticMesh1) "ShaftColor" _returnvalue)
      (Rendering|Material|SetScalarParameterValueonMaterials _staticmesh2 "Emissive" (/ (Variables|Base|GetLightIntensity) 3e+02))
      (Rendering|Material|SetScalarParameterValueonMaterials _staticmesh2 "Foggy" (Variables|LightShaft|GetFoggy))
      (Rendering|Material|SetScalarParameterValueonMaterials _staticmesh2 "ShaftLenght" (Variables|LightShaft|GetShaftLenght))
      (else
        (Rendering|SetVisibility (Variables|Default|GetStaticMesh2) false false)
        (Rendering|Components|Light|SetIntensity (Variables|Default|GetSpotLight2) (Variables|Base|GetLightIntensity))
        (Rendering|Material|SetVectorParameterValueonMaterials (Variables|Default|GetEmissive2) "EmissiveColor" (Math|Conversions|ToVector(LinearColor) _lightcolor))
        (Rendering|Components|Light|SetLightColor (Variables|Default|GetSpotLight3) _lightcolor true)))
    (else
      (Rendering|SetVisibility _emissive2 false true))))