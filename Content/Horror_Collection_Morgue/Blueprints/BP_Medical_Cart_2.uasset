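; Configurable medical cart prop from the morgue collection, posed entirely in the Construction Script with no active runtime logic.
; Variables slide the drawer along X, yaw the two doors and four wheel elements, and toggle the cloth mesh's visibility.
; The RotateZ and PositionX helpers take a flag that negates the value, mirroring Door2 against Door1.
; PositionX offsets from the drawer's current relative location, while RotateZ sets absolute relative yaw.
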(event EventBeginPlay)

(event Collision|EventActorBeginOverlap
  (params (OtherActor :type Actor%20Object%20Reference)))

(event EventTick
  (params (DeltaSeconds :type Float%20%28single-precision%29)))

(fn ConstructionScript
  (CallFunction|PositionX (Variables|Default|GetDrawer1) true (Variables|Default|GetDrawer))
  (CallFunction|RotateZ (Variables|Doors|GetDoor1) false (Variables|Default|GetDoor_1))
  (CallFunction|RotateZ (Variables|Doors|GetDoor2) true (Variables|Default|GetDoor_2))
  (Rendering|SetVisibility (Variables|Default|GetSM_Medical_Cart_2_cloth) (Variables|Default|Get?%20Hide\Unhide%20Cloth) false)
  (CallFunction|RotateZ (Variables|WheelRotation|GetWheel_element_1_Rotate) false (Variables|Default|GetWheel_element_1))
  (CallFunction|RotateZ (Variables|WheelRotation|GetWheel_element_2_Rotate) false (Variables|Default|GetWheel_element_2))
  (CallFunction|RotateZ (Variables|WheelRotation|GetWheel_element_3_Rotate) false (Variables|Default|GetWheel_element_3))
  (CallFunction|RotateZ (Variables|WheelRotation|GetWheel_element_4_Rotate) false (Variables|Default|GetWheel_element_4)))

(fn RotateZ
  (params (Z%20%28Yaw%29 :type Float%20%28double-precision%29) (RotateZ :type Boolean) (TargetMesh :type Scene%20Component%20Object%20Reference))
  (if RotateZ
    (Transformation|SetRelativeRotation TargetMesh (Math|Rotator|MakeRotator 0.0 0.0 (* Z%20%28Yaw%29 -1.0)) false false)
    (else
      (Transformation|SetRelativeRotation TargetMesh (Math|Rotator|MakeRotator 0.0 0.0 Z%20%28Yaw%29) false false)))
  (return))

(fn PositionX
  (params (X :type Float%20%28double-precision%29) (Rotate%20X :type Boolean) (TargetMesh :type Scene%20Component%20Object%20Reference))
  (bind _relativelocation (Variables|/Script/Engine.SceneComponent|GetRelativeLocation TargetMesh))
  (bind (_x _y _z) (Math|Vector|BreakVector _relativelocation))
  (if Rotate%20X
    (Transformation|SetRelativeLocation TargetMesh (Math|Vector|MakeVector (+ (* X -1.0) _x) _y _z) false false)
    (else
      (Transformation|SetRelativeLocation TargetMesh (Math|Vector|MakeVector (+ X _x) _y _z) false false)))
  (return))