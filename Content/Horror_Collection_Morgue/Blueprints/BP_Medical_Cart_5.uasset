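; BP_Medical_Cart_5 is a configurable medical cart prop from the morgue horror asset collection, posed in the editor.
; The construction script calls a RotateZ helper to yaw each of four wheel elements by its own rotation variable and toggles the cloth mesh's visibility from a boolean.
; RotateZ supports an inverted yaw, though every call here leaves it off, and the event graph holds no active logic.
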(event EventBeginPlay)

(event Collision|EventActorBeginOverlap
  (params (OtherActor :type Actor%20Object%20Reference)))

(event EventTick
  (params (DeltaSeconds :type Float%20%28single-precision%29)))

(fn ConstructionScript
  (CallFunction|RotateZ (Variables|WheelsRotation|GetWheel_element_1_Rotate) false (Variables|Default|GetWheel_element_1))
  (CallFunction|RotateZ (Variables|WheelsRotation|GetWheel_element_2_Rotate) false (Variables|Default|GetWheel_element_2))
  (CallFunction|RotateZ (Variables|WheelsRotation|GetWheel_element_3_Rotate) false (Variables|Default|GetWheel_element_3))
  (CallFunction|RotateZ (Variables|WheelsRotation|GetWheel_element_4_Rotate) false (Variables|Default|GetWheel_element_4))
  (Rendering|SetVisibility (Variables|Default|GetSM_Medical_Cart_5_cloth) (Variables|Default|Get?%20Hide\Unhide%20Cloth) false))

(fn RotateZ
  (params (Z%20%28Yaw%29 :type Float%20%28double-precision%29) (Invert%20Z :type Boolean) (TargetMesh :type Scene%20Component%20Object%20Reference))
  (if Invert%20Z
    (Transformation|SetRelativeRotation TargetMesh (Math|Rotator|MakeRotator 0.0 0.0 (* Z%20%28Yaw%29 -1.0)) false false)
    (else
      (Transformation|SetRelativeRotation TargetMesh (Math|Rotator|MakeRotator 0.0 0.0 Z%20%28Yaw%29) false false)))
  (return))