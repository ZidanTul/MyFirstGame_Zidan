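; BP_Folding_Screen is a configurable folding screen prop from the morgue collection, set up entirely in the construction script.
; An Angle variable yaws the second screen panel.
; FoldFunc fakes drawing each of the two cloths by scaling it along X to a fold percentage, then offsetting it by half the lost width, with a flip flag choosing the side.
; The event graph holds no logic.
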(event EventBeginPlay)

(event Collision|EventActorBeginOverlap
  (params (OtherActor :type Actor%20Object%20Reference)))

(event EventTick
  (params (DeltaSeconds :type Float%20%28single-precision%29)))

(fn ConstructionScript
  (Transformation|AddLocalRotation (Variables|Default|GetSM_Folding_Screen_second) (Math|Rotator|MakeRotator 0.0 0.0 (Variables|Base|GetAngle)) false false)
  (CallFunction|FoldFunc (Variables|Default|GetSM_Folding_Screen_cloth_1_1) (Variables|Base|GetFold_1st_Screen) (Variables|Base|GetFlip_1st_Screen))
  (CallFunction|FoldFunc (Variables|Default|GetSM_Folding_Screen_cloth_1) (Variables|Base|GetFold_2nd_tScreen) (Variables|Base|GetFlip_2nd_Screen)))

(fn FoldFunc
  (params (Actor :type Scene%20Component%20Object%20Reference) (Fold :type Float%20%28double-precision%29) (Flip :type Boolean))
  (bind _returnvalue (- 1e+02 Fold))
  (Transformation|SetWorldScale3D Actor (Math|Vector|MakeVector (* Fold 0.01) 1.0 1.0))
  (if Flip
    (Transformation|AddLocalOffset Actor (Math|Vector|MakeVector (* _returnvalue -0.5) 0.0 0.0) false false)
    (else
      (Transformation|AddLocalOffset Actor (Math|Vector|MakeVector (* _returnvalue 0.5) 0.0 0.0) false false))))