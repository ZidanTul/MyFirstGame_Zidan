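; Configurable wall-mounted autopsy station prop for a morgue, set up entirely in the Construction Script with no active runtime logic.
; Boolean options toggle the scale (Libra), hoses and four plates, while small axis helper functions with invert flags slide plates and drawers and rotate the faucet and taps.
; A lamp mode enum switches the two spotlights and sets their intensities, driving the paired point lights at a third of each lamp's value.
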(event EventBeginPlay)

(event Collision|EventActorBeginOverlap
  (params (OtherActor :type Actor%20Object%20Reference)))

(event EventTick
  (params (DeltaSeconds :type Float%20%28single-precision%29)))

(fn ConstructionScript
  (bind _libra (Variables|Default|GetLibra))
  (bind _hose_2 (Variables|Default|GetHose_2))
  (bind _spotlight1 (Variables|Default|GetSpotLight1))
  (bind _plates_2 (Variables|Default|GetPlates_2))
  (bind _plates_3 (Variables|Default|GetPlates_3))
  (bind _plates_4 (Variables|Default|GetPlates_4))
  (bind _spotlight2 (Variables|Default|GetSpotLight2))
  (bind _plates_1 (Variables|Default|GetPlates_1))
  (bind _spotlight2_2 (Variables|Default|GetSpotLight2))
  (bind _lamp_1_intensity (Variables|Lights|GetLamp_1_intensity))
  (bind _lamp_1_intensity_2 (Variables|Lights|GetLamp_1_intensity))
  (bind _lamp_2_intensity (Variables|Lights|GetLamp_2_intensity))
  (bind _lamp_2_intensity_2 (Variables|Lights|GetLamp_2_intensity))
  (if (Variables|Default|Get?%20Libra)
    (Rendering|SetVisibility _libra true true)
    (else
      (Rendering|SetVisibility _libra false true)))
  (if (Variables|Default|Get?%20Hoses)
    (Rendering|SetVisibility _hose_2 true true)
    (else
      (Rendering|SetVisibility _hose_2 false true)))
  (if (Variables|Plates|Get?%20Plate_1)
    (Rendering|SetVisibility _plates_1 true true)
    (else
      (Rendering|SetVisibility _plates_1 false true)))
  (if (Variables|Plates|Get?%20Plate_2)
    (Rendering|SetVisibility _plates_2 true true)
    (else
      (Rendering|SetVisibility _plates_2 false true)))
  (if (Variables|Plates|Get?%20Plate_3)
    (Rendering|SetVisibility _plates_3 true true)
    (else
      (Rendering|SetVisibility _plates_3 false true)))
  (if (Variables|Plates|Get?%20Plate_4)
    (Rendering|SetVisibility _plates_4 true true)
    (else
      (Rendering|SetVisibility _plates_4 false true)))
  (CallFunction|PositionX (Variables|Plates|GetMovePlate_1st) false (Variables|Default|GetPlates_1))
  (CallFunction|PositionX (Variables|Plates|GetMovePlate_2nd) true (Variables|Default|GetPlates_2))
  (CallFunction|PositionX (Variables|Plates|GetMovePlate_3rd) true (Variables|Default|GetPlates_3))
  (CallFunction|PositionX (Variables|Plates|GetMovePlate%204th) false (Variables|Default|GetPlates_4))
  (CallFunction|PositionY (Variables|Drawers|GetDrawer1) false (Variables|Default|GetDrawer_1))
  (CallFunction|PositionY (Variables|Drawers|GetDrawer2) false (Variables|Default|GetDrawer_2))
  (CallFunction|RotateZ (Variables|Taps|GetFaucet_tap) false (Variables|Default|GetFaucet))
  (CallFunction|RotateY (Variables|Taps|GetTap1) false (Variables|Default|GetTap_1))
  (CallFunction|RotateY (Variables|Taps|GetTap2) false (Variables|Default|GetTap_2))
  (CallFunction|RotateX (Variables|Taps|GetTap3) true (Variables|Default|GetTap_3))
  (CallFunction|RotateX (Variables|Taps|GetTap4) true (Variables|Default|GetTap_4))
  (CallFunction|RotateZ (Variables|Taps|GetTap5) true (Variables|Default|GetTap_5))
  (CallFunction|RotateZ (Variables|Taps|GetTap6) false (Variables|Default|GetTap_6))
  (switch Utilities|FlowControl|Switch|SwitchonBP_Wall_Mount_Autopsy_Station_Enum (Variables|Lights|GetWall_Station_Lights:)
    (:NewEnumerator0
      (Rendering|SetVisibility _spotlight2_2 true true)
      (Rendering|Components|Light|SetIntensity (Variables|Default|GetSpotLight1) _lamp_1_intensity_2)
      (Rendering|Components|Light|SetIntensity _spotlight2_2 _lamp_2_intensity)
      (Rendering|Components|Light|SetIntensity (Variables|Default|GetPointLight1) (/ _lamp_1_intensity_2 3.0))
      (Rendering|Components|Light|SetIntensity (Variables|Default|GetPointLight2) (/ _lamp_2_intensity 3.0)))
    (:NewEnumerator1
      (Rendering|SetVisibility (Variables|Default|GetSpotLight2) false true)
      (Rendering|SetVisibility _spotlight1 true true)
      (Rendering|Components|Light|SetIntensity _spotlight1 _lamp_1_intensity)
      (Rendering|Components|Light|SetIntensity (Variables|Default|GetPointLight1) (/ _lamp_1_intensity 3.0)))
    (:NewEnumerator2
      (Rendering|SetVisibility (Variables|Default|GetSpotLight1) false true)
      (Rendering|SetVisibility _spotlight2 true true)
      (Rendering|Components|Light|SetIntensity _spotlight2 _lamp_2_intensity_2)
      (Rendering|Components|Light|SetIntensity (Variables|Default|GetPointLight2) (/ _lamp_2_intensity_2 3.0)))
    (:NewEnumerator3
      (Rendering|SetVisibility (Variables|Default|GetSpotLight2) false true))))

(fn RotateZ
  (params (Z%20%28Yaw%29 :type Float%20%28double-precision%29) (InvertZ :type Boolean) (TargetMesh :type Scene%20Component%20Object%20Reference))
  (if InvertZ
    (Transformation|SetRelativeRotation TargetMesh (Math|Rotator|MakeRotator 0.0 0.0 (* Z%20%28Yaw%29 -1.0)) false false)
    (else
      (Transformation|SetRelativeRotation TargetMesh (Math|Rotator|MakeRotator 0.0 0.0 Z%20%28Yaw%29) false false)))
  (return))

(fn PositionX
  (params (X :type Float%20%28double-precision%29) (InvertX :type Boolean) (TargetMesh :type Scene%20Component%20Object%20Reference))
  (bind _relativelocation (Variables|/Script/Engine.SceneComponent|GetRelativeLocation TargetMesh))
  (bind (_x _y _z) (Math|Vector|BreakVector _relativelocation))
  (if InvertX
    (Transformation|SetRelativeLocation TargetMesh (Math|Vector|MakeVector (+ (* X -1.0) _x) _y _z) false false)
    (else
      (Transformation|SetRelativeLocation TargetMesh (Math|Vector|MakeVector (+ X _x) _y _z) false false)))
  (return))

(fn PositionY
  (params (Y :type Float%20%28double-precision%29) (InvertY :type Boolean) (TargetMesh :type Scene%20Component%20Object%20Reference))
  (bind _relativelocation (Variables|/Script/Engine.SceneComponent|GetRelativeLocation TargetMesh))
  (bind (_x _y _z) (Math|Vector|BreakVector _relativelocation))
  (if InvertY
    (Transformation|SetRelativeLocation TargetMesh (Math|Vector|MakeVector _x (+ (* Y -1.0) 0.0) _z) false false)
    (else
      (Transformation|SetRelativeLocation TargetMesh (Math|Vector|MakeVector _x (+ Y _y) _z) false false)))
  (return))

(fn RotateY
  (params (Y%20%28Pitch%29 :type Float%20%28double-precision%29) (InvertY :type Boolean) (TargetMesh :type Scene%20Component%20Object%20Reference))
  (if InvertY
    (Transformation|SetRelativeRotation TargetMesh (Math|Rotator|MakeRotator 0.0 (* Y%20%28Pitch%29 -1.0) 0.0) false false)
    (else
      (Transformation|SetRelativeRotation TargetMesh (Math|Rotator|MakeRotator 0.0 Y%20%28Pitch%29 0.0) false false)))
  (return))

(fn RotateX
  (params (X%20%28Roll%29 :type Float%20%28double-precision%29) (InvertX :type Boolean) (TargetMesh :type Scene%20Component%20Object%20Reference))
  (if InvertX
    (Transformation|SetRelativeRotation TargetMesh (Math|Rotator|MakeRotator (* X%20%28Roll%29 -1.0) 0.0 0.0) false false)
    (else
      (Transformation|SetRelativeRotation TargetMesh (Math|Rotator|MakeRotator X%20%28Roll%29 0.0 0.0) false false)))
  (return))