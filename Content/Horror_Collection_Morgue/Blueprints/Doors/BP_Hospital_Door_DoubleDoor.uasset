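; Configurable hospital double-door prop for the morgue environment, set up entirely in the Construction Script with no runtime behaviour.
; The Open flag poses both leaves and their sub-meshes at fixed rotations.
; DoorColor, WindowFrameColor and FrameColor drive the CustomColor parameter, using dynamic material instances where slots need different colors.
; WindowStyle shows one paired panel variant (Solid, Long, Medium or Short) and hides the rest.
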(event EventBeginPlay)

(event Collision|EventActorBeginOverlap
  (params (OtherActor :type Actor%20Object%20Reference)))

(event EventTick
  (params (DeltaSeconds :type Float%20%28single-precision%29)))

(fn ConstructionScript
  (bind _windowframe_color (Variables|Default|GetWindowFrame%20Color))
  (bind _doorcolor (Variables|Default|GetDoorColor))
  (bind _sm_doorsingler_intframe31 (Variables|Default|GetSM_DoorSingler_IntFrame31))
  (bind _sm_doorsingler_intframe0 (Variables|Default|GetSM_DoorSingler_IntFrame0))
  (if (Variables|Default|Get?Open)
    (Transformation|SetRelativeRotation (Variables|Default|GetSM_DoorDouble_Doorl_low) "0,-110.000000, 0" false false)
    (Transformation|SetRelativeRotation (Variables|Default|GetSM_DoorDouble_M2) "0,-50.000000, 0" false false)
    (Transformation|SetRelativeRotation (Variables|Default|GetSM_DoorDouble_M1) "0,121.000000, 0" false false)
    (Transformation|SetRelativeRotation (Variables|Default|GetSM_DoorDouble_Doorr_low) "0,110.000000, 0" false false)
    (Transformation|SetRelativeRotation (Variables|Default|GetSM_DoorDoubleR_M2) "0,50.000000, 0" false false)
    (Transformation|SetRelativeRotation (Variables|Default|GetSM_DoorDoubler_M1) "0,-121.000000, 0" false false))
  (Rendering|Material|SetVectorParameterValueonMaterials (Variables|Default|GetSM_DoorSingle_IntFrame0) "CustomColor" (Math|Conversions|ToVector(LinearColor) _doorcolor))
  (bind _returnvalue (Rendering|Material|CreateDynamicMaterialInstance (Variables|Default|GetSM_DoorSingle_IntFrame21) 1 0 "None" :!class /Script/Engine.PrimitiveComponent))
  (bind _returnvalue_2 (Rendering|Material|CreateDynamicMaterialInstance (Variables|Default|GetSM_DoorSingle_IntFrame11) 1 0 "None" :!class /Script/Engine.PrimitiveComponent))
  (bind _returnvalue_3 (Rendering|Material|CreateDynamicMaterialInstance (Variables|Default|GetSM_DoorSingler_IntFrame11) 1 0 "None" :!class /Script/Engine.PrimitiveComponent))
  (bind _returnvalue_4 (Rendering|Material|CreateDynamicMaterialInstance (Variables|Default|GetSM_DoorSingler_IntFrame21) 1 0 "None" :!class /Script/Engine.PrimitiveComponent))
  (Rendering|Material|SetVectorParameterValue _returnvalue "CustomColor" _doorcolor :!class /Script/Engine.MaterialInstanceDynamic)
  (bind _returnvalue_5 (Rendering|Material|CreateDynamicMaterialInstance (Variables|Default|GetSM_DoorSingler_IntFrame21) 0 0 "None" :!class /Script/Engine.PrimitiveComponent))
  (bind _returnvalue_6 (Rendering|Material|CreateDynamicMaterialInstance (Variables|Default|GetSM_DoorSingle_IntFrame11) 0 0 "None" :!class /Script/Engine.PrimitiveComponent))
  (bind _returnvalue_7 (Rendering|Material|CreateDynamicMaterialInstance (Variables|Default|GetSM_DoorSingle_IntFrame21) 0 0 "None" :!class /Script/Engine.PrimitiveComponent))
  (bind _returnvalue_8 (Rendering|Material|CreateDynamicMaterialInstance (Variables|Default|GetSM_DoorSingler_IntFrame11) 0 0 "None" :!class /Script/Engine.PrimitiveComponent))
  (Rendering|Material|SetVectorParameterValue _returnvalue_5 "CustomColor" _windowframe_color :!class /Script/Engine.MaterialInstanceDynamic)
  (Rendering|Material|SetVectorParameterValueonMaterials (Variables|Default|GetSM_DoorSingle_IntFrame31) "CustomColor" (Math|Conversions|ToVector(LinearColor) _windowframe_color))
  (Rendering|Material|SetVectorParameterValueonMaterials (Variables|Default|GetSM_DoorSingle_Frame) "CustomColor" (Math|Conversions|ToVector(LinearColor) (Variables|Default|GetFrame%20Color)))
  (switch Utilities|FlowControl|Switch|SwitchonE_Door_Windows_Enum (Variables|Default|GetWindowStyle)
    (:NewEnumerator0
      (Rendering|SetVisibility _sm_doorsingler_intframe31 false true)
      (Rendering|SetVisibility _sm_doorsingler_intframe0 true true))
    (:NewEnumerator1
      (Rendering|SetVisibility _sm_doorsingler_intframe0 false true)
      (Rendering|SetVisibility _sm_doorsingler_intframe31 true true))
    (:NewEnumerator2
      (Rendering|SetVisibility _sm_doorsingler_intframe0 false true)
      (Rendering|SetVisibility (Variables|Default|GetSM_DoorSingle_IntFrame21) true true))
    (:NewEnumerator3
      (Rendering|SetVisibility (Variables|Default|GetSM_DoorSingle_IntFrame0) false true)
      (Rendering|SetVisibility (Variables|Default|GetSM_DoorSingler_IntFrame11) true true))))