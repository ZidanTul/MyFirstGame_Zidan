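; Fuse box prop for the morgue environment, with a door and lock posed at construction time and no active gameplay logic.
; When DoorLock is set, the construction script zeroes both angle variables and hides a large set of static meshes without applying rotations.
; Otherwise it shows those meshes only if DoorOpenClose is above near-zero, then yaws Door by that value and pitches Lock to open, using two rotation helpers.
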(event EventBeginPlay)

(event Collision|EventActorBeginOverlap
  (params (OtherActor :type Actor%20Object%20Reference)))

(event EventTick
  (params (DeltaSeconds :type Float%20%28single-precision%29)))

(fn ConstructionScript
  (bind _staticmesh (Variables|Default|GetStaticMesh))
  (if (Variables|Default|GetDoor_Lock)
    (Variables|Default|SetDoor_Open/Close 0.0)
    (Variables|Default|SetLock_Open/Close 0.0)
    (Rendering|SetVisibility (Variables|Default|GetStaticMesh) false true)
    (else
      (if (> (Variables|Default|GetDoor_Open/Close) 0.01)
        (Rendering|SetVisibility _staticmesh true true)
        (else
          (Rendering|SetVisibility _staticmesh false true)))
      (Variables|Default|SetLock_Open/Close 9e+01)
      (CallFunction|RotateZ (Variables|Default|GetDoor_Open/Close) false (Variables|Default|GetDoor))
      (CallFunction|RotateY (Variables|Default|GetLock_Open/Close) false (Variables|Default|GetLock)))))

(fn RotateY
  (params (Y%20%28Pitch%29 :type Float%20%28double-precision%29) (Invert%20Y :type Boolean) (TargetMesh :type Scene%20Component%20Object%20Reference))
  (if Invert%20Y
    (Transformation|SetRelativeRotation TargetMesh (Math|Rotator|MakeRotator 0.0 (* Y%20%28Pitch%29 -1.0) 0.0) false false)
    (else
      (Transformation|SetRelativeRotation TargetMesh (Math|Rotator|MakeRotator 0.0 Y%20%28Pitch%29 0.0) false false)))
  (return))

(fn RotateZ
  (params (Z%20%28Yaw%29 :type Float%20%28double-precision%29) (Invert%20Z :type Boolean) (TargetMesh :type Scene%20Component%20Object%20Reference))
  (if Invert%20Z
    (Transformation|SetRelativeRotation TargetMesh (Math|Rotator|MakeRotator 0.0 0.0 (* Z%20%28Yaw%29 -1.0)) false false)
    (else
      (Transformation|SetRelativeRotation TargetMesh (Math|Rotator|MakeRotator 0.0 0.0 Z%20%28Yaw%29) false false)))
  (return))