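; BP_Fuse_Box_5 is a fuse box prop for the morgue environment with an adjustable door and optional lock, configured entirely in the Construction Script.
; When Lock is set, it shows the lock mesh, zeroes DoorOpenClose and hides a large set of static meshes.
; Otherwise it hides the lock, yaws the Door by DoorOpenClose through the RotateZ helper, and shows those meshes only when the door is open past a tiny threshold.
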(event EventBeginPlay)

(event Collision|EventActorBeginOverlap
  (params (OtherActor :type Actor%20Object%20Reference)))

(event EventTick
  (params (DeltaSeconds :type Float%20%28single-precision%29)))

(fn ConstructionScript
  (bind _staticmesh1 (Variables|Default|GetStaticMesh1))
  (if (Variables|Default|GetLock)
    (Variables|Default|SetDoor_Open/Close 0.0)
    (Rendering|SetVisibility (Variables|Default|GetLock_static) true false)
    (Rendering|SetVisibility (Variables|Default|GetStaticMesh1) false true)
    (else
      (Rendering|SetVisibility (Variables|Default|GetLock_static) false false)
      (if (> (Variables|Default|GetDoor_Open/Close) 0.01)
        (Rendering|SetVisibility _staticmesh1 true true)
        (else
          (Rendering|SetVisibility _staticmesh1 false true)))
      (CallFunction|RotateZ (Variables|Default|GetDoor_Open/Close) false (Variables|Default|GetDoor)))))

(fn RotateZ
  (params (Z%20%28Yaw%29 :type Float%20%28double-precision%29) (Invert%20Z :type Boolean) (TargetMesh :type Scene%20Component%20Object%20Reference))
  (if Invert%20Z
    (Transformation|SetRelativeRotation TargetMesh (Math|Rotator|MakeRotator 0.0 0.0 (* Z%20%28Yaw%29 -1.0)) false false)
    (else
      (Transformation|SetRelativeRotation TargetMesh (Math|Rotator|MakeRotator 0.0 0.0 Z%20%28Yaw%29) false false)))
  (return))