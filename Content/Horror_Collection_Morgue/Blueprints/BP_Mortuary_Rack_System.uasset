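; Configurable mortuary rack prop with eight rack meshes that can each be slid along local Y and shown or hidden.
; The construction script feeds per-rack move and visibility variables into the meshes, with no active runtime logic.
; A shared PositionY helper adds the offset to each mesh's current relative Y, with an optional inversion that every call leaves off.
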(event EventBeginPlay)

(event Collision|EventActorBeginOverlap
  (params (OtherActor :type Actor%20Object%20Reference)))

(event EventTick
  (params (DeltaSeconds :type Float%20%28single-precision%29)))

(fn ConstructionScript
  (CallFunction|PositionY (Variables|Movement|GetRack_1_Move) false (Variables|Default|GetRack_1))
  (CallFunction|PositionY (Variables|Movement|GetRack_2_Move) false (Variables|Default|GetRack_2))
  (CallFunction|PositionY (Variables|Movement|GetRack_3_Move) false (Variables|Default|GetRack_3))
  (CallFunction|PositionY (Variables|Movement|GetRack_4_Move) false (Variables|Default|GetRack_4))
  (CallFunction|PositionY (Variables|Movement|GetRack_5_Move) false (Variables|Default|GetRack_5))
  (CallFunction|PositionY (Variables|Movement|GetRack_6_Move) false (Variables|Default|GetRack_6))
  (CallFunction|PositionY (Variables|Movement|GetRack_7_Move) false (Variables|Default|GetRack_7))
  (CallFunction|PositionY (Variables|Movement|GetRack_8_Move) false (Variables|Default|GetRack_8))
  (Rendering|SetVisibility (Variables|Default|GetRack_1) (Variables|Visibility|GetRack_1_Visible) false)
  (Rendering|SetVisibility (Variables|Default|GetRack_2) (Variables|Visibility|GetRack_2_Visible) false)
  (Rendering|SetVisibility (Variables|Default|GetRack_3) (Variables|Visibility|GetRack_3_Visible) false)
  (Rendering|SetVisibility (Variables|Default|GetRack_4) (Variables|Visibility|GetRack_4_Visible) false)
  (Rendering|SetVisibility (Variables|Default|GetRack_5) (Variables|Visibility|GetRack_5_Visible) false)
  (Rendering|SetVisibility (Variables|Default|GetRack_6) (Variables|Visibility|GetRack_6_Visible) false)
  (Rendering|SetVisibility (Variables|Default|GetRack_7) (Variables|Visibility|GetRack_7_Visible) false)
  (Rendering|SetVisibility (Variables|Default|GetRack_8) (Variables|Visibility|GetRack_8_Visible) false))

(fn PositionY
  (params (Y :type Float%20%28double-precision%29) (Invert%20Y :type Boolean) (TargetMesh :type Scene%20Component%20Object%20Reference))
  (bind _relativelocation (Variables|/Script/Engine.SceneComponent|GetRelativeLocation TargetMesh))
  (bind (_x _y _z) (Math|Vector|BreakVector _relativelocation))
  (if Invert%20Y
    (Transformation|SetRelativeLocation TargetMesh (Math|Vector|MakeVector _x (+ (* Y -1.0) _y) _z) false false)
    (else
      (Transformation|SetRelativeLocation TargetMesh (Math|Vector|MakeVector _x (+ Y _y) _z) false false)))
  (return))