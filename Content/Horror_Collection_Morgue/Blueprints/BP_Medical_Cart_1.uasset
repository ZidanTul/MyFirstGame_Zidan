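; BP_Medical_Cart_1 is a configurable morgue medical cart prop, posed in the editor with no active gameplay logic.
; Its Construction Script slides five drawers along local X by negated offset variables, yaws four wheel elements, and toggles cloth visibility.
; Helper functions PositionX and RotateZ do the transforms, with PositionX adding to the current relative location and RotateZ overwriting the relative rotation.
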(event EventBeginPlay)

(event Collision|EventActorBeginOverlap
  (params (OtherActor :type Actor%20Object%20Reference)))

(event EventTick
  (params (DeltaSeconds :type Float%20%28single-precision%29)))

(fn ConstructionScript
  (CallFunction|PositionX (Variables|Drawers|GetDrawer1) true (Variables|Default|GetDrawer_1))
  (CallFunction|PositionX (Variables|Drawers|GetDrawer2) true (Variables|Default|GetDrawer_2))
  (CallFunction|PositionX (Variables|Drawers|GetDrawer3) true (Variables|Default|GetDrawer_3))
  (CallFunction|PositionX (Variables|Drawers|GetDrawer4) true (Variables|Default|GetDrawer_4))
  (CallFunction|PositionX (Variables|Drawers|GetDrawer5) true (Variables|Default|GetDrawer_5))
  (CallFunction|RotateZ (Variables|WheelsRotation|GetWheel_element_1_Rotate) false (Variables|Default|GetWheel_element_1))
  (CallFunction|RotateZ (Variables|WheelsRotation|GetWheel_element_2_Rotate) false (Variables|Default|GetWheel_element_2))
  (CallFunction|RotateZ (Variables|WheelsRotation|GetWheel_element_3_Rotate) false (Variables|Default|GetWheel_element_3))
  (CallFunction|RotateZ (Variables|WheelsRotation|GetWheel_element_4_Rotate) false (Variables|Default|GetWheel_element_4))
  (Rendering|SetVisibility (Variables|Default|GetSM_Medical_Cart_1_cloth) (Variables|Default|Get?%20Hide\Unhide%20Cloth) false))

(fn PositionX
  (params (X :type Float%20%28double-precision%29) (Invert%20X :type Boolean) (TargetMesh :type Scene%20Component%20Object%20Reference))
  (bind _relativelocation (Variables|/Script/Engine.SceneComponent|GetRelativeLocation TargetMesh))
  (bind (_x _y _z) (Math|Vector|BreakVector _relativelocation))
  (if Invert%20X
    (Transformation|SetRelativeLocation TargetMesh (Math|Vector|MakeVector (+ (* X -1.0) _x) _y _z) false false)
    (else
      (Transformation|SetRelativeLocation TargetMesh (Math|Vector|MakeVector (+ X _x) _y _z) false false)))
  (return))

(fn RotateZ
  (params (Z%20%28Yaw%29 :type Float%20%28double-precision%29) (Invert%20Z :type Boolean) (TargetMesh :type Scene%20Component%20Object%20Reference))
  (if Invert%20Z
    (Transformation|SetRelativeRotation TargetMesh (Math|Rotator|MakeRotator 0.0 0.0 (* Z%20%28Yaw%29 -1.0)) false false)
    (else
      (Transformation|SetRelativeRotation TargetMesh (Math|Rotator|MakeRotator 0.0 0.0 Z%20%28Yaw%29) false false)))
  (return))