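; Posable mortuary trolley prop whose handle, rod and body element move together from a single handle value.
; The construction script scales TrolleyHandle by ratios of each part's maximum to derive the rod's travel and the body element's angle.
; Small helper functions with invert flags pitch the handle, offset the rod along local Z and roll the body element in reverse.
; The event graph is empty, so the Blueprint adds no runtime behavior.
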(event EventBeginPlay)

(event Collision|EventActorBeginOverlap
  (params (OtherActor :type Actor%20Object%20Reference)))

(event EventTick
  (params (DeltaSeconds :type Float%20%28single-precision%29)))

(fn ConstructionScript
  (bind _trolley_handle_max (Variables|Default|GetTrolley_Handle_Max))
  (Variables|Default|SetTrolley_Rod (* (Variables|Default|GetTrolley_Handle) (/ (Variables|Default|GetTrolley_Rod_Max) _trolley_handle_max)))
  (Variables|Default|SetTrolley_Body_Element (* (Variables|Default|GetTrolley_Handle) (/ (Variables|Default|GetTrolley_Body_Max) _trolley_handle_max)))
  (CallFunction|RotateY (Variables|Default|GetTrolley_Handle) false (Variables|Default|GetSM_Mortuary_Trolley_handle))
  (CallFunction|PositionZ (Variables|Default|GetTrolley_Rod) false (Variables|Default|GetSM_Mortuary_Trolley_rod))
  (CallFunction|RotateX (Variables|Default|GetTrolley_Body_Element) true (Variables|Default|GetSM_Mortuary_Trolley_body_element)))

(fn PositionZ
  (params (Z :type Float%20%28double-precision%29) (Invert%20Z :type Boolean) (TargetMesh :type Scene%20Component%20Object%20Reference))
  (bind _relativelocation (Variables|/Script/Engine.SceneComponent|GetRelativeLocation TargetMesh))
  (bind (_x _y _z) (Math|Vector|BreakVector _relativelocation))
  (if Invert%20Z
    (Transformation|SetRelativeLocation TargetMesh (Math|Vector|MakeVector _x _y (+ (* Z -1.0) _z)) false false)
    (else
      (Transformation|SetRelativeLocation TargetMesh (Math|Vector|MakeVector _x _y (+ Z _z)) false false)))
  (return))

(fn RotateY
  (params (Y%20%28Pitch%29 :type Float%20%28double-precision%29) (Invert%20Y :type Boolean) (TargetMesh :type Scene%20Component%20Object%20Reference))
  (if Invert%20Y
    (Transformation|SetRelativeRotation TargetMesh (Math|Rotator|MakeRotator 0.0 (* Y%20%28Pitch%29 -1.0) 0.0) false false)
    (else
      (Transformation|SetRelativeRotation TargetMesh (Math|Rotator|MakeRotator 0.0 Y%20%28Pitch%29 0.0) false false)))
  (return))

(fn RotateX
  (params (X%20%28Roll%29 :type Float%20%28double-precision%29) (Invert%20X :type Boolean) (TargetMesh :type Scene%20Component%20Object%20Reference))
  (if Invert%20X
    (Transformation|SetRelativeRotation TargetMesh (Math|Rotator|MakeRotator (* X%20%28Roll%29 -1.0) 0.0 0.0) false false)
    (else
      (Transformation|SetRelativeRotation TargetMesh (Math|Rotator|MakeRotator X%20%28Roll%29 0.0 0.0) false false)))
  (return))