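; BP_Door_03a is an interactable hinged door prefab that swings open and closed.
; Interact prints "Locked" if locked; otherwise, when not already moving, it toggles the open state and plays or reverses a timeline.
; The timeline lerps the first mesh's yaw from zero to Degree, forced positive unless IsInverted is set.
; A matching rotation node for a second mesh is left unconnected.
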(event EventInteract
  (if (Variables|Default|GetIsInverted)
    (Variables|Default|SetDegree (Variables|Default|GetDegree))
    (else
      (Variables|Default|SetDegree (Math|Float|Absolute(Float) (Variables|Default|GetDegree)))))
  (if (Variables|Default|GetIsLocked)
    (Development|PrintString "Locked")
    (elif (not (Variables|Default|GetIsMoving))
      (Variables|Default|SetIsMoving true)
      (bind _output_get (Variables|Default|SetIsOpened (not (Variables|Default|GetIsOpened))))
      (if _output_get
        (bind _dooralpha (Timeline|TL_Doors Play)
          (:Update
            (Transformation|SetRelativeRotation (Variables|Default|GetStaticMeshComponent0) (Math|Rotator|MakeRotator 0.0 0.0 (Math|Float|Lerp 0.0 (Variables|Default|GetDegree) _dooralpha)) false false))
          (:Finished
            (Variables|Default|SetIsMoving false)))
        (else
          (Timeline|TL_Doors Reverse))))))

(fn ConstructionScript)