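; Interactable hinged door prefab that swings open and closed, and can be locked until a key item pickup event unlocks it.
; Interact plays or reverses a timeline that lerps mesh yaw toward a set angle, ignoring input while moving and printing a message when locked.
; Two overlap spheres, sized in the construction script, toggle outer and inner interaction icons as the player approaches or leaves.
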(event OnComponentBeginOverlap(InnerSphere)
  (params (OverlappedComponent :type Primitive%20Component%20Object%20Reference) (OtherActor :type Actor%20Object%20Reference) (OtherComp :type Primitive%20Component%20Object%20Reference) (OtherBodyIndex :type Integer) (bFromSweep :type Boolean) (SweepResult :type Hit%20Result%20Structure%20%28by%20ref%29))
  (if (== OtherActor (Game|GetPlayerCharacter 0))
    (Rendering|SetVisibility (Variables|Default|GetInnerInteractIcon) true false)
    (Rendering|SetVisibility (Variables|Default|GetOuterInteractIcon) false false)))

(event OnComponentEndOverlap(InnerSphere)
  (params (OverlappedComponent :type Primitive%20Component%20Object%20Reference) (OtherActor :type Actor%20Object%20Reference) (OtherComp :type Primitive%20Component%20Object%20Reference) (OtherBodyIndex :type Integer))
  (if (== OtherActor (Game|GetPlayerCharacter 0))
    (Rendering|SetVisibility (Variables|Default|GetInnerInteractIcon) false false)
    (Rendering|SetVisibility (Variables|Default|GetOuterInteractIcon) true false)))

(event OnComponentBeginOverlap(OuterSphere)
  (params (OverlappedComponent :type Primitive%20Component%20Object%20Reference) (OtherActor :type Actor%20Object%20Reference) (OtherComp :type Primitive%20Component%20Object%20Reference) (OtherBodyIndex :type Integer) (bFromSweep :type Boolean) (SweepResult :type Hit%20Result%20Structure%20%28by%20ref%29))
  (if (== OtherActor (Game|GetPlayerCharacter 0))
    (Rendering|SetVisibility (Variables|Default|GetOuterInteractIcon) true false)))

(event OnComponentEndOverlap(OuterSphere)
  (params (OverlappedComponent :type Primitive%20Component%20Object%20Reference) (OtherActor :type Actor%20Object%20Reference) (OtherComp :type Primitive%20Component%20Object%20Reference) (OtherBodyIndex :type Integer))
  (if (== OtherActor (Game|GetPlayerCharacter 0))
    (Rendering|SetVisibility (Variables|Default|GetOuterInteractIcon) false false)))

(event EventPickupKeyItem
  (params (Doors :type BP%20Door%2001a%20Object%20Reference))
  ;[1 1 1] Unlock Door
  (Variables|Default|SetIsLocked false))

(event EventInteract
  (params (InteractingPlayer :type BP%20Motion%20Character%20Object%20Reference))
  (if (Variables|Default|GetIsInverted)
    (Variables|Default|SetDegree (Variables|Default|GetDegree))
    (else
      (Variables|Default|SetDegree (Math|Float|Absolute(Float) (Variables|Default|GetDegree)))))
  (if (Variables|Default|GetIsLocked)
    (Development|PrintString "Locked")
    (elif (not (Variables|Default|GetIsMoving))
      (Variables|Default|SetIsMoving true)
      (bind _output_get (Variables|Default|SetIsOpened (not (Variables|Default|GetIsOpened))))
      (if _output_get
        (bind _dooralpha (Timeline|TL_Doors Play)
          (:Update
            (Transformation|SetRelativeRotation (Variables|Default|GetStaticMeshComponent0) (Math|Rotator|MakeRotator 0.0 0.0 (Math|Float|Lerp 0.0 (Variables|Default|GetDegree) _dooralpha)) false false))
          (:Finished
            (Variables|Default|SetIsMoving false)))
        (else
          (Timeline|TL_Doors Reverse))))))

(fn ConstructionScript
  (Components|Sphere|SetSphereRadius (Variables|Default|GetInnerSphere) (Variables|Public|GetInnerSphereRadius) true)
  (Components|Sphere|SetSphereRadius (Variables|Default|GetOuterSphere) (Variables|Public|GetOuterShereRadius) true))