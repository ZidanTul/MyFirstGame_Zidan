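; Core component for BP_MotionCharacter that merges camera and walk speed contributions registered by other components.
; Components add or remove rotation curves, location vectors and speeds, keyed by source, with optional priority overrides.
; Each tick it combines these, applies them to the camera and max walk speed with a minimum-speed floor, and caches ground info via floor result or downward trace.
; It also offers component lookup helpers and optional on-screen debug printouts.
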(event EventBeginPlay
  ;[0.0382 0.1529 0.2502] Event Graph
  (Components|GetCoreComponents))

(event EventTick
  (params (DeltaSeconds :type Float%20%28single-precision%29))
  ;[0.0382 0.1529 0.2502] Event Graph
  (Core|HandleonEventTick))

(fn AddCameraOffset
  (params (CameraCurve :type F%20Struct%20Camera%20Curve%20Structure))
  (bind _motioncurve (Utilities|Struct|BreakFStructCameraCurve CameraCurve))
  (bind (_identifier _configuration) (Utilities|Struct|BreakFStructMotionCurve _motioncurve))
  ;[1 1 1] Adds a rotator for a provided component to the dictionary.
  (bind (_bfound _foundcameracurve _index) (Camera|FindCameraOffsetbyIdentifier _identifier))
  (if (not _bfound)
    (Utilities|Array|Add (Variables|ComponentData|GetCameraOffsets) CameraCurve)
    (else
      (Utilities|Array|SetArrayElem (Variables|ComponentData|GetCameraOffsets) _index CameraCurve)))
  (if (.bHasPriority (Utilities|Struct|BreakFStructMotionCurveConfiguration _configuration))
    (Variables|ComponentData|SetPriorityComponentForCameraOverride CameraCurve)))

(fn FindCameraOffsetbyIdentifier
  (params (CurveIdentifier :type F%20Struct%20Motion%20Curve%20Identifier%20Structure))
  (bind (_curvedcomponent _curvevector _curvetype) (Utilities|Struct|BreakFStructMotionCurveIdentifier CurveIdentifier))
  ;[1 1 1] Tries to find a camera offset by its curve identifier and returns it. Returns -1 if none was found.
  (if (not (Utilities|Array|IsEmpty (.CurveType (Utilities|Struct|BreakFStructMotionCurveIdentifier CurveIdentifier))))
    (for (_array_element _array_index) (Variables|ComponentData|GetCameraOffsets)
      (if (Math|Boolean|ANDBoolean (== (.CurvedComponent (Utilities|Struct|BreakFStructMotionCurveIdentifier (.Identifier (Utilities|Struct|BreakFStructMotionCurve (.MotionCurve (Utilities|Struct|BreakFStructCameraCurve _array_element)))))) _curvedcomponent) (== _curvevector (.CurveVector (Utilities|Struct|BreakFStructMotionCurveIdentifier (.Identifier (Utilities|Struct|BreakFStructMotionCurve (.MotionCurve (Utilities|Struct|BreakFStructCameraCurve _array_element))))))) (Utilities|Enum|Equal(Enum) (.CurveType (Utilities|Struct|BreakFStructMotionCurveIdentifier (.Identifier (Utilities|Struct|BreakFStructMotionCurve (.MotionCurve (Utilities|Struct|BreakFStructCameraCurve _array_element)))))) _curvetype))
        (return true _array_element _array_index)))
    (return false "" -1)
    (else
      (CallFunction|HandleMissingDataException "CurveType" "MotionCurveIdentifier when calling FindCameraOffsetByIdentifier."))))

(fn RemoveCameraOffset
  (params (CameraCurve :type F%20Struct%20Camera%20Curve%20Structure))
  ;[1 1 1] Tries to find the provided component and removes it registered offset from the dictionary. If the component is the override one, delete the override.
  (bind (_bfound _foundcameracurve _index) (Camera|FindCameraOffsetbyIdentifier (.Identifier (Utilities|Struct|BreakFStructMotionCurve (.MotionCurve (Utilities|Struct|BreakFStructCameraCurve CameraCurve))))))
  (if _bfound
    (Utilities|Array|RemoveIndex (Variables|ComponentData|GetCameraOffsets) _index)
    (if (.bHasPriority (Utilities|Struct|BreakFStructMotionCurveConfiguration (.Configuration (Utilities|Struct|BreakFStructMotionCurve (.MotionCurve (Utilities|Struct|BreakFStructCameraCurve _foundcameracurve))))))
      (Variables|ComponentData|SetPriorityComponentForCameraOverride ""))))

(fn PrintDebugInformation
  ;[1 1 1] Prints useful information on the screen. Helpful for debugging.
  (if (Variables|Configuration|GetbShowDebugInformation)
    (Utilities|FlowControl|Sequence
      (:then_0
        (|PrintCameraRotationOffsets))
      (:then_1
        (|PrintSpeeds))
      (:then_2
        (|PrintCameraLocationOffsets))
      (:then_3
        (Development|PrintString (Utilities|String|Append "Camera Priority Component: " (Utilities|GetDisplayName (.CurvedComponent (Utilities|Struct|BreakFStructMotionCurveIdentifier (.Identifier (Utilities|Struct|BreakFStructMotionCurve (.MotionCurve (Utilities|Struct|BreakFStructCameraCurve (Variables|ComponentData|GetPriorityComponentForCameraOverride)))))))) " 
Speed Priority Component: " (Utilities|GetDisplayName (Variables|ComponentData|GetPriorityComponentForSpeedOverride))) true true "(R=1.000000,G=1.000000,B=1.000000,A=1.000000)" 0.001)))))

(fn FlushCameraOffsets
  ;[1 1 1] Deletes all rotators from the currently dictionary.
  (Utilities|Array|Clear (Variables|ComponentData|GetCameraOffsets)))

(fn CalculateCameraOffset
  (bind (_offset _found) (|GetPriorityCameraComponent))
  ;[1 1 1] Gets all values from the Camera Offsets Dictionary and combines them to a single Rotator.
  (if (not _found) ; If a priority speed is present, instantly set it and skip computing speeds from other sources
    (for _array_element (Variables|ComponentData|GetCameraOffsets)
      (LocalVariables|SetCameraOffset (Math|Rotator|CombineRotators (.CurrentRotation (Utilities|Struct|BreakFStructCameraCurve _array_element)) (LocalVariables|GetCameraOffset))))
    (Variables|ComponentData|SetGlobalCameraOffset (LocalVariables|GetCameraOffset))
    (else
      (Variables|ComponentData|SetGlobalCameraOffset _offset))))

(fn GetCoreComponents
  ;[1 1 1] Get required components Character, Movement, Camera & Capsule and save their references
  (bind _asbp_motion_character (Utilities|Casting|CastToBP_MotionCharacter (Components|GetOwner)) ; Try to cast owning Blueprint as MotionCharacter
    (:then
      (bind _output_get (Variables|Components|SetCharacter _asbp_motion_character))
      (Variables|Components|SetCharacterMovement (Variables|/Script/Engine.Character|GetCharacterMovement _output_get))
      (Utilities|IsValid (Actor|GetComponentbyClass (Variables|Components|GetCharacter) "/Script/Engine.CameraComponent")
        (:Is%20Valid
          (Variables|Components|SetCamera (Actor|GetComponentbyClass (Variables|Components|GetCharacter) "/Script/Engine.CameraComponent"))
          (Variables|Components|SetCapsule (Variables|/Script/Engine.Character|GetCapsuleComponent (Variables|Components|GetCharacter)))
          (if (> (Utilities|Array|Length (Actor|GetComponentsbyTag (Variables|Components|GetCharacter) "/Script/Engine.SceneComponent" "CenterActor")) 0)
            (Variables|Default|SetCenterActor (Utilities|Array|Get(acopy) (Actor|GetComponentsbyTag (Variables|Components|GetCharacter) "/Script/Engine.SceneComponent" "CenterActor")))
            (Variables|ComponentData|SetInitialCameraLocation (Variables|/Script/Engine.SceneComponent|GetRelativeLocation (Variables|Components|GetCamera)))))
        (:Is%20Not%20Valid
          (CallFunction|HandleMissingDependencyException "/Script/Engine.CameraComponent" "BP_CharacterCoreComponent_C"))))
    (:CastFailed
      (CallFunction|HandleInvalidCastException "/Game/Motion/Blueprints/BP_MotionCharacter.BP_MotionCharacter_C"))))

(fn AddWalkSpeed
  (params (Component :type BP%20Base%20Character%20Curved%20Component%20Object%20Reference) (Value :type Float%20%28double-precision%29) (Priority :type Boolean))
  ;[1 1 1] Adds a speed of type float to the WalkSpeed dictionary
  (Utilities|Map|Add (Variables|ComponentData|GetWalkSpeeds) Component Value)
  (if Priority
    (Variables|ComponentData|SetPriorityComponentForSpeedOverride 0)))

(fn RemoveWalkSpeed
  (params (Component :type BP%20Base%20Character%20Curved%20Component%20Object%20Reference))
  ;[1 1 1] Tries to find the provided component and removes it registered offset from the dictionary. If the component is the override one, delete the override.
  (if (.ReturnValue (Utilities|Map|Find (Variables|ComponentData|GetWalkSpeeds) Component))
    (Utilities|Map|Remove (Variables|ComponentData|GetWalkSpeeds) Component)
    (if (== Component (Variables|ComponentData|GetPriorityComponentForSpeedOverride))
      (Variables|ComponentData|SetPriorityComponentForSpeedOverride 0))))

(fn FlushWalkSpeeds
  ;[1 1 1] Deletes all rotators from the currently dictionary.
  (Utilities|Map|Clear (Variables|ComponentData|GetWalkSpeeds)))

(fn CalculateWalkSpeed
  (bind (_speed _bispresent) (|GetPriorityComponentSpeed))
  ;[1 1 1] Combines the speeds from the WalkSpeeds dictionary to combined walk speed. If a priority component is selected, it will instead use that component's value
  (Variables|ComponentData|SetCalculatedSpeed 0.0)
  (if (not _bispresent) ; If a priority speed is present, instantly set it and skip computing speeds from other sources
    (bind _values (Utilities|Map|Values (Variables|ComponentData|GetWalkSpeeds)))
    (if (> (Utilities|Array|Length _values) 0)
      (for _array_element _values
        (Variables|ComponentData|SetCalculatedSpeed (+ _array_element (Variables|ComponentData|GetCalculatedSpeed))))
      (Variables|ComponentData|SetGlobalMaxWalkSpeed (Math|Float|SelectFloat (Variables|Configuration|GetGlobalMinimumSpeed) (Variables|ComponentData|GetCalculatedSpeed) (Utilities|MustApplyMinimumSpeed))))
    (else
      (Variables|ComponentData|SetGlobalMaxWalkSpeed _speed))))

(fn HandleonEventTick
  ;[1 1 1] Core logic handler. Calculates camera offset and player speed from data provided by components.
  (Utilities|FlowControl|Sequence
    (:then_0
      (Camera|CalculateCameraOffset)
      (Transformation|SetRelativeRotation (Variables|Components|GetCamera) (Math|Rotator|CombineRotators (Variables|ComponentData|GetGlobalCameraOffset) (Pawn|GetControlRotation (Game|GetPlayerController 0) :!class /Script/Engine.Controller)) false false))
    (:then_1
      (CameraLocationOffset|CalculateCameraLocation)
      (Transformation|SetRelativeLocation (Variables|Components|GetCamera) (+ (Variables|ComponentData|GetGlobalCameraLocationOffset) (Variables|ComponentData|GetInitialCameraLocation)) false false))
    (:then_2
      (WalkSpeed|CalculateWalkSpeed)
      (Variables|/Script/Engine.CharacterMovementComponent|SetMaxWalkSpeed (Variables|Components|GetCharacterMovement) (Variables|ComponentData|GetGlobalMaxWalkSpeed)))
    (:then_3
      (Core|GetGroundInfo))
    (:then_4
      (Debug|PrintDebugInformation))))

(fn GetActorsOfClasses
  (params (ActorClasses :type Array%20of%20Actor%20Class%20References))
  ;[1 1 1] Takes a list of actor classes and returns all actors of said classes.
  (for _array_element ActorClasses
    (bind _outactors (Actor|GetAllActorsOfClass _array_element))
    (for _array_element_2 _outactors
      (Utilities|Array|Add (LocalVariables|GetReturnList) _array_element_2)))
  (return (LocalVariables|GetReturnList)))

(fn GetComponent
  (params (ComponentClass :type Actor%20Component%20Class%20Reference) (RequiredBy :type Actor%20Component%20Object%20Reference))
  (bind _character (Variables|Components|GetCharacter))
  (bind _returnvalue (Actor|GetComponentbyClass _character ComponentClass))
  ;[1 1 1] Tries to find a component with the provided class name in the character blueprint. Will trigger an exception if not found.
  (Utilities|IsValid _returnvalue
    (:Is%20Valid
      (return _returnvalue))
    (:Is%20Not%20Valid
      (CallFunction|HandleMissingDependencyException ComponentClass (Utilities|GetClass RequiredBy)))))

(fn AddCameraLocationOffset
  (params (Component :type BP%20Base%20Character%20Curved%20Component%20Object%20Reference) (Value :type Vector) (Priority :type Boolean))
  ;[1 1 1] Adds a speed of type float to the WalkSpeed dictionary
  (Utilities|Map|Add (Variables|ComponentData|GetCameraVectors) Component Value)
  (if Priority
    (Variables|ComponentData|SetPriorityComponentForSpeedOverride 0)))

(fn RemoveCameraLocationOffset
  (params (Component :type BP%20Base%20Character%20Curved%20Component%20Object%20Reference))
  ;[1 1 1] Tries to find the provided component and removes it registered offset from the dictionary. If the component is the override one, delete the override.
  (if (.ReturnValue (Utilities|Map|Find (Variables|ComponentData|GetCameraVectors) Component))
    (Utilities|Map|Remove (Variables|ComponentData|GetCameraVectors) Component)
    (if (== Component (Variables|ComponentData|GetPriorityComponentForSpeedOverride))
      (Variables|ComponentData|SetPriorityComponentForSpeedOverride 0))))

(fn FlushCameraLocationOffsets
  ;[1 1 1] Deletes all rotators from the currently dictionary.
  (Utilities|Map|Clear (Variables|ComponentData|GetCameraVectors)))

(fn CalculateCameraLocation
  (bind (_vector _bispresent) (|GetPriorityComponentVector))
  ;[1 1 1] Combines the vectors from the CameraVectors dictionary to a combined camera location offset. If a priority component is selected, it will instead use that component's value
  (Variables|ComponentData|SetCalculatedCameraLocationOffset "0, 0, 0")
  (if (not _bispresent)
    (bind _values (Utilities|Map|Values (Variables|ComponentData|GetCameraVectors)))
    (if (> (Utilities|Array|Length _values) 0)
      (for _array_element _values
        (Variables|ComponentData|SetCalculatedCameraLocationOffset (+ (Variables|ComponentData|GetCalculatedCameraLocationOffset) _array_element)))
      (Variables|ComponentData|SetGlobalCameraLocationOffset (Variables|ComponentData|GetCalculatedCameraLocationOffset)))
    (else
      (Variables|ComponentData|SetGlobalCameraLocationOffset _vector))))

(fn AddHeadMovementCameraLocationOffset
  (bind _character (Variables|Components|GetCharacter))
  ;[1 1 1] Get the player's control rotation and add it to the location offset dictionary to prevent camera clipping into the mesh.
  (CameraLocationOffset|AddCameraLocationOffset (Variables|/Game/Motion/Blueprints/BP_MotionCharacter.BP_MotionCharacter_C|GetBP_TrueFirstPersonComponent (Variables|Components|GetCharacter)) (+ "0, 0, 0" (Math|Vector|MakeVector 0.0 0.0 (* (Math|Float|Lerp (Variables|/Game/Motion/Blueprints/BP_MotionCharacter.BP_MotionCharacter_C|GetMaximumCameraAdjustmentAngleForHeadMovement _character) (Variables|/Game/Motion/Blueprints/BP_MotionCharacter.BP_MotionCharacter_C|GetMinimumCameraAdjustmentAngleForHeadMovement _character) (Math|Float|Absolute(Float) (Math|Float|NormalizetoRange (- (.Pitch (Math|Rotator|BreakRotator (Pawn|GetControlRotation (Variables|Components|GetCharacter) :!class /Script/Engine.Pawn))) 1.8e+02) 0.0 3.6e+02))) -1.0))) false))

(fn GetGroundInfo
  (if (or (not (Utilities|IsValid (Components|GetOwner))) (!= (Utilities|GetFrameCount) (.LastUpdateFrame (Utilities|Struct|BreakFStructCharacterGroundInfo (Variables|ComponentData|GetCachedGroundInfo)))))
    (if (Utilities|Enum|Equal(Enum) (Variables|/Script/Engine.CharacterMovementComponent|GetMovementMode (Variables|Components|GetCharacterMovement)) "MOVE_Walking")
      (Pawn|Components|CharacterMovement|IsWalking)
      (else
        (|IsNotWalking)))))