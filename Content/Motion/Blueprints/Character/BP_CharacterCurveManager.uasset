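; Camera curve manager component that turns motion vector curves into rotation offsets on the owning character's camera through BP_CharacterCoreComponent.
; It extends a base curve manager, mirroring its curve and transition arrays into camera-specific structs whenever they update.
; Running curves are sampled for rotation each update.
; Transitions ease the source rotation toward zero while ramping the tick rate of a target curve created with the source's configuration.
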(event EventOnCurveArrayUpdated
  ;[0 0.1429 1] Event Graph
  (Utilities|FlowControl|Sequence
    (:then_0
      (CurveFunctions|UpdateCameraCurveArray))
    (:then_1
      (CurveFunctions|UpdateCameraCurveData))))

(event EventOnTransitionArrayUpdated
  ;[0 0.1429 1] Event Graph
  (Utilities|FlowControl|Sequence
    (:then_0
      (Transitions|UpdateCameraTransitionArray))
    (:then_1
      (Transitions|UpdateCameraTransitionData))))

(event EventBeginPlay
  ;[0 0.1429 1] Event Graph
  (Core|HandleonEventBeginPlay))

(fn UpdateCameraCurveArray
  ;[1 1 1] Updates the Camera Curve Array with the Motion Curve Array's base data.
  (for (_array_element _array_index) (Variables|Default|GetActiveMotionCurves)
    (if (Utilities|Enum|Equal(Enum) (.CurveType (Utilities|Struct|BreakFStructMotionCurveIdentifier (Utilities|Struct|BreakFStructMotionCurve _array_element))) (Variables|Constants|GetCurveType))
      (bind _structout (Utilities|Struct|SetmembersinFStructCameraCurve (Utilities|GetCameraCurve _array_index) _array_element))
      (Utilities|SetCameraCurve _structout _array_index))))

(fn UpdateCameraCurveData
  (bind (_returnvalue_x _returnvalue_y _returnvalue_z) (|GetCurrentRotation))
  ;[1 1 1] Loops through Camera Curves array and updates their tickrate (if transitioning) or rotation (if not transitioning).
  (for (_array_element _array_index) (Variables|ManagerData|GetActiveCameraCurves)
    (LocalVariables|SetCurrentIndex _array_index)
    (LocalVariables|SetCurrentCameraCurve _array_element)
    (if (not (Utilities|IsCurvePaused (LocalVariables|GetCurrentCameraCurve)))
      (Utilities|FlowControl|Sequence
        (:then_0
          ;;[1 1 1] Handle transitioning curves that are being transitioned from
          (if (Utilities|IsCurveTransitioning (LocalVariables|GetCurrentCameraCurve))
            (bind (_bfound _index) (CallFunction|GetTransitionbyIdentifier (Utilities|GetCurveIdentifierfromCameraCurve (LocalVariables|GetCurrentCameraCurve)) "NewEnumerator0"))
            (if _bfound
              (bind _structout (Utilities|Struct|SetmembersinFStructCameraCurve (LocalVariables|GetCurrentCameraCurve) (Math|Rotator|Lerp(Rotator) (.CurrentRotation (Utilities|Struct|BreakFStructCameraCurve (LocalVariables|GetCurrentCameraCurve))) "0, 0, 0" (Math|Float|Clamp(Float) (Math|Float|NormalizetoRange (Utilities|GetTransitionActiveSeconds (Utilities|Array|Get(acopy) (Variables|ManagerData|GetActiveCameraTransitions) _index)) 0.0 (Utilities|GetTransitionLength (Utilities|Array|Get(acopy) (Variables|ManagerData|GetActiveCameraTransitions) _index)))))))
              (Default|AddCameraOffset (Variables|Components|GetCharacterCoreComponent) _structout))))
        (:then_1
          ;;[1 1 1] Handle non-transitioning curves
          (if (not (Utilities|IsCurveTransitioning (LocalVariables|GetCurrentCameraCurve)))
            (bind (_bfound_2 _index_2) (CallFunction|GetCurvebyIdentifier (Utilities|GetCurveIdentifierfromCameraCurve (LocalVariables|GetCurrentCameraCurve))))
            (if _bfound_2
              (bind _bisvalid (CallFunction|ValidateCurve (Utilities|GetCurveIdentifierfromCameraCurve (LocalVariables|GetCurrentCameraCurve)) true))
              (if (and _bisvalid (not (Utilities|IsCurvePaused (LocalVariables|GetCurrentCameraCurve))))
                (bind _structout_2 (Utilities|Struct|SetmembersinFStructCameraCurve (Utilities|GetCameraCurve _index_2) (Math|Rotator|MakeRotator _returnvalue_x _returnvalue_y _returnvalue_z)))
                (Utilities|SetCameraCurve _structout_2 _index_2
                  (:_
                    (Default|AddCameraOffset (Variables|Components|GetCharacterCoreComponent) _structout_2)))))))))))

(fn UpdateCameraTransitionArray
  ;[1 1 1] Updates the Camera Transition Array from data of the base curve manager.
  (Utilities|Array|Clear (Variables|ManagerData|GetActiveCameraTransitions))
  (for (_array_element _array_index) (Variables|Default|GetActiveMotionCurveTransitions)
    (bind _structout (Utilities|Struct|SetmembersinFStructCameraCurveTransition (Utilities|Array|Get(acopy) (Variables|ManagerData|GetActiveCameraTransitions) _array_index) _array_element))
    (Utilities|Array|SetArrayElem (Variables|ManagerData|GetActiveCameraTransitions) _array_index _structout true)))

(fn UpdateCameraTransitionData
  ;[1 1 1] Loops through Camera Transitions array and updates their tickrate.
  (for _array_element (Variables|ManagerData|GetActiveCameraTransitions)
    (if (not (.bIsPaused (Utilities|Struct|BreakFStructMotionCurveTransition (Utilities|Struct|BreakFStructCameraCurveTransition _array_element))))
      (CallFunction|SetCurveTickRate (.TargetIdentifier (Utilities|Struct|BreakFStructMotionCurveTransitionConfiguration (.TransitionConfiguration (Utilities|Struct|BreakFStructMotionCurveTransition (Utilities|Struct|BreakFStructCameraCurveTransition _array_element))))) (Math|Float|Clamp(Float) (Math|Float|NormalizetoRange (.ActiveTransitionSeconds (Utilities|Struct|BreakFStructMotionCurveTransition (Utilities|Struct|BreakFStructCameraCurveTransition _array_element))) 0.0 (.TransitionTime (Utilities|Struct|BreakFStructMotionCurveTransitionConfiguration (.TransitionConfiguration (Utilities|Struct|BreakFStructMotionCurveTransition (Utilities|Struct|BreakFStructCameraCurveTransition _array_element)))))))))))

(fn StartTransition
  (params (TransitionData :type F%20Struct%20Motion%20Curve%20Transition%20Structure))
  ;[1 1 1] Creates a new transition. Finds the source curve, copies it configuration into the new target curve and adds the transition to the array.
  (LocalVariables|SetLocalTransitionData TransitionData)
  (bind (_bsuccessful _index) (|CallParentFunction TransitionData))
  (if _bsuccessful
    (LocalVariables|SetLocalTransitionIndex _index)
    (Utilities|FlowControl|Sequence
      (:then_0
        ;;[1 1 1] Copy configuration from source curve and create new target curve.
        (bind (_bfound _index_2) (CallFunction|GetCurvebyIdentifier (.Identifier (Utilities|Struct|BreakFStructMotionCurveTransitionConfiguration (.TransitionConfiguration (Utilities|Struct|BreakFStructMotionCurveTransition (LocalVariables|GetLocalTransitionData)))))))
        (if _bfound
          (CallFunction|AddCurve (Utilities|Struct|MakeFStructMotionCurve (Utilities|Struct|MakeFStructMotionCurveIdentifier (.CurvedComponent (Utilities|Struct|BreakFStructMotionCurveIdentifier (.TargetIdentifier (Utilities|Struct|BreakFStructMotionCurveTransitionConfiguration (.TransitionConfiguration (Utilities|Struct|BreakFStructMotionCurveTransition (LocalVariables|GetLocalTransitionData))))))) (.CurveVector (Utilities|Struct|BreakFStructMotionCurveIdentifier (.TargetIdentifier (Utilities|Struct|BreakFStructMotionCurveTransitionConfiguration (.TransitionConfiguration (Utilities|Struct|BreakFStructMotionCurveTransition (LocalVariables|GetLocalTransitionData))))))) (.CurveType (Utilities|Struct|BreakFStructMotionCurveIdentifier (.TargetIdentifier (Utilities|Struct|BreakFStructMotionCurveTransitionConfiguration (.TransitionConfiguration (Utilities|Struct|BreakFStructMotionCurveTransition (LocalVariables|GetLocalTransitionData)))))))) (Utilities|Struct|BreakFStructMotionCurve (Utilities|Struct|BreakFStructCameraCurve (Utilities|GetCameraCurve _index_2))) false false false true))))
      (:then_1
        ;;[1 1 1] Add element to transition array
        (Utilities|Array|SetArrayElem (Variables|ManagerData|GetActiveCameraTransitions) (LocalVariables|GetLocalTransitionIndex) (Utilities|Struct|MakeFStructCameraCurveTransition (LocalVariables|GetLocalTransitionData) "0.000000,0.000000,0.000000" (Utilities|Struct|BreakFStructCameraCurve (Utilities|GetCameraCurve (LocalVariables|GetLocalTransitionIndex)))) true)
        (return true (LocalVariables|GetLocalTransitionIndex))))))

(fn GetTransitionbyIdentifier
  (params (CurveIdentifier :type F%20Struct%20Motion%20Curve%20Identifier%20Structure) (IdentifierType :type ETransitionCurves%20Enum :default "NewEnumerator0"))
  (bind (_curvedcomponent _curvevector _curvetype) (Utilities|Struct|BreakFStructMotionCurveIdentifier CurveIdentifier))
  ;[1 1 1] Tries to find a transition given its configuration. Returns its index if found, returns -1 if not.
  (for (_array_element _array_index) (Variables|ManagerData|GetActiveCameraTransitions)
    (if (Utilities|Enum|Equal(Enum) IdentifierType "NewEnumerator0")
      (if (Math|Boolean|ANDBoolean (== _curvedcomponent (.CurvedComponent (Utilities|Struct|BreakFStructMotionCurveIdentifier (.identifier (.TransitionConfiguration (Utilities|Struct|BreakFStructMotionCurveTransition (Utilities|Struct|BreakFStructCameraCurveTransition _array_element))))))) (== _curvevector (.CurveVector (Utilities|Struct|BreakFStructMotionCurveIdentifier (.identifier (.TransitionConfiguration (Utilities|Struct|BreakFStructMotionCurveTransition (Utilities|Struct|BreakFStructCameraCurveTransition _array_element))))))) (Utilities|Enum|Equal(Enum) _curvetype (.CurveType (Utilities|Struct|BreakFStructMotionCurveIdentifier (.identifier (.TransitionConfiguration (Utilities|Struct|BreakFStructMotionCurveTransition (Utilities|Struct|BreakFStructCameraCurveTransition _array_element))))))))
        (return true _array_index))
      (elif (Math|Boolean|ANDBoolean (== _curvedcomponent (.CurvedComponent (Utilities|Struct|BreakFStructMotionCurveIdentifier (.targetidentifier (.TransitionConfiguration (Utilities|Struct|BreakFStructMotionCurveTransition (Utilities|Struct|BreakFStructCameraCurveTransition _array_element))))))) (== _curvevector (.CurveVector (Utilities|Struct|BreakFStructMotionCurveIdentifier (.targetidentifier (.TransitionConfiguration (Utilities|Struct|BreakFStructMotionCurveTransition (Utilities|Struct|BreakFStructCameraCurveTransition _array_element))))))) (Utilities|Enum|Equal(Enum) _curvetype (.CurveType (Utilities|Struct|BreakFStructMotionCurveIdentifier (.targetidentifier (.TransitionConfiguration (Utilities|Struct|BreakFStructMotionCurveTransition (Utilities|Struct|BreakFStructCameraCurveTransition _array_element))))))))
        (return true _array_index))))
  (return false -1))

(fn PrintDebugInformation
  ;[1 1 1] Prints useful information on the screen. Helpful for debugging.
  (|CallParentFunction)
  (if (Variables|Configuration|GetbShowThisDebugInformation)
    (Utilities|FlowControl|Sequence
      (:then_0
        ;;[1 1 1] Prints Camera Curves
        (LocalVariables|SetOutputMessage (Utilities|String|Append "Registered Camera Curves: " (Utilities|String|ToString(Integer) (Utilities|Array|Length (Variables|ManagerData|GetActiveCameraCurves))) " 
"))
        (for _array_element (Variables|ManagerData|GetActiveCameraCurves)
          (LocalVariables|SetOutputMessage (Utilities|String|Append (LocalVariables|GetOutputMessage) " 
Identifier: " (Utilities|GetDisplayName (.CurvedComponent (Utilities|Struct|BreakFStructMotionCurveIdentifier (.Identifier (Utilities|Struct|BreakFStructMotionCurve (.MotionCurve (Utilities|Struct|BreakFStructCameraCurve _array_element))))))) " - " (Utilities|GetDisplayName (.CurveVector (Utilities|Struct|BreakFStructMotionCurveIdentifier (.Identifier (Utilities|Struct|BreakFStructMotionCurve (.MotionCurve (Utilities|Struct|BreakFStructCameraCurve _array_element))))))) " 
Should Loop: " (Utilities|String|ToString(Boolean) (.bShouldLoop (Utilities|Struct|BreakFStructMotionCurveConfiguration (.Configuration (Utilities|Struct|BreakFStructMotionCurve (.MotionCurve (Utilities|Struct|BreakFStructCameraCurve _array_element))))))) " 
Should Reverse: " (Utilities|String|ToString(Boolean) (.bShouldReverse (Utilities|Struct|BreakFStructMotionCurveConfiguration (.Configuration (Utilities|Struct|BreakFStructMotionCurve (.MotionCurve (Utilities|Struct|BreakFStructCameraCurve _array_element))))))) " 
Has Priority: " (Utilities|String|ToString(Boolean) (.bHasPriority (Utilities|Struct|BreakFStructMotionCurveConfiguration (.Configuration (Utilities|Struct|BreakFStructMotionCurve (.MotionCurve (Utilities|Struct|BreakFStructCameraCurve _array_element))))))) " 
Tickrate: " (Utilities|String|ToString(Float) (.Tickrate (Utilities|Struct|BreakFStructMotionCurveConfiguration (.Configuration (Utilities|Struct|BreakFStructMotionCurve (.MotionCurve (Utilities|Struct|BreakFStructCameraCurve _array_element))))))) " 
Is Reversing: " (Utilities|String|ToString(Boolean) (.bIsReversing (Utilities|Struct|BreakFStructMotionCurve (.MotionCurve (Utilities|Struct|BreakFStructCameraCurve _array_element))))) " 
Is Paused: " (Utilities|String|ToString(Boolean) (.bIsPaused (Utilities|Struct|BreakFStructMotionCurve (.MotionCurve (Utilities|Struct|BreakFStructCameraCurve _array_element))))) " 
Is Transitioning: " (Utilities|String|ToString(Boolean) (.bIsTransitioning (Utilities|Struct|BreakFStructMotionCurve (.MotionCurve (Utilities|Struct|BreakFStructCameraCurve _array_element))))) " 
Active Seconds: " (Utilities|String|ToString(Float) (.ActiveSeconds (Utilities|Struct|BreakFStructMotionCurve (.MotionCurve (Utilities|Struct|BreakFStructCameraCurve _array_element))))) " 
Current Rotation: " (Utilities|String|ToString(Rotator) (.CurrentRotation (Utilities|Struct|BreakFStructCameraCurve _array_element))) " 
Is Transition Curve: " (Utilities|String|ToString(Boolean) (.bIsTransitionCurve (Utilities|Struct|BreakFStructMotionCurve (.MotionCurve (Utilities|Struct|BreakFStructCameraCurve _array_element))))))))
        (Development|PrintString (LocalVariables|GetOutputMessage) true true "(R=1.000000,G=0.160115,B=0.020335,A=1.000000)" 0.001))
      (:then_1
        ;;[1 1 1] Prints Camera Transitions
        (LocalVariables|SetOutputMessage (Utilities|String|Append "Registered Transitions: " (Utilities|String|ToString(Integer) (Utilities|Array|Length (Variables|ManagerData|GetActiveCameraTransitions))) " 
"))
        (for _array_element_2 (Variables|ManagerData|GetActiveCameraTransitions)
          (LocalVariables|SetOutputMessage (Utilities|String|Append (LocalVariables|GetOutputMessage) " 
To: " (Utilities|GetDisplayName (.CurvedComponent (Utilities|Struct|BreakFStructMotionCurveIdentifier (.Identifier (Utilities|Struct|BreakFStructMotionCurveTransitionConfiguration (.TransitionConfiguration (Utilities|Struct|BreakFStructMotionCurveTransition (.TransitionData (Utilities|Struct|BreakFStructCameraCurveTransition _array_element_2))))))))) " - " (Utilities|GetDisplayName (.CurveVector (Utilities|Struct|BreakFStructMotionCurveIdentifier (.Identifier (Utilities|Struct|BreakFStructMotionCurveTransitionConfiguration (.TransitionConfiguration (Utilities|Struct|BreakFStructMotionCurveTransition (.TransitionData (Utilities|Struct|BreakFStructCameraCurveTransition _array_element_2))))))))) " 
Transition Time: " (Utilities|String|ToString(Float) (.TransitionTime (Utilities|Struct|BreakFStructMotionCurveTransitionConfiguration (.TransitionConfiguration (Utilities|Struct|BreakFStructMotionCurveTransition (.TransitionData (Utilities|Struct|BreakFStructCameraCurveTransition _array_element_2))))))) " 
Tick Rate: " (Utilities|String|ToString(Float) (.TickRate (Utilities|Struct|BreakFStructMotionCurveTransitionConfiguration (.TransitionConfiguration (Utilities|Struct|BreakFStructMotionCurveTransition (.TransitionData (Utilities|Struct|BreakFStructCameraCurveTransition _array_element_2))))))) " 
Active Transition Seconds: " (Utilities|String|ToString(Float) (.ActiveTransitionSeconds (Utilities|Struct|BreakFStructMotionCurveTransition (.TransitionData (Utilities|Struct|BreakFStructCameraCurveTransition _array_element_2))))) " 
Current Rotation: " (Utilities|String|ToString(Rotator) (.Rotation (Utilities|Struct|BreakFStructCameraCurveTransition _array_element_2))) " 
Initial Rotation: " (Utilities|String|ToString(Rotator) (.InitialRotation (Utilities|Struct|BreakFStructCameraCurveTransition _array_element_2))))))
        (Development|PrintString (LocalVariables|GetOutputMessage) true true "(R=0.942751,G=0.000000,B=1.000000,A=1.000000)" 0.001)))))

(fn DeleteTransition
  (params (SourceCurveIdentifier :type F%20Struct%20Motion%20Curve%20Identifier%20Structure))
  ;[1 1 1] Removes a transition from the array and delete its camera offset.
  (bind _bsuccessful (|CallParentFunction SourceCurveIdentifier))
  (if _bsuccessful
    (Utilities|FlowControl|Sequence
      (:then_0
        (bind (_bfound _index) (CallFunction|GetTransitionbyIdentifier SourceCurveIdentifier "NewEnumerator0"))
        (if _bfound
          (Utilities|Array|RemoveIndex (Variables|ManagerData|GetActiveCameraTransitions) _index)
          (else
            (return false))))
      (:then_1
        (Default|RemoveCameraOffset (Variables|Components|GetCharacterCoreComponent) (Utilities|Struct|MakeFStructCameraCurve (Utilities|Struct|MakeFStructMotionCurve SourceCurveIdentifier false)))
        (return true)))))

(fn HandleonEventBeginPlay
  (bind _returnvalue (Components|GetOwner))
  (bind _returnvalue_2 (Actor|GetComponentbyClass _returnvalue "/Game/Motion/Blueprints/Character/BP_CharacterCoreComponent.BP_CharacterCoreComponent_C"))
  ;[1 1 1] Called when "Event Begin Play" gets called. Gets a reference to the Example Gameplay Manager from the Game Mode.
  (Utilities|IsValid _returnvalue_2
    (:Is%20Valid
      (Variables|Components|SetCharacterCoreComponent _returnvalue_2))
    (:Is%20Not%20Valid
      (Development|PrintString "UNABLE TO FIND BP_CharacterCoreComponent in Character Blueprint for BP_CameraCurveManager!" true true "(R=1.000000,G=0.000000,B=0.069961,A=1.000000)")
      (Game|QuitGame 0 "Quit" false))))

(fn DeleteCurve
  (params (Curve :type F%20Struct%20Motion%20Curve%20Identifier%20Structure))
  ;[1 1 1] Removes a specified curve. Returns false if the specified curve could not be found.
  (bind (_bsuccessful _curveindex) (|CallParentFunction Curve))
  (if _bsuccessful
    (Utilities|Array|RemoveIndex (Variables|ManagerData|GetActiveCameraCurves) _curveindex)
    (Default|RemoveCameraOffset (Variables|Components|GetCharacterCoreComponent) (Utilities|Struct|MakeFStructCameraCurve (Utilities|Struct|MakeFStructMotionCurve Curve "(bShouldLoop_9_666576974F883E228DB125BEAF8A60D0=False,bShouldReverse_11_5F50FB6143A47A5D2F479EBAAD96DD32=False,bHasPriority_14_E460BB484F65E64110A48FB2A6E597CB=False,Tickrate_16_7FAB02194AA4ADC275096CBD3E8829FC=0.000000)") "0.000000,0.000000,0.000000"))
    (return _bsuccessful _curveindex)))