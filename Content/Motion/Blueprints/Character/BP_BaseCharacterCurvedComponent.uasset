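; Base character component for features driven by motion curves, providing shared setup and default curve-event handling.
; On BeginPlay it finds the owner's CharacterCoreComponent, flags it if missing, and resolves the CharacterCurveManager through it.
; When a transition reaches its maximum, the default handler deletes that transition and its curve from the manager by identifier.
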(event Custom|OnTransitionMaximum
  (params (TransitionData :type F%20Struct%20Motion%20Curve%20Transition%20Structure))
  ;[0.03922 0.1529 0.251] Event Graph
  ;;[1 1 1] Curve Events & their default implementation
  (Core|HandleonTransitionMaximumParent TransitionData))

(event EventBeginPlay
  ;[0.03922 0.1529 0.251] Event Graph
  (|CallParentFunction)
  (Core|HandleonEventBeginPlayParent))

(fn HandleonEventBeginPlayParent
  ;[1 1 1] Called when "Event Begin Play" gets called. Gets a reference to the Camera Curve Manager.
  (Utilities|FlowControl|Sequence
    (:then_0
      (bind _output_get (Variables|Default|SetCharacterCoreComponent (Actor|GetComponentbyClass (Components|GetOwner) "/Game/Motion/Blueprints/Character/BP_CharacterCoreComponent.BP_CharacterCoreComponent_C")))
      (if (not (Utilities|IsValid _output_get))
        (CallFunction|HandleMissingDependencyException "/Game/Motion/Blueprints/Character/BP_CharacterCoreComponent.BP_CharacterCoreComponent_C" (Utilities|GetClass self))))
    (:then_1
      (bind _actorcomponent (Default|GetComponent (Variables|Default|GetCharacterCoreComponent) "/Game/Motion/Blueprints/Character/BP_CharacterCurveManager.BP_CharacterCurveManager_C" self))
      (bind _asbp_character_curve_manager (Utilities|Casting|CastToBP_CharacterCurveManager _actorcomponent))
      (Variables|Default|SetCharacterCurveManager _asbp_character_curve_manager))))

(fn HandleonTransitionMaximumParent
  (params (FStructMotionCurveTransition :type F%20Struct%20Motion%20Curve%20Transition%20Structure%20%28by%20ref%29))
  (bind _transitionconfiguration (Utilities|Struct|BreakFStructMotionCurveTransition FStructMotionCurveTransition))
  (bind _charactercurvemanager (Variables|Default|GetCharacterCurveManager))
  (bind _identifier (Utilities|Struct|BreakFStructMotionCurveTransitionConfiguration _transitionconfiguration))
  ;[1 1 1] Called when "On Transition Maximum" gets called. Deletes the transition and transition curve.
  (Default|DeleteTransition _charactercurvemanager _identifier)
  (Default|DeleteCurve _charactercurvemanager _identifier))