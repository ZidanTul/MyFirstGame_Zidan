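; BP_IdleComponent is a character component that plays a random idle curve, described as a camera offset, after the player is inactive long enough.
; Tick advances an idle timer until it passes a threshold, then registers a random vector curve with the CharacterCurveManager.
; Camera, movement and jump events reset the timer and delete the curve.
; Reaching the curve's maximum also resets it through BPI_CurveComponent, so the idle cycle restarts.
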(event Custom|EventOnPlayerJump
  ;[0 0.1429 1] Event Graph
  (EventHandler|HandleonPlayerJump))

(event Custom|EventOnCameraInput
  (params (AxisValue :type Float%20%28double-precision%29))
  ;[0 0.1429 1] Event Graph
  (EventHandler|HandleonCameraInput))

(event Custom|EventOnMovementInput
  (params (Direction :type Vector) (AxisValue :type Float%20%28double-precision%29))
  ;[0 0.1429 1] Event Graph
  (EventHandler|HandleonMovementInput))

(event EventOnCurveMaximum
  (params (CurveData :type F%20Struct%20Motion%20Curve%20Structure))
  ;[1 1 1] BPI_CurveComponent Implementations
  (EventHandler|HandleonCurveMaximum CurveData))

(event EventTick
  (params (DeltaSeconds :type Float%20%28single-precision%29))
  ;[0 0.1429 1] Event Graph
  (EventHandler|HandleonEventTick DeltaSeconds))

(event EventBeginPlay
  ;[0 0.1429 1] Event Graph
  (|CallParentFunction)
  (EventHandler|HandleonEventBeginPlay (delegate Custom|EventOnCameraInput) (delegate Custom|EventOnMovementInput) (delegate Custom|EventOnPlayerJump)))

(fn PrintDebugInformation
  ;[1 1 1] Prints useful information on the screen. Helpful for debugging.
  (if (Variables|Configuration|GetbShowDebugInformation)
    (Development|PrintString (Utilities|String|Append " 
Active Idle Seconds: " (Utilities|String|ToString(Float) (Variables|ComponentData|GetActiveIdleSeconds)) " 
Is Idle: " (Utilities|String|ToString(Boolean) (Variables|ComponentData|GetbIsIdle)) " 
Has Animation Played: " (Utilities|String|ToString(Boolean) (Variables|ComponentData|GetbHasIdleAnimationPlayed)) " 
Active Curve: " (Utilities|GetDisplayName (Variables|ComponentData|GetActiveCurve))) true true "(R=1.000000,G=0.045011,B=0.000000,A=1.000000)" 0.001)))

(fn UpdateDeltaSeconds
  (params (DeltaSeconds :type Float%20%28double-precision%29))
  ;[1 1 1] Updates the idle timer.
  (bind _updatedactivedeltaseconds (CallFunction|UpdateSeconds (Variables|ComponentData|GetActiveIdleSeconds) (Variables|Constants|GetDeltaTickRate) DeltaSeconds false))
  (Variables|ComponentData|SetActiveIdleSeconds _updatedactivedeltaseconds))

(fn HandleonEventBeginPlay
  (params (EventOnCameraInputDelegate :type Delegate%20%28by%20ref%29) (EventOnMovementInputDelegate :type Delegate%20%28by%20ref%29) (EventOnJumpJumpedDelegate :type Delegate%20%28by%20ref%29))
  ;[1 1 1] Called when "Event Begin Play" gets called. Sets up events.
  (Utilities|FlowControl|Sequence
    (:then_0
      ;;[1 1 1] Validates if any curves were selected prior to initialisation
      (if (== (Utilities|Array|Length (Variables|Configuration|GetIdleCurves)) 0)
        (CallFunction|HandleMissingConfigurationDependencyException "IdleCurves" (Utilities|GetClass self))))
    (:then_1
      ;;[1 1 1] Bind Events
      (EventDispatchers|BindEventtoOnCameraInput (Variables|/Game/Motion/Blueprints/Character/BP_CharacterCoreComponent.BP_CharacterCoreComponent_C|GetCharacter (Variables|Default|GetCharacterCoreComponent)) EventOnCameraInputDelegate)
      (EventDispatchers|BindEventtoOnMovementInput (Variables|/Game/Motion/Blueprints/Character/BP_CharacterCoreComponent.BP_CharacterCoreComponent_C|GetCharacter (Variables|Default|GetCharacterCoreComponent)) EventOnMovementInputDelegate)
      (EventDispatchers|BindEventtoOnJumpJumped (Variables|/Game/Motion/Blueprints/Character/BP_CharacterCoreComponent.BP_CharacterCoreComponent_C|GetCharacter (Variables|Default|GetCharacterCoreComponent)) EventOnJumpJumpedDelegate))))

(fn HandleonEventTick
  (params (DeltaSeconds :type Float%20%28double-precision%29))
  ;[1 1 1] Core logic handler. Updates the timer & checks if idle should kick in.
  (if (Variables|Configuration|GetbIsEnabled)
    (if (not (Variables|ComponentData|GetbIsIdle))
      (Utilities|FlowControl|Sequence
        (:then_0
          (Manipulators|UpdateDeltaSeconds DeltaSeconds))
        (:then_1
          (Manipulators|ValidateIdleSeconds))
        (:then_2
          (Debug|PrintDebugInformation :!label _label)))
      (else
        (goto _label)))
    (else
      (goto _label))))

(fn HandleonCameraInput
  ;[1 1 1] Called when the player moves.
  (if (Variables|Configuration|GetbIsEnabled)
    (Manipulators|ResetIdleSeconds)))

(fn HandleonMovementInput
  ;[1 1 1] Called when the player stops moving.
  (if (Variables|Configuration|GetbIsEnabled)
    (Manipulators|ResetIdleSeconds)))

(fn ResetIdleSeconds
  ;[1 1 1] Resets the idle timer.
  (Variables|ComponentData|SetbIsIdle false)
  (Variables|ComponentData|SetActiveIdleSeconds 0.0)
  (if (Variables|ComponentData|GetbHasIdleAnimationPlayed)
    (Manipulators|StopIdleAnimation)
    (Variables|ComponentData|SetbHasIdleAnimationPlayed false)))

(fn ValidateIdleSeconds
  ;[1 1 1] Checks if the player was idle long enough and prevents multiple set curve calls.
  (bind _output_get (Variables|ComponentData|SetbIsIdle (>= (Variables|ComponentData|GetActiveIdleSeconds) (Variables|Configuration|GetSecondsToIdle))))
  (if (and _output_get (not (Variables|ComponentData|GetbHasIdleAnimationPlayed)))
    (Manipulators|SetIdleCurve)))

(fn SetIdleCurve
  ;[1 1 1] Selects a random curve from the configured list of curves.
  (Variables|ComponentData|SetActiveCurve (.OutItem (Utilities|Array|Random (Variables|Configuration|GetIdleCurves))))
  (Default|AddCurve (Variables|Default|GetCharacterCurveManager) (Utilities|Struct|MakeFStructMotionCurve (Utilities|Struct|MakeFStructMotionCurveIdentifier self (Variables|ComponentData|GetActiveCurve) (Variables|Constants|GetCurveType)) (Utilities|Struct|MakeFStructMotionCurveConfiguration false false false (Variables|Constants|GetDeltaTickRate)) false false false false 0.0))
  (Variables|ComponentData|SetbHasIdleAnimationPlayed true))

(fn StopIdleAnimation
  ;[1 1 1] Removes the camera offset and resets states.
  (Default|DeleteCurve (Variables|Default|GetCharacterCurveManager) (Utilities|Struct|MakeFStructMotionCurveIdentifier self (Variables|ComponentData|GetActiveCurve) (Variables|Constants|GetCurveType)))
  (Variables|ComponentData|SetActiveCurve 0))

(fn HandleonPlayerJump
  ;[1 1 1] Called when the player jumped.
  (if (Variables|Configuration|GetbIsEnabled)
    (Manipulators|ResetIdleSeconds)))

(fn HandleonCurveMaximum
  (params (CurveData :type F%20Struct%20Motion%20Curve%20Structure))
  ;[1 1 1] Called when the component's active curve reaches its peak.
  (Manipulators|ResetIdleSeconds))