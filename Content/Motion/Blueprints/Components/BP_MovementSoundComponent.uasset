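; Character component that plays footstep, jump and landing sounds matched to the floor's physical surface.
; Character movement events drive a velocity-scaled step timer that alternates feet, varies by walk, sprint or crouch, and is muted while sneaking.
; Movement mode changes trigger jump and land sounds, using a box trace when leaving the ground because CurrentFloor can be empty.
; Sounds are picked randomly from DT_MovementSounds by type and surface, unless identifier overrides apply.
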(event Custom|EventOnMovementModeChanged
  (params (Character :type Character%20Object%20Reference) (PrevMovementMode :type EMovementMode%20Enum :default "MOVE_None") (PreviousCustomMode :type Byte))
  ;[0.03922 0.1529 0.251] Event Graph
  (EventHandler|HandleonMovementModeChanged PrevMovementMode PreviousCustomMode))

(event Custom|EventOnCharacterMovementChanged
  (params (DeltaSeconds :type Float%20%28double-precision%29) (OldLocation :type Vector) (OldVelocity :type Vector))
  ;[0.03922 0.1529 0.251] Event Graph
  (EventHandler|HandleonCharacterMovementChanged DeltaSeconds OldLocation OldVelocity))

(event EventBeginPlay
  ;[0.03922 0.1529 0.251] Event Graph
  (|CallParentFunction)
  (EventHandler|HandleEventonBeginPlay (delegate Custom|EventOnMovementModeChanged) (delegate Custom|EventOnCharacterMovementChanged)))

(event EventTick
  (params (DeltaSeconds :type Float%20%28single-precision%29))
  ;[0.03922 0.1529 0.251] Event Graph
  (Debug|PrintDebugInformation))

(fn HandleEventonBeginPlay
  (params (EventOnMovementModeChangedDelegate :type Delegate%20%28by%20ref%29) (EventOnCharacterMovementChangedDelegate :type Delegate%20%28by%20ref%29))
  ;[1 1 1] Called when "Event Begin Play" gets called. Sets up events and saves component references.
  (Utilities|FlowControl|Sequence
    (:then_0
      (Utilities|FlowControl|Sequence
        (:then_0
          ;;[1 1 1] Find and save required components
          (bind _actorcomponent (Default|GetComponent (Variables|Default|GetCharacterCoreComponent) "/Game/Motion/Blueprints/Components/BP_SneakingComponent.BP_SneakingComponent_C" self))
          (bind _asbp_sneaking_component (Utilities|Casting|CastToBP_SneakingComponent _actorcomponent))
          (Variables|Default|SetSneakingComponent _asbp_sneaking_component))
        (:then_1
          (bind _actorcomponent_2 (Default|GetComponent (Variables|Default|GetCharacterCoreComponent) "/Game/Motion/Blueprints/Components/BP_CrouchingComponent.BP_CrouchingComponent_C" self))
          (bind _asbp_crouching_component (Utilities|Casting|CastToBP_CrouchingComponent _actorcomponent_2))
          (Variables|Default|SetCrouchingComponent _asbp_crouching_component))
        (:then_2
          (bind _actorcomponent_3 (Default|GetComponent (Variables|Default|GetCharacterCoreComponent) "/Game/Motion/Blueprints/Components/BP_SprintingComponent.BP_SprintingComponent_C"))
          (bind _asbp_sprinting_component (Utilities|Casting|CastToBP_SprintingComponent _actorcomponent_3))
          (Variables|Default|SetSprintingComponent _asbp_sprinting_component))))
    (:then_1
      ;;[1 1 1] Register Event Listeners
      (Character|BindEventtoMovementModeChangedDelegate (Variables|/Game/Motion/Blueprints/Character/BP_CharacterCoreComponent.BP_CharacterCoreComponent_C|GetCharacter (Variables|Default|GetCharacterCoreComponent)) EventOnMovementModeChangedDelegate)
      (EventDispatchers|BindEventtoOnCharacterMovementChanged (Variables|/Game/Motion/Blueprints/Character/BP_CharacterCoreComponent.BP_CharacterCoreComponent_C|GetCharacter (Variables|Default|GetCharacterCoreComponent)) EventOnCharacterMovementChangedDelegate))))

(fn HandleonMovementModeChanged
  (params (PreviousMovementMode :type EMovementMode%20Enum :default "MOVE_None") (PreviousCustomMode :type Byte))
  ;[1 1 1] Called when the movement mode changes (e.g. from falling to walking)
  (if (Variables|Configuration|GetbIsEnabled)
    (EventHandler|HandleJumpLandSounds PreviousMovementMode)))

(fn HandleonCharacterMovementChanged
  (params (DeltaSeconds :type Float%20%28double-precision%29) (OldLocation :type Vector) (OldVelocity :type Vector))
  ;[1 1 1] Called when the player is moving.
  (if (and (Variables|Configuration|GetbIsEnabled) (not (Variables|/Game/Motion/Blueprints/Components/BP_SneakingComponent.BP_SneakingComponent_C|GetbIsSneaking (Variables|Default|GetSneakingComponent))))
    (EventHandler|HandleFootsteps DeltaSeconds)))

(fn GetSounds
  (params (Type :type EMovementSoundTypes%20Enum :default "NewEnumerator1") (Surface :type EPhysicalSurface%20Enum :default "SurfaceType_Default"))
  ;[1 1 1] Finds sounds with the given sound type and surface type from the sound data table. Prints warning messages if a sound could not be found.
  (bind _outrownames (DataTable|GetDataTableRowNames "/Game/Motion/Blueprints/DT_MovementSounds.DT_MovementSounds"))
  (for _array_element _outrownames
    (bind _returnvalue (Utilities|GetDataTableRow "/Game/Motion/Blueprints/DT_MovementSounds.DT_MovementSounds" _array_element)
      (:then
        (if (|IsValidSound _returnvalue Type Surface)
          (Utilities|Array|Add (LocalVariables|GetSounds) _returnvalue)))))
  (if (Utilities|StructMovementSoundAny (LocalVariables|GetSounds))
    (return (LocalVariables|GetSounds))
    (else
      (if (Variables|Configuration|GetbShowDebugInformation)
        (Development|PrintString (Utilities|String|Append "UNABLE TO FIND SOUND FOR TYPE " (Utilities|String|EnumtoString Type) " AND SURFACE " (Utilities|String|EnumtoString Surface)) true true "(R=1.000000,G=0.000000,B=0.000000,A=1.000000)" 5.0))
      (return 0))))

(fn GetSoundTypeforMovementMode
  (params (bJumped :type Boolean))
  ;[1 1 1] Returns the proper EMovementSoundType given if the player has jumped or not.
  (if bJumped
    (return "NewEnumerator5")
    (else
      (return "NewEnumerator6"))))

(fn GetCurrentFloorSurface
  (params (HitResult :type Hit%20Result%20Structure))
  ;[1 1 1] Returns the current floor's surface type. Returns "Default" is none is set.
  (Utilities|IsValid (.hitactor HitResult)
    (:Is%20Valid
      (return (Variables|/Script/PhysicsCore.PhysicalMaterial|GetSurfaceType (.physmat HitResult))))
    (:Is%20Not%20Valid
      (return "SurfaceType_Default"))))

(fn GetRandomSound
  (params (Type :type EMovementSoundTypes%20Enum :default "NewEnumerator1") (Sounds :type Array%20of%20F%20Struct%20Movement%20Sound%20Structures))
  (bind _outitem (Utilities|Array|Random Sounds))
  (bind _movementsoundoverrideidentifiers (Variables|Configuration|GetMovementSoundOverrideIdentifiers))
  (bind (_value _returnvalue) (Utilities|Map|Find _movementsoundoverrideidentifiers Type))
  ;[1 1 1] Returns a random sound from an array of sounds. If a override sound is set for the given type, it will choose a random identifier sound.
  (if _returnvalue
    (bind _outrownames (DataTable|GetDataTableRowNames "/Game/Motion/Blueprints/DT_MovementSounds.DT_MovementSounds"))
    (for _array_element _outrownames
      (bind _returnvalue_2 (Utilities|GetDataTableRow "/Game/Motion/Blueprints/DT_MovementSounds.DT_MovementSounds" _array_element)
        (:then
          (if (Utilities|Array|ContainsItem (.ConditionIdentifier (Utilities|Struct|BreakFStructMovementSound _returnvalue_2)) _value)
            (Utilities|Array|Add (LocalVariables|GetSoundsWithIdentifier) _returnvalue_2)))))
    (bind _output_get (Variables|ComponentData|SetCurrentSound (.OutItem (Utilities|Array|Random (LocalVariables|GetSoundsWithIdentifier)))))
    (return _output_get)
    (else
      (Variables|ComponentData|SetCurrentSound _outitem)
      (return _outitem))))

(fn GetSoundTypeforSide
  (params (bIsLeft :type Boolean) (bIsSprinting :type Boolean) (bIsCrouching :type Boolean))
  ;[1 1 1] Returns the proper EMovementSoundType given the step side, sprint & crouch state
  (if bIsSprinting
    (return (|GetSprintSoundType bIsLeft))
    (elif bIsCrouching
      (return (|GetCrouchSoundType bIsLeft))
      (else
        (return (|GetStepSoundType bIsLeft))))))

(fn GetSoundVolume
  (params (Sound :type F%20Struct%20Movement%20Sound%20Structure))
  (bind (_type _soundcue) (Utilities|Struct|BreakFStructMovementSound Sound))
  ;[1 1 1] Returns the volume for a sound. If bUseSpeedForVolumeAdjust is true, it will adjust the volume according to the player's speed.
  (if (and (Utilities|IsFootstep _type) (Variables|Configuration|GetbUseSpeedForVolumeAdjustment))
    (return (|GetVolumeAdjustedToSpeed _soundcue))
    (else
      (return (Variables|/Script/Engine.SoundCue|GetVolumeMultiplier _soundcue)))))

(fn PrintDebugInformation
  (bind _currentsound (Variables|ComponentData|GetCurrentSound))
  ;[1 1 1] Prints useful information on the screen. Helpful for debugging.
  (if (Variables|Configuration|GetbShowDebugInformation)
    (for _array_element (.conditionidentifier (Variables|ComponentData|GetCurrentSound))
      (LocalVariables|SetConditionIdentifierString (Utilities|String|Append (LocalVariables|GetConditionIdentifierString) ", " _array_element)))
    (Development|PrintString (Utilities|String|Append "MoveSoundTime: " (Utilities|String|ToString(Float) (Variables|ComponentData|GetMoveSoundTime)) " 
Is Left: " (Utilities|String|ToString(Boolean) (Variables|States|GetbIsLeftStep)) " 
Current Sound: " (Class|KismetSystemLibrary|GetPathName (.soundcue _currentsound)) " 
Current Sound Surface: " (Utilities|String|EnumtoString (.surface _currentsound)) " 
Current Sound Condition Identifier: " (LocalVariables|GetConditionIdentifierString)) true false "(R=0.725896,G=0.000000,B=1.000000,A=1.000000)" 0.001)))

(fn HandleJumpLandSounds
  (params (PreviousMovementMode :type EMovementMode%20Enum :default "MOVE_None"))
  (bind (_start _end _x_y _z) (|GetTraceParams))
  ;[1 1 1] Handles landing sounds. Detects the floor beneath the player, its surface and then chooses a sound fit for that surface.
  (Variables|States|SetbIsLeftStep false)
  (if (|IsFallingAfterWalking PreviousMovementMode)
    (bind _outhit (Collision|BoxTraceByChannel _start _end (Math|Vector|MakeVector _x_y _x_y _z) "0, 0, 0" "TraceTypeQuery1" false 0 "None")) ; We trace here again because CurrentFloor from the Character can sometimes return null even if there is a floor below.
    (LocalVariables|SetHitResult _outhit)
    (LocalVariables|SetbJumped true)
    (else
      (LocalVariables|SetHitResult (.hitresult (Variables|/Script/Engine.CharacterMovementComponent|GetCurrentFloor (Variables|/Game/Motion/Blueprints/Character/BP_CharacterCoreComponent.BP_CharacterCoreComponent_C|GetCharacterMovement (Variables|Default|GetCharacterCoreComponent)))))))
  (bind _selectedsound (|GetSoundForSurfaceAndMovementType)
    (:Is%20Valid
      (LocalVariables|SetSelectedSound _selectedsound)
      (Getters|GetSoundVolume (LocalVariables|GetSelectedSound))
      (Audio|SpawnSoundAttached (.soundcue (LocalVariables|GetSelectedSound)) (Variables|/Script/Engine.Actor|GetRootComponent (Components|GetOwner)) "None" "0, 0, 0" "0, 0, 0" "KeepRelativeOffset" false 1.0 1.0 0.0 0 0))))

(fn HandleFootsteps
  (params (DeltaSeconds :type Float%20%28double-precision%29))
  ;[1 1 1] Handles footsteps & footstep timer. Checks if the player should trigger another sound to be played, if they are fast enough to play a sound and the selection of a sound with volume adjustment for crouching.
  (|GetPlayerVelocity)
  (if (|IsNotFalling)
    (if (> (Variables|ComponentData|GetMoveSoundTime) 0.0)
      (|UpdateSoundTime DeltaSeconds)
      (if (not (> (Variables|ComponentData|GetMoveSoundTime) 0.0))
        (bind _returnvalue (|GetIsSpeedOverThresholdForPlayingSounds :!label _label))
        (if _returnvalue
          (|SetNewSoundTime)
          (bind _selectedsound (|GetSound))
          (bind _volume (Getters|GetSoundVolume _selectedsound))
          (Audio|SpawnSoundAttached (.SoundCue (Utilities|Struct|BreakFStructMovementSound _selectedsound)) (Variables|/Script/Engine.Actor|GetRootComponent (Components|GetOwner)) "None" "0, 0, 0" "0, 0, 0" "KeepRelativeOffset" false _volume 1.0 0.0 0 0)
          (Variables|States|SetbIsLeftStep (not (Variables|States|GetbIsLeftStep)))))
      (else
        (goto _label)))))