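; BP_SneakingComponent is a character component that slows walk speed while the player sneaks, with hold or toggle input.
; It binds the character's sneak key events and, on tick, allows sneaking only when not falling or sprinting.
; While moving, a deceleration curve over key-down time eases the speed adjustment, registered through the core component; standing still applies it fully.
; Reset removes the adjustment, and optional on-screen debug prints while not sneaking.
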(event Custom|Event%20On%20Sneak%20Released
  ;[0.03922 0.1529 0.251] Event Graph
  (EventHandler|HandleonSneakReleased))

(event Custom|Event%20On%20Sneak%20Pressed
  ;[0.03922 0.1529 0.251] Event Graph
  (EventHandler|HandleonSneakPressed))

(event EventBeginPlay
  ;[0.03922 0.1529 0.251] Event Graph
  (|CallParentFunction)
  (EventHandler|HandleonEventBeginPlay (delegate Custom|Event%20On%20Sneak%20Pressed) (delegate Custom|Event%20On%20Sneak%20Released)))

(event EventTick
  (params (DeltaSeconds :type Float%20%28single-precision%29))
  ;[0.03922 0.1529 0.251] Event Graph
  (EventHandler|HandleonEventTick DeltaSeconds))

(fn HandleonEventBeginPlay
  (params (EventOnSneakKeyPressedDelegate :type Delegate%20%28by%20ref%29) (EventOnSneakKeyReleasedDelegate :type Delegate%20%28by%20ref%29))
  ;[1 1 1] Called when "Event Begin Play" gets called. Sets up events and saves component references.
  (Utilities|FlowControl|Sequence
    (:then_0
      ;;[1 1 1] Find and save core component & sprinting component in Owner
      (bind _actorcomponent (Default|GetComponent (Variables|Default|GetCharacterCoreComponent) "/Game/Motion/Blueprints/Components/BP_SprintingComponent.BP_SprintingComponent_C" self))
      (bind _asbp_sprinting_component (Utilities|Casting|CastToBP_SprintingComponent _actorcomponent))
      (Variables|Default|SetSprintComponent _asbp_sprinting_component))
    (:then_1
      ;;[1 1 1] Bind Sneak Events
      (EventDispatchers|BindEventtoOnSneakKeyPressed (Variables|/Game/Motion/Blueprints/Character/BP_CharacterCoreComponent.BP_CharacterCoreComponent_C|GetCharacter (Variables|Default|GetCharacterCoreComponent)) EventOnSneakKeyPressedDelegate)
      (EventDispatchers|AssignOnSneakKeyReleased (Variables|/Game/Motion/Blueprints/Character/BP_CharacterCoreComponent.BP_CharacterCoreComponent_C|GetCharacter (Variables|Default|GetCharacterCoreComponent)) EventOnSneakKeyReleasedDelegate))))

(fn HandleonEventTick
  (params (DeltaTime :type Float%20%28double-precision%29))
  ;[1 1 1] Core logic handlers. Handles Sneak Inputs, Updates timers and prints Debug information
  (if (Variables|Configuration|GetbIsEnabled) ; Only update if component is enabled, otherwise just update Debug text
    (bind __ (Getters|IsAllowedtoSneak))
    (if __ ; Also, only update when we are jumping to avoid unneccessary computations
      (Utilities|FlowControl|Sequence
        (:then_0
          (Manipulators|UpdateDeltaSeconds DeltaTime) ; Updates all timers we use for calculations.\nWe use a custom tick rate as Delta Seconds from Event Tick is not a consistent value
        )
        (:then_1
          (Manipulators|LerpTowardsSneakingSpeed) ; Calculates the speed for the current tick that should be set as maximum speed for the player
        ))
      (else
        (Utilities|FlowControl|Sequence
          (:then_0
            (if (Variables|States|GetbIsSneaking)
              (Manipulators|ResetSneaking) ; Removes the sneak speed adjustment
            ))
          (:then_1
            (Debug|PrintDebugInformation :!label _label)))))
    (else
      (goto _label))))

(fn HandleonSneakPressed
  ;[1 1 1] Called when the player presses the sneak key. Resets timers and sets sneak state.
  (if (Variables|Configuration|GetbIsEnabled)
    (if (Variables|Configuration|GetbIsInputToggle)
      (if (Variables|States|GetbIsSneaking)
        (Manipulators|ResetSneaking)
        (else
          (Variables|States|SetbIsHoldingSneakKey true :!label _label)
          (Variables|ComponentData|SetActiveDeltaSeconds 0.0)
          (Variables|ComponentData|SetActiveSneakKeyDownSeconds 0.0)))
      (else
        (goto _label)))))

(fn HandleonSneakReleased
  ;[1 1 1] Called when the player releases the sneak key. Resets sneaking and its state.
  (if (and (Variables|Configuration|GetbIsEnabled) (not (Variables|Configuration|GetbIsInputToggle)))
    (Manipulators|ResetSneaking)))

(fn UpdateDeltaSeconds
  (params (DeltaSeconds :type Float%20%28double-precision%29))
  ;[1 1 1] Update the progress on the sneak timer.
  (bind _updatedactivedeltaseconds (CallFunction|UpdateSeconds (Variables|ComponentData|GetActiveSneakKeyDownSeconds) (Variables|Constants|GetDeltaTickRate) DeltaSeconds false))
  (Variables|ComponentData|SetActiveSneakKeyDownSeconds _updatedactivedeltaseconds))

(fn ResetSneaking
  ;[1 1 1] Removes speed penalty from sneaking.
  (Variables|States|SetbIsSneaking false)
  (Variables|States|SetbIsHoldingSneakKey false)
  (Default|RemoveWalkSpeed (Variables|Default|GetCharacterCoreComponent) self))

(fn LerpTowardsSneakingSpeed
  ;[1 1 1] Lerps towards sneak speed and updates the speed for this component in the core component.
  (if (Utilities|IsPlayerMoving)
    (Variables|ComponentData|SetCurrentSneakSpeedAdjustment (|GetSneakSpeed))
    (Default|AddWalkSpeed (Variables|Default|GetCharacterCoreComponent) self (Variables|ComponentData|GetCurrentSneakSpeedAdjustment) false)
    (if (|IsCurrentAdjustmentNearTarget)
      (Variables|States|SetbIsSneaking true :!label _label))
    (else
      (Default|AddWalkSpeed (Variables|Default|GetCharacterCoreComponent) self (Variables|Configuration|GetSneakSpeedAdjustment) false)
      (goto _label))))

(fn PrintDebugInformation
  ;[1 1 1] Prints useful information on the screen. Helpful for debugging.
  (if (Variables|Configuration|GetbShowDebugInformation)
    (bind _velocity (Default|GetSquaredPlayerVelocity (Variables|/Game/Motion/Blueprints/Character/BP_CharacterCoreComponent.BP_CharacterCoreComponent_C|GetCharacter (Variables|Default|GetCharacterCoreComponent))))
    (Development|PrintString (Utilities|String|Append "Current Walkspeed (Component): " (Utilities|String|ToString(Float) (Variables|ComponentData|GetCurrentSneakSpeedAdjustment)) " 
Current Walkspeed (Character): " (Utilities|String|ToString(Float) _velocity) " 
Is Sneaking: " (Utilities|String|ToString(Boolean) (Variables|States|GetbIsSneaking)) " 
Active Delta Seconds: " (Utilities|String|ToString(Float) (Variables|ComponentData|GetActiveDeltaSeconds)) " 
Current Target Rotation: " (Utilities|String|ToString(Rotator) (Variables|ComponentData|GetCurrentTargetRotation)) " 
Real Camera Rotation: " (Utilities|String|ToString(Rotator) (Variables|/Script/Engine.SceneComponent|GetRelativeRotation (Variables|/Game/Motion/Blueprints/Character/BP_CharacterCoreComponent.BP_CharacterCoreComponent_C|GetCamera (Variables|Default|GetCharacterCoreComponent)))) " 
Is Holding Sneak Key: " (Utilities|String|ToString(Boolean) (Variables|States|GetbIsHoldingSneakKey)) " 
Is Input Toggle: " (Utilities|String|ToString(Boolean) (Variables|Configuration|GetbIsInputToggle))) true false "(R=0.486456,G=1.000000,B=0.000000,A=1.000000)" 0.001)))

(fn IsAllowedtoSneak
  ;[1 1 1] Returns true if the player is allowed to sneak. Returns false if the player is falling, not holding the sprint key, or sprinting.
  (return (Math|Boolean|ANDBoolean (|IsNotFalling) (Variables|States|GetbIsHoldingSneakKey) (|IsNotSprinting))))