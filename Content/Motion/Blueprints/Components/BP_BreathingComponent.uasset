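; Motion component that drives an idle breathing effect through a camera offset curve while the character stands still.
; On BeginPlay it binds to the character's velocity events and registers a looping, reversing curve with the CharacterCurveManager.
; When enabled, it pauses the curve as movement begins and unpauses it when movement stops.
; When a transition reaches its maximum, it adopts that transition's curve as the camera offset curve.
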(event Custom|Event%20On%20Velocity%20Stop
  ;[0 0.1429 1] Event Graph
  (EventHandler|HandleonVelocityStop))

(event Custom|Event%20On%20Velocity%20Begin
  ;[0 0.1429 1] Event Graph
  (EventHandler|HandleonVelocityBegin))

(event EventBeginPlay
  ;[0 0.1429 1] Event Graph
  (|CallParentFunction)
  (EventHandler|HandleonEventBeginPlay (delegate Custom|Event%20On%20Velocity%20Begin) (delegate Custom|Event%20On%20Velocity%20Stop)))

(event EventOnTransitionMaximum
  (params (TransitionData :type F%20Struct%20Motion%20Curve%20Transition%20Structure))
  ;[0 0.1429 1] Event Graph
  (EventHandler|HandleonTransitionMaximum TransitionData))

(fn HandleonEventBeginPlay
  (params (EventOnVelocityBeginDelegate :type Delegate%20%28by%20ref%29) (EventOnVelocityStopDelegate :type Delegate%20%28by%20ref%29))
  ;[1 1 1] Called when "Event Begin Play" gets called. Sets up events & creates curve.
  (Utilities|FlowControl|Sequence
    (:then_0
      ;;[1 1 1] Bind Velocity Events
      (EventDispatchers|BindEventtoOnVelocityBegin (Variables|/Game/Motion/Blueprints/Character/BP_CharacterCoreComponent.BP_CharacterCoreComponent_C|GetCharacter (Variables|Default|GetCharacterCoreComponent)) EventOnVelocityBeginDelegate)
      (EventDispatchers|BindEventtoOnVelocityStop (Variables|/Game/Motion/Blueprints/Character/BP_CharacterCoreComponent.BP_CharacterCoreComponent_C|GetCharacter (Variables|Default|GetCharacterCoreComponent)) EventOnVelocityStopDelegate))
    (:then_1
      ;;[1 1 1] Create Active Curve
      (Default|AddCurve (Variables|Default|GetCharacterCurveManager) (Utilities|Struct|MakeFStructMotionCurve (Utilities|Struct|MakeFStructMotionCurveIdentifier self (Variables|Configuration|GetCameraOffsetCurve) (Variables|Constants|GetCurveType)) (Utilities|Struct|MakeFStructMotionCurveConfiguration true true false (Variables|Constants|GetDeltaTickRate)))))))

(fn HandleonVelocityBegin
  ;[1 1 1] Called when the player moves.
  (if (Variables|Configuration|GetbIsEnabled)
    (Default|PauseCurve (Variables|Default|GetCharacterCurveManager) (Utilities|Struct|MakeFStructMotionCurveIdentifier self (Variables|Configuration|GetCameraOffsetCurve) (Variables|Constants|GetCurveType)) false)))

(fn HandleonVelocityStop
  ;[1 1 1] Called when the player stops moving.
  (if (Variables|Configuration|GetbIsEnabled)
    (Default|UnpauseCurve (Variables|Default|GetCharacterCurveManager) (Utilities|Struct|MakeFStructMotionCurveIdentifier self (Variables|Configuration|GetCameraOffsetCurve) (Variables|Constants|GetCurveType)) false)))

(fn HandleonTransitionMaximum
  (params (TransitionData :type F%20Struct%20Motion%20Curve%20Transition%20Structure))
  ;[1 1 1] Called when a transition reaches it's peak. Used to update the offset curve configuration.
  (|CallParentFunction TransitionData)
  (Variables|Configuration|SetCameraOffsetCurve (.curvevector (.Identifier (Utilities|Struct|BreakFStructMotionCurveTransitionConfiguration (.TransitionConfiguration (Utilities|Struct|BreakFStructMotionCurveTransition TransitionData)))))))