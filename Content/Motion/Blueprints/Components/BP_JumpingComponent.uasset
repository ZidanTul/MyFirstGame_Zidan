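; Character component that adds jump stamina and procedural camera motion for jumps and landings.
; Binds character jump, landing and movement events, zeroing stamina after each jump lands, then recovering it on tick to gate jumping and scale jump velocity.
; Airborne camera rotation follows a stamina-scaled vector curve, while landings lerp into a velocity-based pitch bounce that reverses back.
; Each tick sends the resulting rotation to CharacterCoreComponent as a camera offset.
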(event Custom|EventOnMovementModeChanged
  (params (Previous%20Movement%20Mode :type EMovementMode%20Enum :default "MOVE_None") (New%20Movement%20Mode :type EMovementMode%20Enum :default "MOVE_None") (Previous%20Custom%20Mode :type Byte) (New%20Custom%20Mode :type Byte))
  ;[0.03922 0.1529 0.251] Event Graph
  (EventHandler|HandleonMovementModeChanged Previous%20Movement%20Mode New%20Movement%20Mode))

(event Custom|EventOnJumpedReleased
  ;[0.03922 0.1529 0.251] Event Graph
  (EventHandler|HandleonJumpReleased))

(event Custom|EventOnJumpJumped
  ;[0.03922 0.1529 0.251] Event Graph
  (EventHandler|HandleonJumpJumped))

(event Custom|EventOnJumpStopped
  ;[0.03922 0.1529 0.251] Event Graph
  (EventHandler|HandleonJumpStopped))

(event Custom|EventOnPlayerLanded
  ;[0.03922 0.1529 0.251] Event Graph
  (EventHandler|HandleonPlayerLanded))

(event Custom|EventOnJumpedPressed
  ;[0.03922 0.1529 0.251] Event Graph
  (EventHandler|HandleonJumpPressed))

(event EventBeginPlay
  ;[0.03922 0.1529 0.251] Event Graph
  (|CallParentFunction)
  (EventHandler|HandleonEventBeginPlay (delegate Custom|EventOnJumpedPressed) (delegate Custom|EventOnJumpedReleased) (delegate Custom|EventOnJumpJumped) (delegate Custom|EventOnJumpStopped) (delegate Custom|EventOnPlayerLanded) (delegate Custom|EventOnMovementModeChanged)))

(event EventTick
  (params (DeltaSeconds :type Float%20%28single-precision%29))
  ;[0.03922 0.1529 0.251] Event Graph
  (EventHandler|HandleonEventTick DeltaSeconds))

(fn HandleonEventBeginPlay
  (params (EventOnJumpPressedDelegate :type Delegate%20%28by%20ref%29) (EventOnJumpReleasedDelegate :type Delegate%20%28by%20ref%29) (EventOnJumpJumpedDelegate :type Delegate%20%28by%20ref%29) (EventOnJumpStoppedDelegate :type Delegate%20%28by%20ref%29) (EventOnJumpLandedDelegate :type Delegate%20%28by%20ref%29) (EventOnMovementModeChangedDelegate :type Delegate%20%28by%20ref%29))
  (bind _charactercorecomponent (Variables|Default|GetCharacterCoreComponent))
  (bind _character (Variables|/Game/Motion/Blueprints/Character/BP_CharacterCoreComponent.BP_CharacterCoreComponent_C|GetCharacter _charactercorecomponent))
  ;[1 1 1] Called when "Event Begin Play" gets called. Sets up events and saves base values.
  (Utilities|FlowControl|Sequence
    (:then_0
      ;;[1 1 1] Get Reference Jump Velocity
      (Variables|ComponentData|SetBaseJumpZVelocity (Variables|/Script/Engine.CharacterMovementComponent|GetJumpZVelocity (Variables|/Game/Motion/Blueprints/Character/BP_CharacterCoreComponent.BP_CharacterCoreComponent_C|GetCharacterMovement (Variables|Default|GetCharacterCoreComponent)))))
    (:then_1
      ;;[1 1 1] Bind Jump and Landing Events
      (Utilities|FlowControl|Sequence
        (:then_0
          (EventDispatchers|BindEventtoOnJumpPressed _character EventOnJumpPressedDelegate))
        (:then_1
          (EventDispatchers|BindEventtoOnJumpReleased _character EventOnJumpReleasedDelegate))
        (:then_2
          (EventDispatchers|BindEventtoOnJumpJumped _character EventOnJumpJumpedDelegate))
        (:then_3
          (EventDispatchers|BindEventtoOnJumpStopped _character EventOnJumpStoppedDelegate))
        (:then_4
          (EventDispatchers|BindEventtoOnPlayerLanded _character EventOnJumpLandedDelegate))
        (:then_5
          (EventDispatchers|BindEventtoOnMovementModeChanged _character EventOnMovementModeChangedDelegate))))))

(fn HandleonEventTick
  (params (DeltaSeconds :type Float%20%28double-precision%29))
  ;[1 1 1] Core logic handlers. Handles rotation and stamina updates.
  (if (Variables|Configuration|GetbIsEnabled)
    (Manipulators|UpdateDeltaSeconds DeltaSeconds)
    (Utilities|FlowControl|Sequence
      (:then_0
        (Manipulators|UpdateFallingVelocity))
      (:then_1
        (Manipulators|UpdateTargetRotation))
      (:then_2
        (Manipulators|MoveCameratoTargetRotation))
      (:then_3
        (Manipulators|ValidateRotationTarget))
      (:then_4
        (Manipulators|UpdateStamina))
      (:then_5
        (Debug|PrintDebugInformation :!label _label)))
    (else
      (goto _label))))

(fn HandleonJumpPressed
  ;[1 1 1] Called when the player presses the Jump key. Adjusts the JumpZ Velocity based on the available stamina
  (if (Variables|Configuration|GetbIsEnabled)
    (Variables|/Script/Engine.CharacterMovementComponent|SetJumpZVelocity (Variables|/Game/Motion/Blueprints/Character/BP_CharacterCoreComponent.BP_CharacterCoreComponent_C|GetCharacterMovement (Variables|Default|GetCharacterCoreComponent)) (|CalculateJumpVelocity))))

(fn HandleonJumpReleased
  ;[1 1 1] Called when the player releases the jump key. Currently unused.
)

(fn HandleonJumpJumped
  ;[1 1 1] Called when after a jump was executed. Useful for post-jump logic.
  (if (Variables|Configuration|GetbIsEnabled)
    (Manipulators|AbortBounce)
    (Variables|States|SetbIsJumping true)))

(fn HandleonJumpStopped
  ;[1 1 1] Called after "Jump Stopped" has executed. Currenly unused.
)

(fn UpdateTargetRotation
  ;[1 1 1] Handles Rotation updates given the current player state
  (Utilities|FlowControl|Sequence
    (:then_0
      (|HandleNotBouncingAndJumping)
      (return))
    (:then_1
      (|HandleBouncingAndNotJumping)
      (return))
    (:then_2
      (|HandleBouncingAndJumping)
      (return))))

(fn UpdateDeltaSeconds
  (params (DeltaSeconds :type Float%20%28double-precision%29))
  ;[1 1 1] Updates progress on either the jumping camera curve or the bounce camera curve, depending on the player's state
  (if (Variables|States|GetbIsJumping)
    (bind _updateddeltaseconds (CallFunction|UpdateSecondswithCurve (Variables|Configuration|GetCameraBounceCurve) (Variables|ComponentData|GetActiveDeltaSeconds) (Variables|Constants|GetDeltaTickRate) DeltaSeconds false))
    (Variables|ComponentData|SetActiveDeltaSeconds _updateddeltaseconds)
    (elif (Variables|States|GetbIsBouncing)
      (bind _updatedactivedeltaseconds (CallFunction|UpdateSeconds (Variables|ComponentData|GetActiveDeltaSeconds) (Variables|Constants|GetDeltaTickRate) DeltaSeconds false))
      (Variables|ComponentData|SetActiveDeltaSeconds _updatedactivedeltaseconds))))

(fn ValidateRotationTarget
  ;[1 1 1] Checks if we are close to the end of the bounce and stops it if so.
  (if (and (Variables|States|GetbIsBounceReversed) (Utilities|IsTargetRotationNearBounceRotation))
    (Manipulators|AbortBounce)))

(fn MoveCameratoTargetRotation
  ;[1 1 1] Adds the target offset to the core component
  ;;[1 0 0] Manually calling "Add Camera Offset" is deprecated and will soon be removed.
  (Default|AddCameraOffset (Variables|Default|GetCharacterCoreComponent) (Utilities|Struct|MakeFStructCameraCurve (Utilities|Struct|MakeFStructMotionCurve (Utilities|Struct|MakeFStructMotionCurveIdentifier self (Variables|Constants|GetCurveType)) "(bShouldLoop_9_666576974F883E228DB125BEAF8A60D0=False,bShouldReverse_11_5F50FB6143A47A5D2F479EBAAD96DD32=False,bHasPriority_14_E460BB484F65E64110A48FB2A6E597CB=False,Tickrate_16_7FAB02194AA4ADC275096CBD3E8829FC=0.000000)" true) (Variables|ComponentData|GetCurrentTargetRotation))))

(fn HandleImpactBounce
  ;[1 1 1] Sets the bounce target and enables bounce state.
  (Variables|ComponentData|SetBounceTargetRotation (Math|Rotator|MakeRotator 0.0 (|GetBounceRotationPitch) 0.0))
  (Variables|States|SetbIsBouncing true))

(fn AbortBounce
  ;[1 1 1] Resets bounce state and saves the current target rotation
  (Variables|States|SetbIsBouncing false)
  (Variables|States|SetbIsBounceReversed false)
  (Variables|ComponentData|SetStaminaStartRotation (Variables|ComponentData|GetCurrentTargetRotation))
  (Variables|ComponentData|SetActiveDeltaSeconds 0.0))

(fn PrintDebugInformation
  ;[1 1 1] Prints useful information on the screen. Helpful for debugging.
  (if (Variables|Configuration|GetbShowDebugInformation)
    (Development|PrintString (Utilities|String|Append " 
Active Delta Seconds: " (Utilities|String|ToString(Float) (Variables|ComponentData|GetActiveDeltaSeconds)) " 
Current Target Rotation: " (Utilities|String|ToString(Rotator) (Variables|ComponentData|GetCurrentTargetRotation)) " 
Real Camera Rotation: " (Utilities|String|ToString(Rotator) (Variables|/Script/Engine.SceneComponent|GetRelativeRotation (Variables|/Game/Motion/Blueprints/Character/BP_CharacterCoreComponent.BP_CharacterCoreComponent_C|GetCamera (Variables|Default|GetCharacterCoreComponent)))) " 
Bounce Target Rotation: " (Utilities|String|ToString(Rotator) (Variables|ComponentData|GetBounceTargetRotation)) " 
Is Jumping: " (Utilities|String|ToString(Boolean) (Variables|States|GetbIsJumping)) " 
Is Bouncing: " (Utilities|String|ToString(Boolean) (Variables|States|GetbIsBouncing)) " 
Is Bounce Reversed: " (Utilities|String|ToString(Boolean) (Variables|States|GetbIsBounceReversed)) " 
Stamina Recovery Seconds: " (Utilities|String|ToString(Float) (Variables|ComponentData|GetStaminaRecoverySeconds)) " 
Jump Stamina: " (Utilities|String|ToString(Float) (Variables|ComponentData|GetJumpStamina)) " 
Current JumpZ Velocity:" (Utilities|String|ToString(Float) (Variables|/Script/Engine.CharacterMovementComponent|GetJumpZVelocity (Variables|/Game/Motion/Blueprints/Character/BP_CharacterCoreComponent.BP_CharacterCoreComponent_C|GetCharacterMovement (Variables|Default|GetCharacterCoreComponent)))) " 
Stamina Camera Offset: " (Utilities|String|ToString(Rotator) (Variables|ComponentData|GetStaminaStartRotation))) true false "(R=0.043207,G=1.000000,B=0.000000,A=1.000000)" 0.001)))

(fn HandleonPlayerLanded
  ;[1 1 1] Called when the player has landed on the floor. Clears stamina and updates jump states.
  (if (and (Variables|Configuration|GetbIsEnabled) (Variables|States|GetbIsJumping))
    (Variables|ComponentData|SetActiveDeltaSeconds 0.0)
    (Variables|ComponentData|SetJumpStamina 0.0)
    (Variables|States|SetbIsJumping false)
    (Variables|States|SetbIsRecovering true)
    (Variables|ComponentData|SetStaminaStartRotation "0, 0, 0"))
  (Manipulators|HandleImpactBounce))

(fn UpdateStamina
  (bind (_newstamina _bisstillrecovering) (|IsStillRecoveringAfterTick))
  ;[1 1 1] Updates Stamina and determines if the player is capable of jumping (has enough stamina)
  (if (Variables|States|GetbIsRecovering)
    (if _bisstillrecovering
      (Variables|ComponentData|SetJumpStamina _newstamina)
      (Manipulators|SetPlayerJumpEnabled (>= (Variables|ComponentData|GetJumpStamina) (Variables|Configuration|GetJumpStaminaThreshold)))
      (else
        (Manipulators|ResetStamina)))))

(fn ResetStamina
  ;[1 1 1] Resets stamina values.
  (Variables|ComponentData|SetJumpStamina 1.0)
  (Variables|States|SetbIsRecovering false))

(fn SetPlayerJumpEnabled
  (params (bCanJump :type Boolean))
  (bind _charactercorecomponent (Variables|Default|GetCharacterCoreComponent))
  (bind _charactermovement (Variables|/Game/Motion/Blueprints/Character/BP_CharacterCoreComponent.BP_CharacterCoreComponent_C|GetCharacterMovement _charactercorecomponent))
  ;[1 1 1] Sets the ability to jump in the characters movement component.
  (bind _structout (Utilities|Struct|SetmembersinNavAgentProperties (Variables|/Script/Engine.NavMovementComponent|GetNavAgentProps _charactermovement) bCanJump))
  (Variables|/Script/Engine.NavMovementComponent|SetNavAgentProps _charactermovement _structout))

(fn HandleonMovementModeChanged
  (params (PreviousMovementMode :type EMovementMode%20Enum :default "MOVE_None") (NewMovementMode :type EMovementMode%20Enum :default "MOVE_None"))
  ;[1 1 1] Called when the movement mode changes (e.g. from falling to walking)
  (Variables|States|SetbIsFalling (Utilities|Enum|Equal(Enum) NewMovementMode "MOVE_Falling")))

(fn UpdateFallingVelocity
  ;[1 1 1] Updates last known falling velocity if we fall. Used to prevent camera bounce from little drops.
  (if (Variables|States|GetbIsFalling)
    (Variables|ComponentData|SetLastKnownFallingVelocity (* (Math|Float|Min(Float) 0.0 (.z (Pawn|Components|CharacterMovement|GetLastUpdateVelocity (Variables|/Game/Motion/Blueprints/Character/BP_CharacterCoreComponent.BP_CharacterCoreComponent_C|GetCharacterMovement (Variables|Default|GetCharacterCoreComponent))))) -1.0))))