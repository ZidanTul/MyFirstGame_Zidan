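; Character component that provides smooth crouching with hold or toggle input, working through a CharacterCoreComponent.
; Each tick it interpolates capsule half height and camera offset toward crouched or standing values, keeping the capsule base planted while walking.
; Uncrouching runs overlap and trace checks to wait out blocking geometry.
; A walk speed penalty applies when fully crouched, and crouch progress events notify listeners, useful for sliding.
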(event Custom|EventOnMovementModeChange
  (params (Previous%20Movement%20Mode :type EMovementMode%20Enum :default "MOVE_None") (New%20Movement%20Mode :type EMovementMode%20Enum :default "MOVE_None") (Previous%20Custom%20Mode :type Byte) (New%20Custom%20Mode :type Byte))
  ;[0.03922 0.1529 0.251] Event Graph
  (EventHandler|HandleonMovementModeChanged Previous%20Movement%20Mode New%20Movement%20Mode Previous%20Custom%20Mode New%20Custom%20Mode))

(event Custom|EventOnCrouchPressed
  ;[0.03922 0.1529 0.251] Event Graph
  (EventHandler|HandleonCrouchPressed))

(event Custom|EventOnCrouchReleased
  ;[0.03922 0.1529 0.251] Event Graph
  (EventHandler|HandleonCrouchReleased))

(event EventBeginPlay
  ;[0.03922 0.1529 0.251] Event Graph
  (|CallParentFunction)
  (EventHandler|HandleonEventBeginPlay (delegate Custom|EventOnMovementModeChange) (delegate Custom|EventOnCrouchPressed) (delegate Custom|EventOnCrouchReleased)))

(event EventTick
  (params (DeltaSeconds :type Float%20%28single-precision%29))
  ;[0.03922 0.1529 0.251] Event Graph
  (EventHandler|HandleonEventTick DeltaSeconds))

(fn HandleonEventBeginPlay
  (params (EventOnMovementModeChangedDelegate :type Delegate%20%28by%20ref%29) (EventOnCrouchPressedDelegate :type Delegate%20%28by%20ref%29) (EventOnCrouchReleasedDelegate :type Delegate%20%28by%20ref%29))
  (bind _charactercorecomponent (Variables|Default|GetCharacterCoreComponent))
  (bind _character (Variables|/Game/Motion/Blueprints/Character/BP_CharacterCoreComponent.BP_CharacterCoreComponent_C|GetCharacter _charactercorecomponent))
  ;[1 1 1] Called when "Event Begin Play" gets called. Sets up events and saves base values.
  (Utilities|FlowControl|Sequence
    (:then_0
      ;;[1 1 1] Get Base Values
      (Variables|ComponentData|SetBaseMaxWalkSpeed (Variables|/Script/Engine.CharacterMovementComponent|GetMaxWalkSpeed (Variables|/Game/Motion/Blueprints/Character/BP_CharacterCoreComponent.BP_CharacterCoreComponent_C|GetCharacterMovement (Variables|Default|GetCharacterCoreComponent))))
      (Variables|ComponentData|SetBaseUnscaledCapsuleRadius (Class|CapsuleComponent|GetUnscaledCapsuleRadius (Variables|/Game/Motion/Blueprints/Character/BP_CharacterCoreComponent.BP_CharacterCoreComponent_C|GetCapsule (Variables|Default|GetCharacterCoreComponent))))
      (Variables|ComponentData|SetBaseUnscaledCapsuleHalfHeight (Components|Capsule|GetUnscaledCapsuleHalfHeight (Variables|/Game/Motion/Blueprints/Character/BP_CharacterCoreComponent.BP_CharacterCoreComponent_C|GetCapsule (Variables|Default|GetCharacterCoreComponent)))))
    (:then_1
      ;;[1 1 1] Bind Events for Crouching and Movement Mode Changed
      (Utilities|FlowControl|Sequence
        (:then_0
          (EventDispatchers|BindEventtoOnMovementModeChanged _character EventOnMovementModeChangedDelegate))
        (:then_1
          (EventDispatchers|BindEventtoOnCrouchPressed _character EventOnCrouchPressedDelegate))
        (:then_2
          (EventDispatchers|BindEventtoOnCrouchReleased _character EventOnCrouchReleasedDelegate))))))

(fn HandleonEventTick
  (params (DeltaTime :type Float%20%28double-precision%29))
  ;[1 1 1] Core logic handlers. Handles Crouch Inputs and prints Debug information
  (if (Variables|Configuration|GetbIsEnabled)
    (Utilities|FlowControl|Sequence
      (:then_0
        (CrouchHandlers|HandleCrouchInput DeltaTime))
      (:then_1
        (Debug|PrintDebugInformation :!label _label)))
    (else
      (goto _label))))

(fn HandleonMovementModeChanged
  (params (PreviousMovementMode :type EMovementMode%20Enum :default "MOVE_None") (NewMovementMode :type EMovementMode%20Enum :default "MOVE_None") (PreviousCustomMode :type Byte) (NewCustomMode :type Byte))
  ;[1 1 1] Handles all Movement related changes
  (if (Variables|Configuration|GetbIsEnabled)
    (Utilities|FlowControl|Sequence
      (:then_0
        ;[1 1 1] If the player jumps or falls and isn't crouched, remove crouch speed modifiers.
        ; Useful if you intend to add in-air gameplay
        (if (and (Utilities|Enum|Equal(Enum) PreviousMovementMode "MOVE_Walking") (Utilities|Enum|Equal(Enum) NewMovementMode "MOVE_Falling"))
          (if (not (Variables|States|GetbIsCrouched))
            (Manipulators|ResetMaxWalkSpeed))))
      (:then_1
        ;[1 1 1] Update if the player maintains base location or not depending on whether or not they are walking
        (Variables|States|SetbCrouchMaintainsBaseLocation (Utilities|Enum|Equal(Enum) NewMovementMode "MOVE_Walking"))))))

(fn HandleonCrouchPressed
  ;[1 1 1] Upon crouch key-press, mark the character as wanting to crouch
  (if (Variables|Configuration|GetbIsEnabled)
    (if (Variables|Configuration|GetbIsInputToggle)
      (if (or (Variables|States|GetbIsInCrouch) (Variables|States|GetbIsCrouched))
        (CrouchHandlers|SetCrouch false)
        (else
          (CrouchHandlers|SetCrouch true :!label _label)))
      (else
        (goto _label)))))

(fn HandleonCrouchReleased
  ;[1 1 1] When releasing the crouch button, update crouch intention state
  (if (and (Variables|Configuration|GetbIsEnabled) (not (Variables|Configuration|GetbIsInputToggle)))
    (CrouchHandlers|SetCrouch false)))

(fn HandleonCrouchCrouched
  (params (HalfHeightAdjust :type Float%20%28double-precision%29))
  ;[1 1 1] Called whenever the crouch position updates. Calls event for other components that listen to crouch changes.
  ; Useful for implementing sliding.
  (if (Variables|Configuration|GetbIsEnabled)
    (if (|IsFullyCrouched HalfHeightAdjust)
      (Variables|States|SetbIsCrouched true)
      (Default|AddWalkSpeed (Variables|Default|GetCharacterCoreComponent) self (Variables|Configuration|GetCrouchSpeedPenalty) false)
      (Default|CallOnCrouchFullyCrouched)
      (else
        (Default|CallOnCrouchUpdate HalfHeightAdjust)))))

(fn HandleonCrouchUncrouched
  (params (HalfHeightAdjust :type Float%20%28double-precision%29))
  ;[1 1 1] Called whenever the uncrouch position updates. Calls event for other components that listen to uncrouch changes.
  ; Useful for implementing sliding.
  (if (Variables|Configuration|GetbIsEnabled)
    (if (|IsFullyUncrouched HalfHeightAdjust)
      (Manipulators|ResetMaxWalkSpeed)
      (Default|CallOnCrouchFullyUncrouched)
      (else
        (Default|CallOnCrouchUpdate HalfHeightAdjust)))))

(fn GetCharacterVelocity
  ;[1 1 1] Returns the player speed in units per second.
  (bind _velocity (Default|GetSquaredPlayerVelocity (Variables|/Game/Motion/Blueprints/Character/BP_CharacterCoreComponent.BP_CharacterCoreComponent_C|GetCharacter (Variables|Default|GetCharacterCoreComponent))))
  (return _velocity))

(fn PrintDebugInformation
  (bind _charactercorecomponent (Variables|Default|GetCharacterCoreComponent))
  (bind _charactermovement (Variables|/Game/Motion/Blueprints/Character/BP_CharacterCoreComponent.BP_CharacterCoreComponent_C|GetCharacterMovement _charactercorecomponent))
  ;[1 1 1] Prints useful information on the screen. Helpful for debugging.
  (if (Variables|Configuration|GetbShowDebugInformation)
    (bind _velocity (Getters|GetCharacterVelocity))
    (Development|PrintString (Utilities|String|Append "Current Max Walk Speed (Character): " (Utilities|String|ToString(Float) (Variables|/Script/Engine.CharacterMovementComponent|GetMaxWalkSpeed _charactermovement)) " 
Wants to crouch: " (Utilities|String|ToString(Boolean) (Variables|States|GetbWantsToCrouch)) " 
Is in crouch: " (Utilities|String|ToString(Boolean) (Variables|States|GetbIsInCrouch)) " 
Is crouched: " (Utilities|String|ToString(Boolean) (Variables|States|GetbIsCrouched)) " 
Current Movement Mode: " (Utilities|String|EnumtoString (Variables|/Script/Engine.CharacterMovementComponent|GetMovementMode _charactermovement)) " 
Current Custom Movement Mode. " (Utilities|String|ToString(Byte) (Variables|/Script/Engine.CharacterMovementComponent|GetCustomMovementMode _charactermovement)) " 
Player Velocity: " (Utilities|String|ToString(Float) _velocity)) true true "(R=0.014317,G=0.105290,B=1.000000,A=1.000000)" 0.001)))

(fn ResetMaxWalkSpeed
  ;[1 1 1] Removes the crouch speed modifiers
  (Default|RemoveWalkSpeed (Variables|Default|GetCharacterCoreComponent) self))

(fn HandleCrouchInput
  (params (DeltaTime :type Float%20%28double-precision%29))
  ;[1 1 1] Handles input set by player input
  (if (Variables|States|GetbWantsToCrouch)
    (CrouchHandlers|DoCrouch (Variables|Configuration|GetCrouchSpeed) DeltaTime)
    (elif (Variables|States|GetbIsInCrouch)
      (CrouchHandlers|DoUncrouch (Variables|Configuration|GetUncrouchSpeed) DeltaTime))))

(fn DoCrouch
  (params (CrouchSpeed :type Float%20%28double-precision%29) (DeltaTime :type Float%20%28double-precision%29))
  ;[1 1 1] Logic for Crouching.
  (LocalVariables|SetCrouchSpeedRef CrouchSpeed)
  (LocalVariables|SetDeltaTimeRef DeltaTime)
  (LocalVariables|SetPreAdjustmentCapsuleHeight (Components|Capsule|GetUnscaledCapsuleHalfHeight (Variables|/Game/Motion/Blueprints/Character/BP_CharacterCoreComponent.BP_CharacterCoreComponent_C|GetCapsule (Variables|Default|GetCharacterCoreComponent))))
  (if (Math|Float|NearlyEqual(Float) (LocalVariables|GetPreAdjustmentCapsuleHeight) (Variables|Configuration|GetCapulseHalfHeightWhenCrouching) 1e-06)
    (EventHandler|HandleonCrouchCrouched 0.0)
    (Variables|States|SetbIsInCrouch false)
    (else
      (LocalVariables|SetPostAdjustmentCapsuleHeight (|GetPostAdjustmentCapsuleHeight))
      (Variables|/Script/Engine.CharacterMovementComponent|SetbForceNextFloorCheck (Variables|/Game/Motion/Blueprints/Character/BP_CharacterCoreComponent.BP_CharacterCoreComponent_C|GetCharacterMovement (Variables|Default|GetCharacterCoreComponent)) true)
      (Components|Capsule|SetCapsuleHalfHeight (Variables|/Game/Motion/Blueprints/Character/BP_CharacterCoreComponent.BP_CharacterCoreComponent_C|GetCapsule (Variables|Default|GetCharacterCoreComponent)) (LocalVariables|GetPostAdjustmentCapsuleHeight) true)
      (Default|AddCameraLocationOffset (Variables|Default|GetCharacterCoreComponent) 0 (Math|Vector|Lerp(Vector) "0, 0, 0" (Variables|Configuration|GetTargetCrouchCameraOffset) (Math|Float|MapRangeClamped (LocalVariables|GetPostAdjustmentCapsuleHeight) (Variables|ComponentData|GetBaseUnscaledCapsuleHalfHeight) (Variables|Configuration|GetCapulseHalfHeightWhenCrouching) 0.0 1.0)) false)
      (Variables|/Script/Engine.CharacterMovementComponent|SetbForceNextFloorCheck (Variables|/Game/Motion/Blueprints/Character/BP_CharacterCoreComponent.BP_CharacterCoreComponent_C|GetCharacterMovement (Variables|Default|GetCharacterCoreComponent)) true) ; Forcing next floor check to ensure default Unreal Engine crouch behaviour
      (Default|AdjusttoCapsuleCenter (Variables|/Game/Motion/Blueprints/Character/BP_CharacterCoreComponent.BP_CharacterCoreComponent_C|GetCharacter (Variables|Default|GetCharacterCoreComponent))) ; Adjust Capsule Center to new, smaller center to ensure camera is in the right position
      (EventHandler|HandleonCrouchCrouched (- (LocalVariables|GetPostAdjustmentCapsuleHeight) (LocalVariables|GetPreAdjustmentCapsuleHeight))))))

(fn DoUncrouch
  (params (UncrouchSpeed :type Float%20%28double-precision%29) (DeltaTime :type Float%20%28double-precision%29))
  (bind _postadjustmentcapsuleheight (LocalVariables|GetPostAdjustmentCapsuleHeight))
  ;[1 1 1] Logic for Uncrouching. See comments for details.
  (|SetReferencesforUncrouch UncrouchSpeed DeltaTime)
  ;;[1 1 1] Check if the current Capsule Half Height is already back to normal size
  (LocalVariables|SetPreAdjustmentCapsuleHeight (Components|Capsule|GetUnscaledCapsuleHalfHeight (LocalVariables|GetCharacterCapsule)))
  (if (Math|Float|NearlyEqual(Float) (LocalVariables|GetPreAdjustmentCapsuleHeight) (Variables|ComponentData|GetBaseUnscaledCapsuleHalfHeight) 1e-05)
    (EventHandler|HandleonCrouchUncrouched 0.0)
    (Variables|States|SetbIsInCrouch false)
    (else
      (|SetUncrouchVariables)
      (if (Variables|States|GetbCrouchMaintainsBaseLocation) ; If true, crouching should keep the base of the capsule in place by lowering the center of the shrunken capsule. \nIf false, the base of the capsule moves up and the center stays in place. \n\nThe same behavior applies when the character uncrouches: \nif true, the base is kept in the same location and the center moves up. \nIf false, the capsule grows and only moves up if the base impacts something.
        (|HandleCrouchMaintainsBaseLocation)
        (else
          (|HandleCrouchDoesNotMaintainBaseLocation)))
      (if (not (LocalVariables|GetbIsBetweenGeometry)) ; If the player is still enroached at this point, don't attempt further for this tick
        (Variables|States|SetbIsCrouched false)
        (Components|Capsule|SetCapsuleHalfHeight (LocalVariables|GetCharacterCapsule) _postadjustmentcapsuleheight true)
        (Default|AddCameraLocationOffset (Variables|Default|GetCharacterCoreComponent) 0 (Math|Vector|Lerp(Vector) (Variables|Configuration|GetTargetCrouchCameraOffset) "0, 0, 0" (Math|Float|MapRangeClamped _postadjustmentcapsuleheight (Variables|Configuration|GetCapulseHalfHeightWhenCrouching) (Variables|ComponentData|GetBaseUnscaledCapsuleHalfHeight) 0.0 1.0)) false)
        (Default|AdjusttoCapsuleCenter (Variables|/Game/Motion/Blueprints/Character/BP_CharacterCoreComponent.BP_CharacterCoreComponent_C|GetCharacter (Variables|Default|GetCharacterCoreComponent)))
        (EventHandler|HandleonCrouchUncrouched (- (LocalVariables|GetPreAdjustmentCapsuleHeight) (LocalVariables|GetPostAdjustmentCapsuleHeight)))))))

(fn GetCapsuleOverlapCheckResult
  (params (CapsulePos :type Vector) (PreUnscaledHalfHeight :type Float%20%28double-precision%29) (HalfHeightAdjusted :type Float%20%28double-precision%29))
  ;[1 1 1] Checks if the player would be still enroached if we'd adjust their position
  (bind _actors (Default|GetActorsOfClasses (Variables|Default|GetCharacterCoreComponent) (Variables|Configuration|GetClassExceptionListForOverlap)))
  (bind _output_get (LocalVariables|SetIgnoredActors _actors))
  (Utilities|Array|AppendArray _output_get (Actor|GetAllChildActors (Components|GetOwner) true))
  (bind _returnvalue (Collision|CapsuleOverlapActors CapsulePos (Class|CapsuleComponent|GetUnscaledCapsuleRadius (Variables|/Game/Motion/Blueprints/Character/BP_CharacterCoreComponent.BP_CharacterCoreComponent_C|GetCapsule (Variables|Default|GetCharacterCoreComponent))) (- PreUnscaledHalfHeight (- -0.0001 HalfHeightAdjusted)) (Variables|ComponentData|GetOverlapActorTypes) 0 (LocalVariables|GetIgnoredActors)))
  (return _returnvalue))

(fn SetCrouch
  (params (bWantsToCrouch :type Boolean))
  ;[1 1 1] Updates crouch states. Used by input events.
  (Variables|States|SetbWantsToCrouch bWantsToCrouch)
  (Variables|States|SetbIsInCrouch true))