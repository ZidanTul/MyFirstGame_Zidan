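; Walking component for a modular character that sets base walk speed and drives a looping camera shake curve through the curve manager.
; Velocity start and stop events unpause and pause the shake and toggle walking state.
; While walking, Tick advances an acceleration curve to ramp speed from zero, with optional swapping to a post-landing curve until it peaks.
; The walking camera-offset logic is present but disconnected.
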(event Custom|Event%20On%20Velocity%20Begin
  ;[0.03922 0.1529 0.251] Event Graph
  (EventHandler|HandleonVelocityBegin))

(event Custom|Event%20On%20Player%20Landed
  ;[0.03922 0.1529 0.251] Event Graph
  (EventHandler|HandleonPlayerLanded))

(event Custom|Event%20On%20Velocity%20Stop
  ;[0.03922 0.1529 0.251] Event Graph
  (EventHandler|HandleonVelocityStop))

(event EventBeginPlay
  ;[0.03922 0.1529 0.251] Event Graph
  (|CallParentFunction)
  (EventHandler|HandleonEventBeginPlay (delegate Custom|Event%20On%20Velocity%20Begin) (delegate Custom|Event%20On%20Velocity%20Stop) (delegate Custom|Event%20On%20Player%20Landed)))

(event EventTick
  (params (DeltaSeconds :type Float%20%28single-precision%29))
  ;[0.03922 0.1529 0.251] Event Graph
  (EventHandler|HandleonEventTick DeltaSeconds))

(event EventOnCurveMaximum
  (params (CurveData :type F%20Struct%20Motion%20Curve%20Structure))
  (EventHandler|HandleonCurveMaximum))

(fn UpdateDeltaSeconds
  (params (DeltaTime :type Float%20%28double-precision%29))
  ;[1 1 1] Updates progress on walk shake camera curve.
  (if (Utilities|IsAccelerationorLandedandShouldAccelerateEnabled)
    (bind _updateddeltaseconds (CallFunction|UpdateSecondswithCurve (Variables|ComponentData|GetActiveAccelerationCurve) (Variables|ComponentData|GetActiveWalkAccelerationSeconds) (Variables|Constants|GetDeltaTickRate) DeltaTime false))
    (Variables|ComponentData|SetActiveWalkAccelerationSeconds _updateddeltaseconds)))

(fn PrintDebugInformation
  ;[1 1 1] Prints useful information on the screen. Helpful for debugging.
  (if (Variables|Configuration|GetbShowDebugInformation)
    (bind _velocity (Default|GetSquaredPlayerVelocity (Variables|/Game/Motion/Blueprints/Character/BP_CharacterCoreComponent.BP_CharacterCoreComponent_C|GetCharacter (Variables|Default|GetCharacterCoreComponent))))
    (Development|PrintString (Utilities|String|Append "Current Walkspeed (Component): " (Utilities|String|ToString(Float) (Variables|Configuration|GetBaseMaxWalkSpeed)) " 
Current Walkspeed (Character): " (Utilities|String|ToString(Float) _velocity) " 
Is Walking: " (Utilities|String|ToString(Boolean) (Variables|States|GetbIsWalking)) " 
Active Delta Seconds: " (Utilities|String|ToString(Float) (Variables|ComponentData|GetActiveDeltaSeconds)) " 
Current Target Rotation: " (Utilities|String|ToString(Rotator) (Variables|ComponentData|GetCurrentTargetRotation)) " 
Real Camera Rotation: " (Utilities|String|ToString(Rotator) (Variables|/Script/Engine.SceneComponent|GetRelativeRotation (Variables|/Game/Motion/Blueprints/Character/BP_CharacterCoreComponent.BP_CharacterCoreComponent_C|GetCamera (Variables|Default|GetCharacterCoreComponent)))) " 
Walk Acceleration Seconds: " (Utilities|String|ToString(Float) (Variables|ComponentData|GetActiveWalkAccelerationSeconds))) true false "(R=0.000000,G=1.000000,B=0.328099,A=1.000000)" 0.001)))

(fn HandleonEventBeginPlay
  (params (EventOnVelocityBeginDelegate :type Delegate%20%28by%20ref%29) (EventOnVelocityStopDelegate :type Delegate%20%28by%20ref%29) (EventOnPlayerLandedDelegate :type Delegate%20%28by%20ref%29))
  ;[1 1 1] Called when "Event Begin Play" gets called. Sets up events and saves component references.
  (Utilities|FlowControl|Sequence
    (:then_0
      ;;[1 1 1] Find and save Core Component in Owner
      (Utilities|FlowControl|Sequence
        (:then_0
          (bind _actorcomponent (Default|GetComponent (Variables|Default|GetCharacterCoreComponent) "/Game/Motion/Blueprints/Components/BP_CrouchingComponent.BP_CrouchingComponent_C" self))
          (bind _asbp_crouching_component (Utilities|Casting|CastToBP_CrouchingComponent _actorcomponent))
          (Variables|Default|SetCrouchComponent _asbp_crouching_component))
        (:then_1
          (bind _actorcomponent_2 (Default|GetComponent (Variables|Default|GetCharacterCoreComponent) "/Game/Motion/Blueprints/Components/BP_SprintingComponent.BP_SprintingComponent_C" self))
          (bind _asbp_sprinting_component (Utilities|Casting|CastToBP_SprintingComponent _actorcomponent_2))
          (Variables|Default|SetSprintingComponent _asbp_sprinting_component))
        (:then_2
          (bind _actorcomponent_3 (Default|GetComponent (Variables|Default|GetCharacterCoreComponent) "/Game/Motion/Blueprints/Components/BP_JumpingComponent.BP_JumpingComponent_C" self))
          (bind _asbp_jumping_component (Utilities|Casting|CastToBP_JumpingComponent _actorcomponent_3))
          (Variables|Default|SetJumpingComponent _asbp_jumping_component))))
    (:then_1
      ;;[1 1 1] Bind Events
      (EventDispatchers|BindEventtoOnVelocityBegin (Variables|/Game/Motion/Blueprints/Character/BP_CharacterCoreComponent.BP_CharacterCoreComponent_C|GetCharacter (Variables|Default|GetCharacterCoreComponent)) EventOnVelocityBeginDelegate)
      (EventDispatchers|BindEventtoOnVelocityStop (Variables|/Game/Motion/Blueprints/Character/BP_CharacterCoreComponent.BP_CharacterCoreComponent_C|GetCharacter (Variables|Default|GetCharacterCoreComponent)) EventOnVelocityStopDelegate)
      (EventDispatchers|BindEventtoOnPlayerLanded (Variables|/Game/Motion/Blueprints/Character/BP_CharacterCoreComponent.BP_CharacterCoreComponent_C|GetCharacter (Variables|Default|GetCharacterCoreComponent)) EventOnPlayerLandedDelegate))
    (:then_2
      ;;[1 1 1] Add Base Walk Speed to Core Component & create curve
      (Default|AddWalkSpeed (Variables|Default|GetCharacterCoreComponent) self (Variables|Configuration|GetBaseMaxWalkSpeed) false)
      (if (Variables|Configuration|GetbIsEnabled)
        (Default|AddCurve (Variables|Default|GetCharacterCurveManager) (Utilities|Struct|MakeFStructMotionCurve (Utilities|Struct|MakeFStructMotionCurveIdentifier self (Variables|Configuration|GetWalkShakeCurve) (Variables|Constants|GetCurveType)) (Utilities|Struct|MakeFStructMotionCurveConfiguration true false false (Variables|Constants|GetDeltaTickRate)) false true))))))

(fn HandleonEventTick
  (params (DeltaTime :type Float%20%28double-precision%29))
  ;[1 1 1] Core logic handling. See detailed comments.
  (if (Variables|Configuration|GetbIsEnabled) ; Only update if component is enabled, otherwise just update Debug text
    (if (Variables|States|GetbIsWalking) ; Also, only update when we are only walking to avoid unneccessary computations
      (Utilities|FlowControl|Sequence
        (:then_0
          (Manipulators|UpdateDeltaSeconds DeltaTime) ; Updates all timers we use for calculations.\nWe use a custom tick rate as Delta Seconds from Event Tick is not a consistent value
        )
        (:then_1
          (Manipulators|LerpTorwardsWalkingSpeed) ; Applies the current walking speed, relative to curve progression.
        )
        (:then_2
          (Debug|PrintDebugInformation :!label _label)))
      (else
        (Utilities|FlowControl|Sequence
          (:then_0
            (Manipulators|ResetWalkAccelerationSeconds DeltaTime))
          (:then_1
            (goto _label)))))
    (else
      (goto _label))))

(fn HandleonVelocityBegin
  ;[1 1 1] Called when player starts moving.
  (Variables|States|SetbIsWalking true)
  (Default|UnpauseCurve (Variables|Default|GetCharacterCurveManager) (Utilities|Struct|MakeFStructMotionCurveIdentifier self (Variables|Configuration|GetWalkShakeCurve) (Variables|Constants|GetCurveType)) false))

(fn HandleonVelocityStop
  ;[1 1 1] Called when player stops moving.
  (Variables|States|SetbIsWalking false)
  (Default|PauseCurve (Variables|Default|GetCharacterCurveManager) (Utilities|Struct|MakeFStructMotionCurveIdentifier self (Variables|Configuration|GetWalkShakeCurve) (Variables|Constants|GetCurveType)) false))

(fn LerpTorwardsWalkingSpeed
  ;[1 1 1] Applies the current walking speed, relative to curve progression.
  (if (Utilities|IsAccelerationorLandedandShouldAccelerateEnabled)
    (Default|AddWalkSpeed (Variables|Default|GetCharacterCoreComponent) self (Math|Float|Lerp 0.0 (Variables|Configuration|GetBaseMaxWalkSpeed) (.x (Math|Curves|GetVectorValue (Variables|ComponentData|GetActiveAccelerationCurve) (Variables|ComponentData|GetActiveWalkAccelerationSeconds)))) false)
    (Manipulators|UpdateTargetCameraLocation false)))

(fn ResetWalkAccelerationSeconds
  (params (DeltaTime :type Float%20%28double-precision%29))
  ;[1 1 1] Resets walk acceleration, e.g. after stopping to walk
  (if (Utilities|IsAccelerationorLandedandShouldAccelerateEnabled)
    (Variables|ComponentData|SetActiveWalkAccelerationSeconds 0.0)))

(fn HandleonPlayerLanded
  ;[1 1 1] Called when the player lands.
  (if (Variables|Configuration|GetbUseLandingAcceleration)
    (Variables|ComponentData|SetActiveAccelerationCurve (Variables|Configuration|GetPostLandingAccelerationCurve))
    (Variables|States|SetbHasLandedWithOverride true)))

(fn HandleonCurveMaximum
  ;[1 1 1] Called when the component's active curve reaches its peak.
  (if (Math|Boolean|ANDBoolean (Variables|Configuration|GetbUseLandingAcceleration) (Variables|States|GetbHasLandedWithOverride) (Variables|Configuration|GetbUseWalkAcceleration))
    (Variables|ComponentData|SetActiveAccelerationCurve (Variables|Configuration|GetWalkAccelerationCurve))
    (Variables|States|SetbHasLandedWithOverride false)
    (bind _time (CallFunction|GetCurveTime (Variables|Configuration|GetWalkAccelerationCurve) "NewEnumerator1"))
    (Variables|ComponentData|SetActiveWalkAccelerationSeconds _time)))

(fn UpdateTargetCameraLocation
  (params (Reverse :type Boolean)))