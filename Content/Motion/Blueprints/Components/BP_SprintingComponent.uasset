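; Character sprinting component that adds a walk speed boost and looping camera shake while sprint is active, with hold or toggle input.
; It binds the character's key and velocity-stop events, finds sibling components through the Character Core component, and submits speed and camera offsets to it.
; Each tick, curves drive acceleration and shake, while velocity-to-forward dot products classify direction to block sprinting or apply a recovering speed penalty.
; Crouching also cancels sprint.
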(event Custom|Event%20On%20Sprint%20Released
  ;[0.03922 0.1529 0.251] Event Graph
  (EventHandler|HandleonSprintReleased))

(event Custom|Event%20On%20Sprint%20Pressed
  ;[0.03922 0.1529 0.251] Event Graph
  (EventHandler|HandleonSprintPressed))

(event Custom|Event%20On%20Velocity%20Stop
  ;[0.03922 0.1529 0.251] Event Graph
  (EventHandler|HandleonVelocityStop))

(event EventBeginPlay
  ;[0.03922 0.1529 0.251] Event Graph
  (|CallParentFunction)
  (EventHandler|HandleonEventBeginPlay (delegate Custom|Event%20On%20Sprint%20Pressed) (delegate Custom|Event%20On%20Sprint%20Released) (delegate Custom|Event%20On%20Velocity%20Stop)))

(event EventTick
  (params (DeltaSeconds :type Float%20%28single-precision%29))
  ;[0.03922 0.1529 0.251] Event Graph
  (EventHandler|HandleonEventTick DeltaSeconds))

(fn HandleonEventBeginPlay
  (params (EventOnSprintKeyPressedDelegate :type Delegate%20%28by%20ref%29) (EventOnSprintKeyReleasedDelegate :type Delegate%20%28by%20ref%29) (EventOnVelocityStopDelegate :type Delegate%20%28by%20ref%29))
  ;[1 1 1] Called when "Event Begin Play" gets called. Sets up events and gets component references.
  (Utilities|FlowControl|Sequence
    (:then_0
      ;;[1 1 1] Find and save Core Component in Owner
      (Utilities|FlowControl|Sequence
        (:then_0
          (bind _actorcomponent (Default|GetComponent (Variables|Default|GetCharacterCoreComponent) "/Game/Motion/Blueprints/Components/BP_CrouchingComponent.BP_CrouchingComponent_C" self))
          (bind _asbp_crouching_component (Utilities|Casting|CastToBP_CrouchingComponent _actorcomponent))
          (Variables|Default|SetCrouchComponent _asbp_crouching_component))
        (:then_1
          (bind _actorcomponent_2 (Default|GetComponent (Variables|Default|GetCharacterCoreComponent) "/Game/Motion/Blueprints/Components/BP_WalkingComponent.BP_WalkingComponent_C" self))
          (bind _asbp_walking_component (Utilities|Casting|CastToBP_WalkingComponent _actorcomponent_2))
          (Variables|Default|SetWalkingComponent _asbp_walking_component))))
    (:then_1
      ;;[1 1 1] Bind Sprint Events
      (EventDispatchers|BindEventtoOnSprintKeyPressed (Variables|/Game/Motion/Blueprints/Character/BP_CharacterCoreComponent.BP_CharacterCoreComponent_C|GetCharacter (Variables|Default|GetCharacterCoreComponent)) EventOnSprintKeyPressedDelegate)
      (EventDispatchers|BindEventtoOnSprintKeyReleased (Variables|/Game/Motion/Blueprints/Character/BP_CharacterCoreComponent.BP_CharacterCoreComponent_C|GetCharacter (Variables|Default|GetCharacterCoreComponent)) EventOnSprintKeyReleasedDelegate)
      (EventDispatchers|BindEventtoOnVelocityStop (Variables|/Game/Motion/Blueprints/Character/BP_CharacterCoreComponent.BP_CharacterCoreComponent_C|GetCharacter (Variables|Default|GetCharacterCoreComponent)) EventOnVelocityStopDelegate))))

(fn HandleonEventTick
  (params (DeltaTime :type Float%20%28double-precision%29))
  ;[1 1 1] Core logic handling. See detailed comments.
  (if (Variables|Configuration|GetbIsEnabled) ; Only update if component is enabled, otherwise just update Debug text
    (if (|IsNotFallingButSprintingAndMoving) ; Also, only update when we are jumping to avoid unneccessary computations
      (if (|IsNotCrouching)
        (Utilities|FlowControl|Sequence
          (:then_0
            (Manipulators|UpdateDeltaSeconds DeltaTime) ; Updates all timers we use for calculations.\nWe use a custom tick rate as Delta Seconds from Event Tick is not a consistent value
          )
          (:then_1
            (Manipulators|ValidateActiveDeltaSeconds) ; Checks if we are at the maximum / end of the sprint curve and resets the timer used for sprint shake & acceleration to ensure it loops
          )
          (:then_2
            (Manipulators|UpdateMovementDirection) ; Checks in which direction the player is moving
          )
          (:then_3
            (Manipulators|ValidateMovement) ; Checks if we are running backwards to disable sprinting and penalizes the player for side-sprinting.\nAlso checks if we are crouched.
          )
          (:then_4
            (Manipulators|CalculateCurrentPenalty) ; If penalized, calculates the current speed penalty that will be applied
          )
          (:then_5
            (if (Variables|States|GetbCanSprint) ; Checks if sprinting got disabled due to disallowed movement changes
              (Utilities|FlowControl|Sequence
                (:then_0
                  (Manipulators|LerpTowardsSprintingSpeed) ; Calculates the speed for the current tick that should be set as maximum speed for the player
                )
                (:then_1
                  (Manipulators|UpdateTargetCameraRotation) ; Gets the camera vector at the current time on the curve
                )
                (:then_2
                  ;;[1 0 0] Manually calling "Add Camera Offset" is deprecated and will soon be removed.
                  (Default|AddCameraOffset (Variables|Default|GetCharacterCoreComponent) (Utilities|Struct|MakeFStructCameraCurve (Utilities|Struct|MakeFStructMotionCurve (Utilities|Struct|MakeFStructMotionCurveIdentifier self (Variables|Configuration|GetSprintShakeCurve) (Variables|Constants|GetCurveType)) "(bShouldLoop_9_666576974F883E228DB125BEAF8A60D0=False,bShouldReverse_11_5F50FB6143A47A5D2F479EBAAD96DD32=False,bHasPriority_14_E460BB484F65E64110A48FB2A6E597CB=False,Tickrate_16_7FAB02194AA4ADC275096CBD3E8829FC=0.000000)" false true) (Variables|ComponentData|GetCurrentTargetRotation)))))
              (else
                (Manipulators|ResetSprint :!label _label) ; Resets the sprint to the default Max Walk Speed
              )))
          (:then_6
            (Debug|PrintDebugInformation :!label _label_2)))
        (else
          (Utilities|FlowControl|Sequence
            (:then_0
              (goto _label))
            (:then_1
              (goto _label_2)))))
      (else
        (Utilities|FlowControl|Sequence
          (:then_0
            (if (and (Variables|States|GetbIsSprinting) (not (Variables|States|GetbIsHoldingSprintKey)))
              (goto _label)))
          (:then_1
            (goto _label_2)))))
    (else
      (goto _label_2))))

(fn HandleonSprintPressed
  ;[1 1 1] When pressing the sprint key, reset timers & toggle sprint key state
  (if (Variables|Configuration|GetbIsEnabled)
    (if (Variables|Configuration|GetbIsInputToggle)
      (if (Variables|States|GetbIsSprinting)
        (Manipulators|ResetSprint)
        (else
          (Variables|States|SetbIsHoldingSprintKey true :!label _label)
          (Variables|ComponentData|SetActiveDeltaSeconds 0.0)
          (Variables|ComponentData|SetActiveSprintKeyDownSeconds 0.0)))
      (else
        (goto _label)))))

(fn HandleonSprintReleased
  ;[1 1 1] When releasing the sprint key, reset sprint timers, state & values
  (if (Variables|Configuration|GetbIsEnabled)
    (Variables|States|SetbIsHoldingSprintKey false)
    (Variables|ComponentData|SetActiveSprintKeyDownSeconds 0.0)
    (if (not (Variables|Configuration|GetbIsInputToggle))
      (Manipulators|ResetSprint))))

(fn CalculateCurrentPenalty
  ;[1 1 1] Gets the current penalty and applies it, unless the newly calculated penalty is near to zero
  (if (Variables|States|GetbIsPenalized)
    (bind _output_get (Variables|ComponentData|SetCurrentAppliedPenalty (|GetCurrentPenalty)))
    (if (Math|Float|NearlyEqual(Float) _output_get 0.0 1e-06)
      (Manipulators|ResetPenalty))))

(fn LerpTowardsSprintingSpeed
  ;[1 1 1] Applies the current speed bonus
  (bind _output_get (Variables|ComponentData|SetCurrentWalkSpeed (|GetSpeedValueFromCurve)))
  (Variables|States|SetbIsSprinting true)
  (Default|AddWalkSpeed (Variables|Default|GetCharacterCoreComponent) self _output_get false))

(fn UpdateTargetCameraRotation
  (bind _sprintshakecurve (Variables|Configuration|GetSprintShakeCurve))
  (bind _activedeltaseconds (Variables|ComponentData|GetActiveDeltaSeconds))
  (bind _returnvalue (Math|Curves|GetVectorValue _sprintshakecurve _activedeltaseconds))
  ;[1 1 1] Gets the current position of the camera shake curve and updates the target rotation
  (Variables|ComponentData|SetCurrentTargetRotation (Math|Rotator|MakeRotator (.z _returnvalue) (.y _returnvalue) (.x _returnvalue)))
  (return))

(fn UpdateTargetCameraLocation
  (Default|AddCameraLocationOffset (Variables|Default|GetCharacterCoreComponent) self (Math|Vector|Lerp(Vector) "0, 0, 0" (Variables|Configuration|GetSprintCameraLocationOffset) (Math|Float|Clamp(Float) (Math|Float|NormalizetoRange (Variables|ComponentData|GetActiveSprintKeyDownSeconds) 0.0 (Variables|Configuration|GetSprintCameraLocationOffsetAnimationTime)))) false))

(fn UpdateMovementDirection
  ;[1 1 1] Determines which direction the player is moving towards to by parsing their normalized direction
  (LocalVariables|SetPreviousMovementDirection (Variables|ComponentData|GetCurrentMovementDirection))
  (Variables|ComponentData|SetNormalizedDirection (|GetNormalizedDirection))
  (if (Math|Float|NearlyEqual(Float) (Variables|ComponentData|GetNormalizedDirection) 1.0 0.05)
    (Variables|ComponentData|SetCurrentMovementDirection "NewEnumerator1")
    (if (Utilities|Enum|NotEqual(Enum) (LocalVariables|GetPreviousMovementDirection) (Variables|ComponentData|GetCurrentMovementDirection)) :!label _label
      (Variables|States|SetbHasBeenPenalized false))
    (elif (Math|Float|NearlyEqual(Float) (Variables|ComponentData|GetNormalizedDirection) -1.0 0.05)
      (Variables|ComponentData|SetCurrentMovementDirection "NewEnumerator4")
      (goto _label)
      (elif (and (not (Math|Float|NearlyEqual(Float) (Variables|ComponentData|GetNormalizedDirection) 1.0 0.05)) (> (Variables|ComponentData|GetNormalizedDirection) 0.1))
        (Variables|ComponentData|SetCurrentMovementDirection "NewEnumerator2")
        (goto _label)
        (elif (and (not (Math|Float|NearlyEqual(Float) (Variables|ComponentData|GetNormalizedDirection) -1.0 0.05)) (> (Variables|ComponentData|GetNormalizedDirection) -1.0))
          (Variables|ComponentData|SetCurrentMovementDirection "NewEnumerator6")
          (goto _label)
          (else
            (Variables|ComponentData|SetCurrentMovementDirection "NewEnumerator0")))))))

(fn UpdateDeltaSeconds
  (params (DeltaTime :type Float%20%28double-precision%29))
  ;[1 1 1] Updates progress on sprint shake camera curve, timer for holding the key down & penalty timer if penalized
  (Utilities|FlowControl|Sequence
    (:then_0
      (bind _updateddeltaseconds (CallFunction|UpdateSecondswithCurve (Variables|Configuration|GetSprintShakeCurve) (Variables|ComponentData|GetActiveDeltaSeconds) (Variables|Constants|GetDeltaTickRate) DeltaTime false))
      (Variables|ComponentData|SetActiveDeltaSeconds _updateddeltaseconds))
    (:then_1
      (bind _updatedactivedeltaseconds (CallFunction|UpdateSeconds (Variables|ComponentData|GetActiveSprintKeyDownSeconds) (Variables|Constants|GetDeltaTickRate) DeltaTime false))
      (Variables|ComponentData|SetActiveSprintKeyDownSeconds _updatedactivedeltaseconds))
    (:then_2
      (if (Variables|States|GetbIsPenalized)
        (bind _updatedactivedeltaseconds_2 (CallFunction|UpdateSeconds (Variables|ComponentData|GetActivePenaltySeconds) (Variables|Constants|GetMovementDirectionChangeSpeedPenaltyRecoveryDeltaTickRate) DeltaTime false))
        (Variables|ComponentData|SetActivePenaltySeconds _updatedactivedeltaseconds_2)))))

(fn ValidateActiveDeltaSeconds
  ;[1 1 1] Checks if the sprint shake curve progress is at its peak and resets it then to ensure looped camera movement
  (bind _state (CallFunction|IsCurveatCurveTime (Variables|Configuration|GetSprintShakeCurve) "NewEnumerator1" (Variables|ComponentData|GetActiveDeltaSeconds)))
  (if _state
    (Variables|ComponentData|SetActiveDeltaSeconds 0.0)))

(fn ValidateMovement
  ;[1 1 1] Updates status of player being able to sprint and applies / resets penalty according to movement changes
  (Variables|States|SetbCanSprint (|CheckIfPlayerCanSprint))
  (if (Utilities|Enum|Equal(Enum) (Variables|ComponentData|GetCurrentMovementDirection) "NewEnumerator2")
    (if (not (and (Variables|States|GetbIsPenalized) (not (Variables|States|GetbHasBeenPenalized))))
      (Variables|ComponentData|SetCurrentAppliedPenalty (Variables|Configuration|GetMovementDirectionChangeSpeedPenalty))
      (Variables|States|SetbIsPenalized true)
      (Variables|ComponentData|SetActivePenaltySeconds 0.0))
    (elif (Variables|States|GetbIsPenalized)
      (Manipulators|ResetPenalty))))

(fn ResetPenalty
  ;[1 1 1] Resets penalty related variables
  (Variables|States|SetbIsPenalized false)
  (Variables|ComponentData|SetCurrentAppliedPenalty 0.0)
  (Variables|ComponentData|SetActivePenaltySeconds 0.0)
  (Variables|States|SetbHasBeenPenalized true))

(fn ResetSprint
  ;[1 1 1] Resets sprint state and speed
  (Variables|States|SetbIsSprinting false)
  (Variables|ComponentData|SetCurrentWalkSpeed 0.0)
  (Default|RemoveWalkSpeed (Variables|Default|GetCharacterCoreComponent) self)
  (Default|RemoveCameraLocationOffset (Variables|Default|GetCharacterCoreComponent) self))

(fn PrintDebugInformation
  ;[1 1 1] Prints useful information on the screen. Helpful for debugging.
  (if (Variables|Configuration|GetbShowDebugInformation)
    (bind _velocity (Default|GetSquaredPlayerVelocity (Variables|/Game/Motion/Blueprints/Character/BP_CharacterCoreComponent.BP_CharacterCoreComponent_C|GetCharacter (Variables|Default|GetCharacterCoreComponent))))
    (Development|PrintString (Utilities|String|Append "Current Walkspeed (Component): " (Utilities|String|ToString(Float) (Variables|ComponentData|GetCurrentWalkSpeed)) " 
Current Walkspeed (Character): " (Utilities|String|ToString(Float) _velocity) " 
Is Sprinting: " (Utilities|String|ToString(Boolean) (Variables|States|GetbIsSprinting)) " 
Active Delta Seconds: " (Utilities|String|ToString(Float) (Variables|ComponentData|GetActiveDeltaSeconds)) " 
Current Target Rotation: " (Utilities|String|ToString(Rotator) (Variables|ComponentData|GetCurrentTargetRotation)) " 
Real Camera Rotation: " (Utilities|String|ToString(Rotator) (Variables|/Script/Engine.SceneComponent|GetRelativeRotation (Variables|/Game/Motion/Blueprints/Character/BP_CharacterCoreComponent.BP_CharacterCoreComponent_C|GetCamera (Variables|Default|GetCharacterCoreComponent)))) " 
Normalized Direction: " (Utilities|String|ToString(Float) (Variables|ComponentData|GetNormalizedDirection)) " 
Can Sprint: " (Utilities|String|ToString(Boolean) (Variables|States|GetbCanSprint)) " 
Active Penalty Seconds: " (Utilities|String|ToString(Float) (Variables|ComponentData|GetActivePenaltySeconds)) " 
Is Penalized: " (Utilities|String|ToString(Boolean) (Variables|States|GetbIsPenalized)) " 
Is holding Sprint Key: " (Utilities|String|ToString(Boolean) (Variables|States|GetbIsHoldingSprintKey)) " 
Current Movement Direction: " (Utilities|String|EnumtoString (Variables|ComponentData|GetCurrentMovementDirection))) true false "(R=0.725896,G=0.000000,B=1.000000,A=1.000000)" 1.0 "MotionCrouchingDebug")))

(fn HandleonVelocityStop
  ;[1 1 1] Called when player stops moving. Resets sprinting.
  (Manipulators|ResetSprint))