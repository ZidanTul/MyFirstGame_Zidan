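; Base manager that drives time-based vector Motion Curves and timed transitions between them on behalf of curved components.
; While enabled, each tick advances unpaused curves, handling looping and reversing, then advances unpaused transitions.
; Each entry's position triggers minimum, update or maximum events on its component, which receives the updated struct.
; Helper functions add, find, pause and delete array entries, with optional on-screen debug output.
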(event EventBeginPlay
  ;[0 0.1429 1] Event Graph
  (Core|HandleEventBeginPlay))

(event EventTick
  (params (DeltaSeconds :type Float%20%28single-precision%29))
  ;[0 0.1429 1] Event Graph
  (Core|HandleEventTick DeltaSeconds))

(fn HandleEventBeginPlay
  ;[1 1 1] Called when "Event Begin Play" gets called. Sets up core references.
)

(fn HandleEventTick
  (params (DeltaTime :type Float%20%28double-precision%29))
  ;[1 1 1] Called every tick. Handles core logic.
  (if (Variables|Configuration|GetbIsEnabled)
    (Utilities|FlowControl|Sequence
      (:then_0
        (Curves|UpdateCurveArray DeltaTime)
        (CallFunction|OnCurveArrayUpdated))
      (:then_1
        (Transitions|UpdateTransitionArray DeltaTime)
        (CallFunction|OnTransitionArrayUpdated))
      (:then_2
        (Debug|PrintDebugInformation :!label _label)))
    (else
      (goto _label))))

(fn UpdateCurveArray
  (params (DeltaTime :type Float%20%28double-precision%29))
  ;[1 1 1] Loops through all registered Motion Curves, updates them & triggers update events.
  (LocalVariables|SetLocalDeltaTime DeltaTime)
  (for (_array_element _array_index) (Variables|ManagerData|GetActiveMotionCurves)
    (if (not (.bIsPaused (Utilities|Struct|BreakFStructMotionCurve _array_element)))
      (bind (_updatedcurve _curveposition) (Curves|UpdateCurve _array_element (LocalVariables|GetLocalDeltaTime)))
      (if (Utilities|IsValid (.curvedcomponent (.Identifier (Utilities|Struct|BreakFStructMotionCurve _updatedcurve))))
        (Utilities|SetMotionCurve _updatedcurve _array_index
          (:_
            (LocalVariables|SetCurrentCurve _updatedcurve)
            (|HandleCurveEvents _curveposition)))))))

(fn UpdateCurve
  (params (Curve :type F%20Struct%20Motion%20Curve%20Structure) (DeltaTime :type Float%20%28double-precision%29))
  ;[1 1 1] Validates a curve and updates it's progression.
  (LocalVariables|SetCurrentCurve Curve)
  (LocalVariables|SetLocalDeltaTime DeltaTime)
  (bind _bisvalid (Curves|ValidateCurve (.Identifier (Utilities|Struct|BreakFStructMotionCurve (LocalVariables|GetCurrentCurve))) true))
  (if _bisvalid
    (LocalVariables|SetbIsCurrentAtMin (== (.ActiveSeconds (Utilities|Struct|BreakFStructMotionCurve (LocalVariables|GetCurrentCurve))) 0.0))
    (bind _state (CallFunction|IsCurveatCurveTime (.curvevector (.Identifier (Utilities|Struct|BreakFStructMotionCurve (LocalVariables|GetCurrentCurve)))) "NewEnumerator1" (.ActiveSeconds (Utilities|Struct|BreakFStructMotionCurve (LocalVariables|GetCurrentCurve)))))
    (LocalVariables|SetbIsCurrentAtMax _state)
    (if (LocalVariables|GetbIsCurrentAtMax)
      (if (or (and (.bshouldloop (.Configuration (Utilities|Struct|BreakFStructMotionCurve (LocalVariables|GetCurrentCurve)))) (.bshouldreverse (.Configuration (Utilities|Struct|BreakFStructMotionCurve (LocalVariables|GetCurrentCurve))))) (and (not (.bshouldloop (.Configuration (Utilities|Struct|BreakFStructMotionCurve (LocalVariables|GetCurrentCurve))))) (.bshouldreverse (.Configuration (Utilities|Struct|BreakFStructMotionCurve (LocalVariables|GetCurrentCurve))))))
        (bind _updateddeltaseconds (CallFunction|UpdateSecondswithCurve (.curvevector (.Identifier (Utilities|Struct|BreakFStructMotionCurve (LocalVariables|GetCurrentCurve)))) (.ActiveSeconds (Utilities|Struct|BreakFStructMotionCurve (LocalVariables|GetCurrentCurve))) (.tickrate (.Configuration (Utilities|Struct|BreakFStructMotionCurve (LocalVariables|GetCurrentCurve)))) (LocalVariables|GetLocalDeltaTime) true))
        (bind _structout (Utilities|Struct|SetmembersinFStructMotionCurve (LocalVariables|GetCurrentCurve) true _updateddeltaseconds))
        (return _structout "NewEnumerator1")
        (elif (and (.bshouldloop (.Configuration (Utilities|Struct|BreakFStructMotionCurve (LocalVariables|GetCurrentCurve)))) (not (.bshouldreverse (.Configuration (Utilities|Struct|BreakFStructMotionCurve (LocalVariables|GetCurrentCurve))))))
          (bind _structout_2 (Utilities|Struct|SetmembersinFStructMotionCurve (LocalVariables|GetCurrentCurve) 0.0))
          (return _structout_2 "NewEnumerator1")
          (else
            (return (LocalVariables|GetCurrentCurve) "NewEnumerator1"))))
      (else
        (if (LocalVariables|GetbIsCurrentAtMin)
          (if (or (.bshouldloop (Utilities|Struct|BreakFStructMotionCurve (LocalVariables|GetCurrentCurve))) (and (.bshouldloop (Utilities|Struct|BreakFStructMotionCurve (LocalVariables|GetCurrentCurve))) (.bshouldreverse (Utilities|Struct|BreakFStructMotionCurve (LocalVariables|GetCurrentCurve)))))
            (bind _updateddeltaseconds_2 (CallFunction|UpdateSecondswithCurve (.curvevector (.Identifier (Utilities|Struct|BreakFStructMotionCurve (LocalVariables|GetCurrentCurve)))) (.ActiveSeconds (Utilities|Struct|BreakFStructMotionCurve (LocalVariables|GetCurrentCurve))) (.tickrate (.Configuration (Utilities|Struct|BreakFStructMotionCurve (LocalVariables|GetCurrentCurve)))) (LocalVariables|GetLocalDeltaTime) false))
            (bind _structout_3 (Utilities|Struct|SetmembersinFStructMotionCurve (LocalVariables|GetCurrentCurve) false _updateddeltaseconds_2))
            (return _structout_3 "NewEnumerator0")
            (else
              _))
          (elif (.bIsReversing (Utilities|Struct|BreakFStructMotionCurve (LocalVariables|GetCurrentCurve)))
            (bind _updateddeltaseconds_3 (CallFunction|UpdateSecondswithCurve (.curvevector (.Identifier (Utilities|Struct|BreakFStructMotionCurve (LocalVariables|GetCurrentCurve)))) (.ActiveSeconds (Utilities|Struct|BreakFStructMotionCurve (LocalVariables|GetCurrentCurve))) (.tickrate (.Configuration (Utilities|Struct|BreakFStructMotionCurve (LocalVariables|GetCurrentCurve)))) (LocalVariables|GetLocalDeltaTime) true))
            (bind _structout_4 (Utilities|Struct|SetmembersinFStructMotionCurve (LocalVariables|GetCurrentCurve) true _updateddeltaseconds_3))
            (return _structout_4 "NewEnumerator4")
            (else
              _)))
        (bind _updateddeltaseconds_4 (CallFunction|UpdateSecondswithCurve (.curvevector (.Identifier (Utilities|Struct|BreakFStructMotionCurve (LocalVariables|GetCurrentCurve)))) (.ActiveSeconds (Utilities|Struct|BreakFStructMotionCurve (LocalVariables|GetCurrentCurve))) (.tickrate (.Configuration (Utilities|Struct|BreakFStructMotionCurve (LocalVariables|GetCurrentCurve)))) (LocalVariables|GetLocalDeltaTime) false))
        (bind _structout_5 (Utilities|Struct|SetmembersinFStructMotionCurve (LocalVariables|GetCurrentCurve) false _updateddeltaseconds_4))
        (return _structout_5 "NewEnumerator4")))))

(fn ValidateCurve
  (params (Curve :type F%20Struct%20Motion%20Curve%20Identifier%20Structure) (bThrowException :type Boolean))
  ;[1 1 1] Checks if the provided component and curve vector are valid objects.
  (Utilities|IsValid (.curvedcomponent Curve)
    (:Is%20Valid
      (Utilities|IsValid (.curvevector Curve)
        (:Is%20Valid
          (return true))
        (:Is%20Not%20Valid
          (return false))))
    (:Is%20Not%20Valid
      (return false))))

(fn PrintDebugInformation
  ;[1 1 1] Prints useful information on the screen. Helpful for debugging.
  (if (Variables|Configuration|GetbShowDebugInformation)
    (LocalVariables|SetOutputMessage (Utilities|String|Append "Registered Curves: " (Utilities|String|ToString(Integer) (Utilities|Array|Length (Variables|ManagerData|GetActiveMotionCurves))) " 
"))
    (for _array_element (Variables|ManagerData|GetActiveMotionCurves)
      (LocalVariables|SetOutputMessage (Utilities|String|Append (LocalVariables|GetOutputMessage) " 
#####" (Utilities|GetDisplayName (.curvedcomponent (.Identifier (Utilities|Struct|BreakFStructMotionCurve _array_element)))) " - " (Utilities|GetDisplayName (.curvevector (.Identifier (Utilities|Struct|BreakFStructMotionCurve _array_element)))) " 
Active Seconds: " (Utilities|String|ToString(Float) (.ActiveSeconds (Utilities|Struct|BreakFStructMotionCurve _array_element))) " 
Loops: " (Utilities|String|ToString(Boolean) (.bshouldloop (.Configuration (Utilities|Struct|BreakFStructMotionCurve _array_element)))) " 
Reverses: " (Utilities|String|ToString(Boolean) (.bshouldreverse (.Configuration (Utilities|Struct|BreakFStructMotionCurve _array_element)))) " 
Has Priority: " (Utilities|String|ToString(Boolean) (.bhaspriority (.Configuration (Utilities|Struct|BreakFStructMotionCurve _array_element)))) " 
Is Reversing: " (Utilities|String|ToString(Boolean) (.bIsReversing (Utilities|Struct|BreakFStructMotionCurve _array_element))) " 
Is Paused: " (Utilities|String|ToString(Boolean) (.bIsPaused (Utilities|Struct|BreakFStructMotionCurve _array_element))) " 
Is Transitioning: " (Utilities|String|ToString(Boolean) (.bIsTransitioning (Utilities|Struct|BreakFStructMotionCurve _array_element))) " 
Is Transition Curve: " (Utilities|String|ToString(Boolean) (.bIsTransitionCurve (Utilities|Struct|BreakFStructMotionCurve _array_element))))))
    (Development|PrintString (LocalVariables|GetOutputMessage) true true "(R=0.000000,G=0.300544,B=1.000000,A=1.000000)" 0.001)))

(fn AddCurve
  (params (Curve :type F%20Struct%20Motion%20Curve%20Structure))
  ;[1 1 1] Adds a new curve to the curve array.
  (bind _returnvalue (Utilities|Array|Add (Variables|ManagerData|GetActiveMotionCurves) Curve))
  (return (!= _returnvalue -1) _returnvalue))

(fn GetCurvebyComponent
  (params (Curve :type F%20Struct%20Motion%20Curve%20Identifier%20Structure))
  ;[1 1 1] Tries to find a curve by its component. Returns first curve found, returns -1 if no curve was found.
  (if (not (Utilities|Array|IsEmpty (.curvetype Curve)))
    (bind (_array_element _array_index) (Utilities|Array|ForEachLoopwithBreak (Variables|ManagerData|GetActiveMotionCurves))
      (:LoopBody
        (if (and (== (.curvedcomponent Curve) (.curvedcomponent (Utilities|Struct|BreakFStructMotionCurve _array_element))) (Utilities|Enum|Equal(Enum) (.curvetype Curve) (.curvetype (Utilities|Struct|BreakFStructMotionCurve _array_element))))
          (return true _array_index)))
      (:Completed
        (return false -1)))))

(fn GetCurvebyIdentifier
  (params (Curve :type F%20Struct%20Motion%20Curve%20Identifier%20Structure))
  ;[1 1 1] Tries to find a curve by its identifier. Returns first curve found, returns -1 if no curve was found.
  (bind (_array_element _array_index) (Utilities|Array|ForEachLoopwithBreak (Variables|ManagerData|GetActiveMotionCurves))
    (:LoopBody
      (if (Math|Boolean|ANDBoolean (== (.curvedcomponent Curve) (.curvedcomponent (.Identifier (Utilities|Struct|BreakFStructMotionCurve _array_element)))) (== (.curvevector Curve) (.curvevector (.Identifier (Utilities|Struct|BreakFStructMotionCurve _array_element)))) (Utilities|Enum|Equal(Enum) (.curvetype Curve) (.curvetype (.Identifier (Utilities|Struct|BreakFStructMotionCurve _array_element)))))
        (return true _array_index)))
    (:Completed
      (return false -1))))

(fn PauseCurve
  (params (Curve :type F%20Struct%20Motion%20Curve%20Identifier%20Structure) (bPauseTransition :type Boolean))
  (bind _activemotioncurves (Variables|ManagerData|GetActiveMotionCurves))
  ;[1 1 1] Pauses a specified curve. Returns false if the specified curve could not be found.
  (Utilities|FlowControl|Sequence
    (:then_0
      (bind (_bfound _index) (CurveFunctions|GetCurvebyComponent Curve))
      (if _bfound
        (bind _structout (Utilities|Struct|SetmembersinFStructMotionCurve (Utilities|Array|Get(acopy) _activemotioncurves _index) true))
        (Utilities|Array|SetArrayElem _activemotioncurves _index _structout true)
        (else
          (return false))))
    (:then_1
      (if bPauseTransition
        (bind _bsuccessful (Transitions|PauseTransition Curve true))
        (return _bsuccessful)))))

(fn UnpauseCurve
  (params (Curve :type F%20Struct%20Motion%20Curve%20Identifier%20Structure) (bUnpauseTransition :type Boolean))
  (bind _activemotioncurves (Variables|ManagerData|GetActiveMotionCurves))
  ;[1 1 1] Unpauses a specified curve. Returns false if the specified curve could not be found.
  (Utilities|FlowControl|Sequence
    (:then_0
      (bind (_bfound _index) (CurveFunctions|GetCurvebyComponent Curve))
      (if _bfound
        (bind _structout (Utilities|Struct|SetmembersinFStructMotionCurve (Utilities|Array|Get(acopy) _activemotioncurves _index) false))
        (Utilities|Array|SetArrayElem _activemotioncurves _index _structout true)
        (else
          (return false))))
    (:then_1
      (if bUnpauseTransition
        (bind _bsuccessful (Transitions|PauseTransition Curve false))
        (return _bsuccessful)))))

(fn DeleteCurve
  (params (Curve :type F%20Struct%20Motion%20Curve%20Identifier%20Structure))
  ;[1 1 1] Removes a specified curve. Returns false if the specified curve could not be found.
  (bind (_bfound _index) (CurveFunctions|GetCurvebyIdentifier Curve))
  (if _bfound
    (Utilities|Array|RemoveIndex (Variables|ManagerData|GetActiveMotionCurves) _index)
    (return true _index)
    (else
      (return false 0))))

(fn StartTransition
  (params (TransitionData :type F%20Struct%20Motion%20Curve%20Transition%20Structure))
  ;[1 1 1] Adds a new transition to the array and updates the source curve's transition state.
  (bind _returnvalue (Utilities|Array|Add (Variables|ManagerData|GetActiveMotionCurveTransitions) TransitionData))
  (Transitions|SetinTransitionState true TransitionData)
  (return (!= _returnvalue -1) _returnvalue))

(fn GetTransitionsbyComponent
  (params (CurveIdentifier :type F%20Struct%20Motion%20Curve%20Identifier%20Structure))
  ;[1 1 1] Returns all transitions that are associated with the provided component. Returns an empty array if none are found.
  (for _array_element (Variables|ManagerData|GetActiveMotionCurveTransitions)
    (if (== (.curvedcomponent CurveIdentifier) (.CurvedComponent (Utilities|Struct|BreakFStructMotionCurveIdentifier (.identifier (.TransitionConfiguration (Utilities|Struct|BreakFStructMotionCurveTransition _array_element))))))
      (Utilities|Array|Add (LocalVariables|GetTransitionArray) _array_element)))
  (return (> (Utilities|Array|Length (LocalVariables|GetTransitionArray)) 0) (LocalVariables|GetTransitionArray)))

(fn GetTransitionbyIdentifier
  (params (CurveIdentifier :type F%20Struct%20Motion%20Curve%20Identifier%20Structure) (IdentifierType :type ETransitionCurves%20Enum :default "NewEnumerator0"))
  ;[1 1 1] Tries to find a transition given its configuration. Returns its index if found, returns -1 if not.
  (for (_array_element _array_index) (Variables|ManagerData|GetActiveMotionCurveTransitions)
    (if (Utilities|Enum|Equal(Enum) IdentifierType "NewEnumerator0")
      (if (Math|Boolean|ANDBoolean (== (.curvedcomponent CurveIdentifier) (.CurvedComponent (Utilities|Struct|BreakFStructMotionCurveIdentifier (.targetidentifier (.TransitionConfiguration (Utilities|Struct|BreakFStructMotionCurveTransition _array_element)))))) (== (.curvevector CurveIdentifier) (.CurveVector (Utilities|Struct|BreakFStructMotionCurveIdentifier (.identifier (.TransitionConfiguration (Utilities|Struct|BreakFStructMotionCurveTransition _array_element)))))) (Utilities|Enum|Equal(Enum) (.curvetype CurveIdentifier) (.CurveType (Utilities|Struct|BreakFStructMotionCurveIdentifier (.identifier (.TransitionConfiguration (Utilities|Struct|BreakFStructMotionCurveTransition _array_element)))))))
        (return true _array_index))
      (elif (Math|Boolean|ANDBoolean (== (.curvedcomponent CurveIdentifier) (.CurvedComponent (Utilities|Struct|BreakFStructMotionCurveIdentifier (.identifier (.TransitionConfiguration (Utilities|Struct|BreakFStructMotionCurveTransition _array_element)))))) (== (.curvevector CurveIdentifier) (.CurveVector (Utilities|Struct|BreakFStructMotionCurveIdentifier (.targetidentifier (.TransitionConfiguration (Utilities|Struct|BreakFStructMotionCurveTransition _array_element)))))) (Utilities|Enum|Equal(Enum) (.curvetype CurveIdentifier) (.CurveType (Utilities|Struct|BreakFStructMotionCurveIdentifier (.targetidentifier (.TransitionConfiguration (Utilities|Struct|BreakFStructMotionCurveTransition _array_element)))))))
        (return true _array_index))))
  (return false -1))

(fn PauseTransition
  (params (CurveIdentifier :type F%20Struct%20Motion%20Curve%20Identifier%20Structure) (bIsPaused :type Boolean))
  ;[1 1 1] Sets the pause state for a transition of a given Curved Component.
  (Utilities|FlowControl|Sequence
    (:then_0
      (bind (_bfound _index) (Transitions|GetTransitionbyIdentifier CurveIdentifier "NewEnumerator0"))
      (if _bfound
        (bind _structout (Utilities|Struct|SetmembersinFStructMotionCurveTransition (Utilities|GetMotionTransition _index) bIsPaused))
        (Utilities|SetMotionTransition _structout _index)
        (else
          (return false))))
    (:then_1
      (bind (_bfound_2 _index_2) (CurveFunctions|GetCurvebyIdentifier (.TargetIdentifier (Utilities|Struct|BreakFStructMotionCurveTransitionConfiguration (.TransitionConfiguration (Utilities|Struct|BreakFStructMotionCurveTransition (Utilities|GetMotionTransition _index)))))))
      (if _bfound_2
        (bind _structout_2 (Utilities|Struct|SetmembersinFStructMotionCurve (Utilities|GetMotionCurve _index_2) bIsPaused))
        (Utilities|SetMotionCurve _structout_2 _index_2
          (:_
            (return true)))
        (else
          (return false))))))

(fn UpdateTransitionArray
  (params (DeltaTime :type Float%20%28double-precision%29))
  ;[1 1 1] Loops through all Motion Curve Transitions, updates their progression & triggers transition updates as required.
  (LocalVariables|SetLocalDeltaTime DeltaTime)
  (for (_array_element _array_index) (Variables|ManagerData|GetActiveMotionCurveTransitions)
    (if (not (.bIsPaused (Utilities|Struct|BreakFStructMotionCurveTransition _array_element)))
      (bind (_updatedtransitiondata _transitionposition) (Transitions|UpdateTransition _array_element (LocalVariables|GetLocalDeltaTime)))
      (LocalVariables|SetCurrentTransitionData _updatedtransitiondata)
      (Utilities|Array|SetArrayElem (Variables|ManagerData|GetActiveMotionCurveTransitions) _array_index _updatedtransitiondata true)
      (|HandleTransitionEvents _transitionposition))))

(fn UpdateTransition
  (params (TransitionData :type F%20Struct%20Motion%20Curve%20Transition%20Structure) (DeltaTime :type Float%20%28double-precision%29))
  ;[1 1 1] Updates the active transition seconds of a transition and determines position.
  (LocalVariables|SetLocalTransitionData TransitionData)
  (LocalVariables|SetLocalDeltaTime DeltaTime)
  (LocalVariables|SetbIsCurrentlyAtMin (== (.ActiveTransitionSeconds (Utilities|Struct|BreakFStructMotionCurveTransition (LocalVariables|GetLocalTransitionData))) 0.0))
  (LocalVariables|SetbIsCurrentlyAtMax (>= (.ActiveTransitionSeconds (Utilities|Struct|BreakFStructMotionCurveTransition (LocalVariables|GetLocalTransitionData))) (.transitiontime (.TransitionConfiguration (Utilities|Struct|BreakFStructMotionCurveTransition (LocalVariables|GetLocalTransitionData))))))
  (bind _updatedactivedeltaseconds (CallFunction|UpdateSeconds (.ActiveTransitionSeconds (Utilities|Struct|BreakFStructMotionCurveTransition (LocalVariables|GetLocalTransitionData))) (.tickrate (.TransitionConfiguration (Utilities|Struct|BreakFStructMotionCurveTransition (LocalVariables|GetLocalTransitionData)))) (LocalVariables|GetLocalDeltaTime) false))
  (bind _structout (Utilities|Struct|SetmembersinFStructMotionCurveTransition (LocalVariables|GetLocalTransitionData) _updatedactivedeltaseconds))
  (if (LocalVariables|GetbIsCurrentlyAtMin)
    (return _structout "NewEnumerator1")
    (elif (LocalVariables|GetbIsCurrentlyAtMax)
      (return _structout "NewEnumerator4")
      (else
        (return _structout "NewEnumerator0")))))

(fn SetTransitionPauseState
  (params (CurveTransition :type F%20Struct%20Motion%20Curve%20Transition%20Structure) (bIsPaused :type Boolean))
  ;[1 1 1] Sets the pause state for a given curve transition.
  (bind (_bfound _index) (Transitions|GetTransitionbyIdentifier (.Identifier (Utilities|Struct|BreakFStructMotionCurveTransitionConfiguration (.TransitionConfiguration (Utilities|Struct|BreakFStructMotionCurveTransition CurveTransition)))) "NewEnumerator0"))
  (if _bfound
    (bind _structout (Utilities|Struct|SetmembersinFStructMotionCurveTransition (Utilities|GetMotionTransition _index) bIsPaused))
    (Utilities|SetMotionTransition _structout _index)))

(fn SetinTransitionState
  (params (bIsInTransition :type Boolean) (TransitionData :type F%20Struct%20Motion%20Curve%20Transition%20Structure))
  ;[1 1 1] Updates the transition flag for a transition.
  (bind (_bfound _index) (CurveFunctions|GetCurvebyComponent (.Identifier (Utilities|Struct|BreakFStructMotionCurveTransitionConfiguration (.TransitionConfiguration (Utilities|Struct|BreakFStructMotionCurveTransition TransitionData))))))
  (if _bfound
    (bind _structout (Utilities|Struct|SetmembersinFStructMotionCurve (Utilities|Array|Get(acopy) (Variables|ManagerData|GetActiveMotionCurves) _index) bIsInTransition))
    (Utilities|SetMotionCurve _structout _index)))

(fn DeleteTransition
  (params (SourceCurveIdentifier :type F%20Struct%20Motion%20Curve%20Identifier%20Structure))
  ;[1 1 1] Removes a transition from the array.
  (bind (_bfound _index) (Transitions|GetTransitionbyIdentifier SourceCurveIdentifier "NewEnumerator0"))
  (if _bfound
    (Utilities|Array|RemoveIndex (Variables|ManagerData|GetActiveMotionCurveTransitions) _index)
    (return true)
    (else
      (return false))))

(fn SetCurveTickRate
  (params (Curve :type F%20Struct%20Motion%20Curve%20Identifier%20Structure) (TickRate :type Float%20%28double-precision%29))
  ;[1 1 1] Sets a Motion Curve's tickrate to the specified value.
  (bind (_bfound _index) (CurveFunctions|GetCurvebyIdentifier Curve))
  (if _bfound
    (bind _structout (Utilities|Struct|SetmembersinFStructMotionCurveConfiguration (.Configuration (Utilities|Struct|BreakFStructMotionCurve (Utilities|GetMotionCurve _index))) TickRate))
    (bind _structout_2 (Utilities|Struct|SetmembersinFStructMotionCurve (Utilities|GetMotionCurve _index) _structout))
    (Utilities|SetMotionCurve _structout_2 _index
      (:_
        (return true)))
    (else
      (return false))))