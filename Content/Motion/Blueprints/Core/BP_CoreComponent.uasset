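; BP_CoreComponent is a core actor component that provides dependency lookup and fail-fast error handling for character Blueprints.
; GetComponent searches the owning actor for a component of the given class and raises a missing-dependency exception when none is found.
; Exception handlers for missing components, configuration and null data print a red on-screen message naming the culprit, then quit the game.
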(fn HandleMissingComponentDependencyException
  (params (MissingDependency :type Actor%20Component%20Class%20Reference) (RequiredBy :type Actor%20Component%20Class%20Reference))
  ;[1 1 1] Quits the game and prints an error message that a required component could not be found.
  (Development|PrintString 0 (Utilities|String|Append "UNABLE TO FIND  " (Utilities|GetClassDisplayName MissingDependency) "IN CHARACTER BLUEPRINT. (REQUIRED BY " (Utilities|GetClassDisplayName RequiredBy) " )") true true "(R=1.000000,G=0.000000,B=0.000000,A=1.000000)" 1e+01)
  (Game|QuitGame 0 0 "Quit" false))

(fn HandleMissingConfigurationDependencyException
  (params (MissingDependency :type String) (RequiredBy :type Actor%20Component%20Class%20Reference))
  ;[1 1 1] Quits the game and prints an error message that a required configuration could not be found.
  (Development|PrintString (LocalVariables|Get__WorldContext) (Utilities|String|Append "MISSING CONFIGURATION OF " MissingDependency " IN " (Utilities|GetClassDisplayName RequiredBy)) true true "(R=1.000000,G=0.000000,B=0.000000,A=1.000000)" 1e+01)
  (Game|QuitGame (LocalVariables|Get__WorldContext) 0 "Quit" false))

(fn HandleMissingDataException
  (params (MissingMember :type String) (MissingIn :type String))
  ;[1 1 1] Quits the game and prints an error message that a required member is NULL.
  (Development|PrintString (LocalVariables|Get__WorldContext) (Utilities|String|Append MissingMember " IS NULL IN " MissingIn) true true "(R=1.000000,G=0.000000,B=0.000000,A=1.000000)" 1e+01)
  (Game|QuitGame (LocalVariables|Get__WorldContext) 0 "Quit" false))

(fn GetComponent
  (params (ComponentClass :type Actor%20Component%20Class%20Reference) (RequiredBy :type Actor%20Component%20Object%20Reference))
  (bind _returnvalue (Components|GetOwner))
  (bind _returnvalue_2 (Actor|GetComponentbyClass _returnvalue ComponentClass))
  ;[1 1 1] Tries to find a component with the provided class name in the character blueprint. Will trigger an exception if not found.
  (Utilities|IsValid _returnvalue_2
    (:Is%20Valid
      (return _returnvalue_2))
    (:Is%20Not%20Valid
      (CallFunction|HandleMissingDependencyException ComponentClass (Utilities|GetClass RequiredBy)))))