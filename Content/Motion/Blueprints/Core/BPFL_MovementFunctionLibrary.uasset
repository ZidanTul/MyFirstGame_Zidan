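; Blueprint function library for the movement system, providing curve-driven timer helpers and fatal setup error handlers.
; Timer functions step seconds forward or backward by a scaled delta, optionally clamping between zero and a curve's end time, read from the curve itself so no length parameter is needed.
; Companion checks report whether a timer sits at either curve end.
; Missing-dependency and failed-cast handlers print a red error and quit the game.
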(fn IsCurveatCurveTime
  (params (Curve :type Curve%20Vector%20Object%20Reference) (CurveTime :type ECurveTimes%20Enum :default "NewEnumerator1") (ActiveDeltaSeconds :type Float%20%28double-precision%29))
  ;[1 1 1] Returns true if the provided delta second timer is close the final point of the provided curve.
  (bind _time (CallFunction|GetCurveTime Curve CurveTime))
  (switch Utilities|FlowControl|Switch|SwitchonECurveTimes CurveTime
    (:NewEnumerator0
      (return (Math|Float|NearlyEqual(Float) ActiveDeltaSeconds 0.0 0.001)))
    (:NewEnumerator1
      (return (or (Math|Float|NearlyEqual(Float) (- _time ActiveDeltaSeconds) 0.0 0.001) (> ActiveDeltaSeconds _time))))))

(fn GetCurveTime
  (params (Curve :type Curve%20Vector%20Object%20Reference) (TimeType :type ECurveTimes%20Enum :default "NewEnumerator0"))
  ;[1 1 1] Returns either the min or max time of the provided Vector curve.
  (switch Utilities|FlowControl|Switch|SwitchonECurveTimes TimeType
    (:NewEnumerator0
      (return 0.0))
    (:NewEnumerator1
      (return (.MaxTime (Math|Curves|GetTimeRange Curve))))))

(fn UpdateSecondswithCurve
  (params (Curve :type Curve%20Vector%20Object%20Reference) (ActiveSeconds :type Float%20%28double-precision%29) (DeltaTickRate :type Float%20%28double-precision%29) (DeltaSeconds :type Float%20%28double-precision%29) (Reverse :type Boolean))
  ;[1 1 1] Updates a timer using a curve. Will stop updating if the timer reached the provided curve's min or max point.
  (LocalVariables|SetAdjustedDelta (* DeltaTickRate DeltaSeconds))
  (if Reverse
    (bind _is_zero (CallFunction|IsCurveatZero ActiveSeconds))
    (if (not _is_zero)
      (if (>= (- ActiveSeconds (LocalVariables|GetAdjustedDelta)) 0.0)
        (return (- ActiveSeconds (LocalVariables|GetAdjustedDelta)))
        (else
          _)))
    (return 0.0)
    (else
      (bind _time (CallFunction|GetCurveTime Curve "NewEnumerator1"))
      (if (not (Math|Float|NearlyEqual(Float) (- _time ActiveSeconds) 0.0 0.001))
        (if (<= (+ ActiveSeconds (LocalVariables|GetAdjustedDelta)) _time)
          (return (+ ActiveSeconds (LocalVariables|GetAdjustedDelta)))
          (else
            _)))
      (return _time))))

(fn UpdateSeconds
  (params (ActiveSeconds :type Float%20%28double-precision%29) (DeltaTickRate :type Float%20%28double-precision%29) (DeltaSeconds :type Float%20%28double-precision%29) (Reverse :type Boolean))
  ;[1 1 1] Updates a timer using the provided tick rate and delta adjustment.
  (LocalVariables|SetAdjustedDelta (* DeltaTickRate DeltaSeconds))
  (if Reverse
    (return (- ActiveSeconds (LocalVariables|GetAdjustedDelta)))
    (else
      (return (+ ActiveSeconds (LocalVariables|GetAdjustedDelta))))))

(fn IsCurveatZero
  (params (ActiveDeltaSeconds :type Float%20%28double-precision%29))
  ;[1 1 1] Returns true if the provided timer is currently exactly at zero.
  (return (== ActiveDeltaSeconds 0.0)))

(fn HandleMissingDependencyException
  (params (MissingDependency :type Actor%20Component%20Class%20Reference) (RequiredBy :type Actor%20Component%20Class%20Reference))
  ;[1 1 1] Quits the game and prints an error message that a required component could not be found.
  (Development|PrintString 0 (Utilities|String|Append "UNABLE TO FIND  " (Utilities|GetClassDisplayName MissingDependency) "IN CHARACTER BLUEPRINT. (REQUIRED BY " (Utilities|GetClassDisplayName RequiredBy) " )") true true "(R=1.000000,G=0.000000,B=0.000000,A=1.000000)" 1e+01)
  (Game|QuitGame 0 0 "Quit" false))

(fn HandleInvalidCastException
  (params (ActorClass :type Actor%20Class%20Reference))
  ;[1 1 1] Quits the game and prints an error message that a component could not be cast to the desired target class.
  (Development|PrintString 0 (Utilities|String|Append "UNABLE TO CAST TO " (Utilities|GetClassDisplayName ActorClass)) true true "(R=1.000000,G=0.000000,B=0.000000,A=1.000000)" 1e+01)
  (Game|QuitGame 0 0 "Quit" false))